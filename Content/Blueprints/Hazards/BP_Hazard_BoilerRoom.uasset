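; Boiler room hazard whose pressure starts draining on a looping timer once the Boiler Core Unlocked event arrives.
; Each tick updates the HUD gauge and maps pressure to four states by integer division, warning the player on changes and triggering overload VFX and LevelEventManager in the lowest.
; Holding R to repair refills pressure on a fast timer, clearing the overload in the top band.
; Full pressure pauses the drain for a buffer delay.
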(event OnComponentBeginOverlap(InputInteraction)
  (params (OverlappedComponent :type Primitive%20Component%20Object%20Reference) (OtherActor :type Actor%20Object%20Reference) (OtherComp :type Primitive%20Component%20Object%20Reference) (OtherBodyIndex :type Integer) (bFromSweep :type Boolean) (SweepResult :type Hit%20Result%20Structure%20%28by%20ref%29))
  (bind _asbp_fpcharacter (Utilities|Casting|CastToBP_FPCharacter OtherActor))
  (Default|DisplayInputPrompt _asbp_fpcharacter "Hold R to repair"))

(event OnComponentEndOverlap(InputInteraction)
  (params (OverlappedComponent :type Primitive%20Component%20Object%20Reference) (OtherActor :type Actor%20Object%20Reference) (OtherComp :type Primitive%20Component%20Object%20Reference) (OtherBodyIndex :type Integer))
  (bind _asbp_fpcharacter (Utilities|Casting|CastToBP_FPCharacter OtherActor))
  (Default|HideInputPrompt _asbp_fpcharacter))

(event Custom|StabilizePressure
  (Utilities|Time|ClearandInvalidateTimerbyHandle (Variables|Default|GetReducePressureTimer))
  (Utilities|FlowControl|Delay (Variables|Default|GetBufferTime))
  (bind _returnvalue (Utilities|Time|SetTimerbyEvent (EventDispatchers|CreateEvent :!event ReducePressure) (Variables|Default|GetPressureReduceTick) true))
  (Variables|Default|SetReducePressureTimer _returnvalue))

(event EventOnNotify
  (params (EventType :type E_LevelEventType%20Enum :default "NewEnumerator0"))
  (switch Utilities|FlowControl|Switch|SwitchonE_LevelEventType EventType
    (:NewEnumerator8
      (Development|PrintString "Started the hazard event")
      (bind _returnvalue (Utilities|Time|SetTimerbyEvent (EventDispatchers|CreateEvent :!event ReducePressure) (Variables|Default|GetPressureReduceTick) true))
      (Variables|Default|SetReducePressureTimer _returnvalue))))

(event EventRepair
  (params (Player :type BP%20FP%20Character%20Object%20Reference) (Repairing? :type Boolean))
  (CallFunction|RepairLoop Player Repairing?))

(event EventBeginPlay
  (|CallParentFunction))

(fn ConstructionScript)

(fn ReducePressure
  (bind _returnvalue (Utilities|Enum|LiteralenumE_HazardBoilerAreaStates "NewEnumerator0"))
  (bind _returnvalue_2 (Utilities|Enum|LiteralenumE_HazardBoilerAreaStates "NewEnumerator3"))
  (bind _returnvalue_3 (Utilities|Enum|LiteralenumE_HazardBoilerAreaStates "NewEnumerator2"))
  (bind _returnvalue_4 (Utilities|Enum|LiteralenumE_HazardBoilerAreaStates "NewEnumerator1"))
  (if (> (Variables|Default|GetPressureLevel) 0)
    (bind _result (Math|Integer|DecrementInt (Variables|Default|GetPressureLevel))
      (:%20%20
        (CallFunction|UpdatePressureGauge)
        (switch int (/ _result 25)
          (:0
            (if (Utilities|Enum|NotEqual(Enum) _returnvalue_2 (Variables|Default|GetHazardStates))
              (CallFunction|AlertPressureStateChange _returnvalue_2))
            (Variables|Default|SetHazardStates "NewEnumerator3")
            (Default|PressureGuageOverloaded (Variables|Default|GetLevelEventManager))
            (Components|Activation|Activate (Variables|Default|GetHazardEvent_VFX) false)
            (return))
          (:1
            (if (Utilities|Enum|NotEqual(Enum) _returnvalue_3 (Variables|Default|GetHazardStates))
              (CallFunction|AlertPressureStateChange _returnvalue_3))
            (Variables|Default|SetHazardStates "NewEnumerator2"))
          (:2
            (if (Utilities|Enum|NotEqual(Enum) _returnvalue_4 (Variables|Default|GetHazardStates))
              (CallFunction|AlertPressureStateChange _returnvalue_4))
            (Variables|Default|SetHazardStates "NewEnumerator1"))
          (:3
            (if (Utilities|Enum|NotEqual(Enum) _returnvalue (Variables|Default|GetHazardStates))
              (CallFunction|AlertPressureStateChange _returnvalue))
            (Variables|Default|SetHazardStates "NewEnumerator0")))))))

(fn GetPressureStatus
  (for (_array_element _array_index) (Variables|Default|GetPressureStatus)
    (if (== _array_element (Variables|Default|GetPressureLevel))
      (return _array_index)
      (else
        (return (LocalVariables|GetDefault))))))

(fn RepairLoop
  (params (Player :type BP%20FP%20Character%20Object%20Reference) (IsRepairing :type Boolean))
  (Variables|Default|SetPlayer Player)
  (if IsRepairing
    (if (< (Variables|Default|GetPressureLevel) (Variables|Default|GetMaxPressure))
      (Variables|/Game/Blueprints/Player/BP_FPCharacter.BP_FPCharacter_C|SetPlayerStates Player "NewEnumerator6")
      (Utilities|Time|ClearandInvalidateTimerbyHandle (Variables|Default|GetRepairTimer))
      (bind _returnvalue (Utilities|Time|SetTimerbyEvent (EventDispatchers|CreateEvent :!event Repairing) 0.05 true))
      (Variables|Default|SetRepairTimer _returnvalue)
      (else
        (Utilities|Time|ClearandInvalidateTimerbyHandle (Variables|Default|GetRepairTimer))))
    (else
      (Utilities|Time|ClearandInvalidateTimerbyHandle (Variables|Default|GetRepairTimer))
      (Default|DisplayRepairing Player (Math|Conversions|ToFloat(Integer) (Variables|Default|GetPressureLevel)) (Math|Conversions|ToFloat(Integer) (Variables|Default|GetMaxPressure)) false))))

(fn Repairing
  (if (< (Variables|Default|GetPressureLevel) (Variables|Default|GetMaxPressure))
    (bind _result (Math|Integer|IncrementInt (Variables|Default|GetPressureLevel))
      (:%20%20
        (CallFunction|UpdatePressureGauge)
        (Default|DisplayRepairing (Variables|Default|GetPlayer) (Math|Conversions|ToFloat(Integer) (Variables|Default|GetPressureLevel)) (Math|Conversions|ToFloat(Integer) (Variables|Default|GetMaxPressure)) true)
        (switch int (/ _result 25)
          (:0
            (Variables|Default|SetHazardStates "NewEnumerator3"))
          (:1
            (Variables|Default|SetHazardStates "NewEnumerator2"))
          (:2
            (Variables|Default|SetHazardStates "NewEnumerator1"))
          (:3
            (Variables|Default|SetHazardStates "NewEnumerator0")
            (Default|PressureGuageRestored (Variables|Default|GetLevelEventManager))
            (Components|Activation|Deactivate (Variables|Default|GetHazardEvent_VFX))))))
    (else
      (CallFunction|AlertPressureStateChange "NewEnumerator0")
      (Utilities|Time|ClearandInvalidateTimerbyHandle (Variables|Default|GetRepairTimer))
      (CallFunction|StabilizePressure)
      (Default|DisplayRepairing (Variables|Default|GetPlayer) (Math|Conversions|ToFloat(Integer) (Variables|Default|GetPressureLevel)) (Math|Conversions|ToFloat(Integer) (Variables|Default|GetMaxPressure)) false))))

(fn AlertPressureStateChange
  (params (HazardStates :type E_HazardBoilerAreaStates%20Enum :default "NewEnumerator0"))
  (Utilities|IsValid (Variables|Default|GetPlayer)
    (:Is%20Valid
      _)
    (:Is%20Not%20Valid
      (bind _asbp_fpcharacter (Utilities|Casting|CastToBP_FPCharacter (Game|GetPlayerCharacter 0)))
      (Variables|Default|SetPlayer _asbp_fpcharacter)))
  (Default|DisplayPressureWarning (Variables|Default|GetPlayer) HazardStates))

(fn UpdatePressureGauge
  (bind _asbpi_ui (Utilities|Casting|CastToBPI_UI (HUD|GetHUD (Game|GetPlayerController 0))))
  (Default|UpdatePressureIndicator _asbpi_ui (Variables|Default|GetPressureLevel)))