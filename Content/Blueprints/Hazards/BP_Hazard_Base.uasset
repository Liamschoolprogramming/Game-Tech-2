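; Base hazard actor for a repairable pressure gauge that drains stocked resources and overloads when one runs out.
; It registers with BP_LevelEventManager as an observer and toggles a hazard menu on player interaction.
; Activate starts a consumption timer; overload and restore alert the player and notify the manager, with restocking scheduling reactivation.
; Gauge widget and inventory seeding logic is disconnected from BeginPlay, and several machine getters are stubs.
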(event OnComponentBeginOverlap(InputInteraction)
  (params (OverlappedComponent :type Primitive%20Component%20Object%20Reference) (OtherActor :type Actor%20Object%20Reference) (OtherComp :type Primitive%20Component%20Object%20Reference) (OtherBodyIndex :type Integer) (bFromSweep :type Boolean) (SweepResult :type Hit%20Result%20Structure%20%28by%20ref%29))
  (bind _asbp_fpcharacter (Utilities|Casting|CastToBP_FPCharacter OtherActor))
  (Default|DisplayInputPrompt _asbp_fpcharacter "Press R to repair"))

(event OnComponentEndOverlap(InputInteraction)
  (params (OverlappedComponent :type Primitive%20Component%20Object%20Reference) (OtherActor :type Actor%20Object%20Reference) (OtherComp :type Primitive%20Component%20Object%20Reference) (OtherBodyIndex :type Integer))
  (bind _asbp_fpcharacter (Utilities|Casting|CastToBP_FPCharacter OtherActor))
  (Default|HideInputPrompt _asbp_fpcharacter))

(event EventBeginPlay
  (CallFunction|SubscribetoLevelEventManager)
  (UserInterface|CreateWidget "/Game/UI/WidgetBlueprints/Hazards/W_HazardMenu.W_HazardMenu_C" 0 self))

(event EventInteract
  (params (Player :type BP%20FP%20Character%20Object%20Reference))
  (CallFunction|PlayerInteract Player))

(fn ConstructionScript)

(fn SubscribetoLevelEventManager
  (bind _returnvalue (Actor|GetActorOfClass "/Game/Blueprints/LevelEventManager/BP_LevelEventManager.BP_LevelEventManager_C"))
  (Variables|Default|SetLevelEventManager _returnvalue)
  (bind _asbpi_observer (Utilities|Casting|CastToBPI_Observer self))
  (Default|SubscribeObserver (Variables|Default|GetLevelEventManager) _asbpi_observer))

(fn Activate
  (bind _asbp_fpcharacter (Utilities|Casting|CastToBP_FPCharacter (Game|GetPlayerCharacter 0)))
  (Default|DisplayAlert _asbp_fpcharacter "Pressure Gauge is rising")
  (bind _returnvalue (Utilities|Time|SetTimerbyEvent (EventDispatchers|CreateEvent :!event DecrementResources) (Variables|Default|GetConsumptionRate) true))
  (Variables|Default|SetConsumptionTimer _returnvalue))

(fn PlayerInteract
  (params (Player :type BP%20FP%20Character%20Object%20Reference))
  (if (Widget|IsVisible (Variables|Default|GetHazardMenu))
    (Widget|RemovefromParent (Variables|Default|GetHazardMenu))
    (Input|SetInputModeGameOnly (Game|GetPlayerController 0) false)
    (Variables|/Script/Engine.PlayerController|SetbShowMouseCursor (Game|GetPlayerController 0) false)
    (Variables|/Game/Blueprints/Player/BP_FPCharacter.BP_FPCharacter_C|SetMovementEnabled Player true)
    (Variables|/Game/Blueprints/Player/BP_FPCharacter.BP_FPCharacter_C|SetMenuOpen Player false)
    (else
      (UserInterface|Viewport|AddtoViewport (Variables|Default|GetHazardMenu) 0)
      (Input|SetInputModeGameandUI (Game|GetPlayerController 0) (Variables|Default|GetHazardMenu) "DoNotLock" true false)
      (Variables|/Script/Engine.PlayerController|SetbShowMouseCursor (Game|GetPlayerController 0) true)
      (Variables|/Game/Blueprints/Player/BP_FPCharacter.BP_FPCharacter_C|SetMovementEnabled Player false)
      (Variables|/Game/Blueprints/Player/BP_FPCharacter.BP_FPCharacter_C|SetMenuOpen Player true))))

(fn DecrementResources
  (bind (_keypin _valuepin) (Utilities|Map|ForEachLoop(Map) (Variables|/Game/Blueprints/Components/BP_Inventory.BP_Inventory_C|GetResource%20Inventory (Variables|Default|GetBP_Inventory)))
    (:then
      (LocalVariables|SetL_ResourceName _keypin)
      (bind _output_get (LocalVariables|SetL_ResourceAmt _valuepin))
      (if (> _output_get 0)
        (Default|RemoveResourcefromInventory (Variables|Default|GetBP_Inventory) (LocalVariables|GetL_ResourceName) 1)
        (Default|UpdateResources (Variables|Default|GetHazardMenu))
        (Default|UpdateConsumptionTimer (Variables|Default|GetGaugeWidgetRef) (Math|Conversions|ToFloat(Integer) (LocalVariables|GetL_ResourceAmt)))
        (if (<= (LocalVariables|GetL_ResourceAmt) 0)
          (CallFunction|HazardOverload true)
          (Utilities|Time|ClearandInvalidateTimerbyHandle (Variables|Default|GetConsumptionTimer)))
        (else
          (Default|UpdateConsumptionTimer (Variables|Default|GetGaugeWidgetRef) (Math|Conversions|ToFloat(Integer) (LocalVariables|GetL_ResourceAmt)))
          (CallFunction|HazardOverload true)
          (Utilities|Time|ClearandInvalidateTimerbyHandle (Variables|Default|GetConsumptionTimer)))))))

(fn CheckifInventoryIsEmpty
  (bind _valuepin (Utilities|Map|ForEachLoop(Map) (Variables|/Game/Blueprints/Components/BP_Inventory.BP_Inventory_C|GetResource%20Inventory (Variables|Default|GetBP_Inventory)))
    (:then
      (if (> _valuepin 0)
        (if (Variables|Default|GetHazardOverloaded?)
          (CallFunction|HazardOverload false)
          (Utilities|Time|SetTimerbyFunctionName 0 "Activate" 2.0))))))

(fn HazardOverload
  (params (Overloaded? :type Boolean))
  (bind _leveleventmanager (Variables|Default|GetLevelEventManager))
  (bind _output_get (Variables|Default|SetHazardOverloaded? Overloaded?))
  (if _output_get
    (Default|CallOnPressureGaugeOverloaded _leveleventmanager)
    (bind _asbp_fpcharacter (Utilities|Casting|CastToBP_FPCharacter (Game|GetPlayerCharacter 0)))
    (Default|DisplayAlert _asbp_fpcharacter "Pressure Gauge is overloaded!")
    (else
      (Default|CallOnPressureGaugeRestored _leveleventmanager)
      (bind _asbp_fpcharacter_2 (Utilities|Casting|CastToBP_FPCharacter (Game|GetPlayerCharacter 0)))
      (Default|DisplayAlert _asbp_fpcharacter_2 "Pressure Gauge is restored"))))

(fn BPHazardBaseAutoGenFunc)

(fn RotateWidgettoFacePlayer
  (Transformation|SetWorldRotation (Variables|Default|GetGaugeWidget) (Math|Rotator|MakeRotator 0.0 0.0 (.yaw (Math|Rotator|FindLookatRotation (Transformation|GetWorldLocation (Variables|Default|GetGaugeWidget)) (Transformation|GetWorldLocation (Variables|/Script/Engine.PlayerCameraManager|GetTransformComponent (Game|GetPlayerCameraManager 0)))))) false false))

(fn SetObjectiveManager
  (bind _returnvalue (Actor|GetActorOfClass "/Game/Blueprints/Managers/BP_ObjectiveManager.BP_ObjectiveManager_C"))
  (Variables|Default|SetObjectiveManager _returnvalue))

(fn GameplayTag
  (return "(TagName=\"Interactable\")"))

(fn GetGameplayTags
  (return "(GameplayTags=((TagName=\"Interactable\")))"))

(fn GetLocation
  (return (Transformation|GetActorLocation)))

(fn GetMachine
  (return 0))

(fn GetMachineClass
  (return (Utilities|GetClass self)))

(fn GetMachineMesh
  (return 0))

(fn GetName
  (return (Variables|Default|Getname)))

(fn GetRotation
  (return 0.0))

(fn HasResource
  (params (Resource%20Name :type Name :default "None"))
  (return 0 false))