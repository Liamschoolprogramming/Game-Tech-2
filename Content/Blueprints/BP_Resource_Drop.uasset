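; BP_Resource_Drop is a pickup that adds a set amount of a resource to the player's inventory on overlap, then destroys itself.
; The construction script loads the resource's data table row and previews its static mesh.
; On BeginPlay it sets the mesh, using a skeletal one for Star Dust, and subscribes to BP_LevelEventManager.
; A Load Game notification from that manager also destroys the drop.
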(event OnComponentBeginOverlap(Collision)
  (params (OverlappedComponent :type Primitive%20Component%20Object%20Reference) (OtherActor :type Actor%20Object%20Reference) (OtherComp :type Primitive%20Component%20Object%20Reference) (OtherBodyIndex :type Integer) (bFromSweep :type Boolean) (SweepResult :type Hit%20Result%20Structure%20%28by%20ref%29))
  (if (Utilities|DoesObjectImplementInterface OtherActor "/Game/Blueprints/Player/BPI_FirstPersonPlayer.BPI_FirstPersonPlayer_C")
    (Default|AddResourcetoInventory (Actor|GetComponentbyClass OtherActor "/Game/Blueprints/Components/BP_Inventory.BP_Inventory_C") (Variables|Default|GetResouce%20Name) (Variables|Default|GetAmount%20To%20Drop))
    (Actor|DestroyActor)))

(event Custom|SetMesh
  (params (Mesh :type Static%20Mesh%20Object%20Reference))
  (Components|StaticMesh|SetStaticMesh (Variables|Default|GetStatic%20Mesh) Mesh))

(event Custom|SetSkeletalMesh
  (params (SkeletalMesh :type Skeletal%20Mesh%20Object%20Reference))
  (Components|SkeletalMesh|SetSkeletalMeshAsset (Variables|Default|GetSkeletalMesh) SkeletalMesh))

(event EventOnNotify
  (params (EventType :type E_LevelEventType%20Enum :default "NewEnumerator0"))
  (switch Utilities|FlowControl|Switch|SwitchonE_LevelEventType EventType
    (:NewEnumerator7
      (Actor|DestroyActor))))

(event EventBeginPlay
  (bind _resource (Variables|Default|GetResource))
  (bind _returnvalue (Actor|GetActorOfClass "/Game/Blueprints/LevelEventManager/BP_LevelEventManager.BP_LevelEventManager_C"))
  (CallFunction|SubscribeLevelEventManager self _returnvalue)
  (switch name (.name _resource)
    (:Default
      (CallFunction|SetMesh (.mesh _resource)))
    (:Star%20Dust
      (CallFunction|SetSkeletalMesh (.skeletalmesh _resource)))))

(fn ConstructionScript
  (bind _returnvalue (Utilities|GetDataTableRow (Variables|Default|GetResource%20Data%20Table) (Variables|Default|GetResouce%20Name))
    (:then
      (Variables|Default|SetResource _returnvalue)
      (Components|StaticMesh|SetStaticMesh (Variables|Default|GetStatic%20Mesh) (.Mesh (Utilities|Struct|BreakS_Resources _returnvalue))))))

(fn GameplayTag
  (return "(TagName=\"Resource\")"))

(fn GetGameplayTags
  (return (Variables|Default|GetGameplay%20Tags)))

(fn GetLocation
  (return "0, 0, 0"))

(fn GetMachine
  (return 0))

(fn GetMachineClass
  (return 0))

(fn GetMachineMesh
  (return 0))

(fn GetName
  (return "None"))

(fn GetRotation
  (return 0.0))

(fn HasResource
  (params (Resource%20Name :type Name :default "None"))
  (return 0 false))