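; Inventory component that stores resources with name, mesh and amount, supporting add, lookup and removal.
; An array holds the resource structs, and a name-to-index map is refreshed after each add for lookups by name.
; Adds by name build structs from a data table; adding increases matching amounts but also appends per non-matching entry.
; Removal by name or index subtracts amounts without clamping or deleting entries.
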(fn GetResourceAmount
  (params (Name :type Name))
  (bind _m_resource_inventory (Variables|Default|GetM%20Resource%20Inventory))
  (bind _s_resource_inventory (Variables|Default|GetS%20Resource%20Inventory))
  (bind _value (Utilities|Map|Find _m_resource_inventory Name))
  (bind _output (Utilities|Array|Get(acopy) _s_resource_inventory _value))
  (bind (_name _mesh _amount) (Utilities|Struct|BreakS_Resources _output))
  (return _name _value _amount))

(fn AddtoInventory
  (params (Item%20to%20Add :type S%20Resources%20Structure))
  (bind (_name _mesh _amount) (Utilities|Struct|BreakS_Resources Item%20to%20Add))
  (bind _s_resource_inventory (Variables|Default|GetS%20Resource%20Inventory))
  (if (Utilities|Array|IsEmpty _s_resource_inventory)
    (Utilities|Array|Add (Variables|Default|GetS%20Resource%20Inventory) Item%20to%20Add)
    (CallFunction|InventoryMap)
    (return)
    (else
      (for (_array_element _array_index) _s_resource_inventory
        (if (== (.Name (Utilities|Struct|BreakS_Resources _array_element)) _name)
          (bind _structout (Utilities|Struct|SetmembersinS_Resources (Utilities|Array|Get(acopy) (Variables|Default|GetS%20Resource%20Inventory) _array_index) (+ _amount (.Amount (Utilities|Struct|BreakS_Resources _array_element)))))
          (Development|PrintString (Utilities|String|ToString(Name) (.Name (Utilities|Struct|BreakS_Resources _structout))))
          (else
            (Utilities|Array|Add _s_resource_inventory Item%20to%20Add))))
      (CallFunction|InventoryMap)
      (return))))

(fn RemoveResourcefromInventorybyIndex
  (params (Resource%20Name :type Name) (Amount%20to%20Remove :type Integer) (Resource%20Index :type Integer))
  (bind _s_resource_inventory (Variables|Default|GetS%20Resource%20Inventory))
  (bind _output (Utilities|Array|Get(acopy) _s_resource_inventory Resource%20Index))
  (Utilities|Struct|SetmembersinS_Resources _output (- (.Amount (Utilities|Struct|BreakS_Resources _output)) Amount%20to%20Remove)))

(fn InventoryMap
  (for (_array_element _array_index) (Variables|Default|GetS%20Resource%20Inventory)
    (Utilities|Map|Add (Variables|Default|GetM%20Resource%20Inventory) (.Name (Utilities|Struct|BreakS_Resources _array_element)) _array_index)))

(fn AddbyNametoInventory
  (params (Name :type Name) (Amount :type Integer))
  (bind _returnvalue (Utilities|GetDataTableRow (Variables|Default|GetResources%20Table) Name)
    (:then
      (CallFunction|AddtoInventory (Utilities|Struct|MakeS_Resources (.Name (Utilities|Struct|BreakS_Resources _returnvalue)) (.Mesh (Utilities|Struct|BreakS_Resources _returnvalue)) Amount)))))

(fn RemoveResourcefromInventorybyName
  (params (Resource%20Name :type Name) (Amount%20to%20Remove :type Integer))
  (bind _s_resource_inventory (Variables|Default|GetS%20Resource%20Inventory))
  (bind _m_resource_inventory (Variables|Default|GetM%20Resource%20Inventory))
  (bind (_value _returnvalue) (Utilities|Map|Find _m_resource_inventory Resource%20Name))
  (bind _output (Utilities|Array|Get(acopy) _s_resource_inventory _value))
  (if _returnvalue
    (Development|PrintString "found")
    (bind _structout (Utilities|Struct|SetmembersinS_Resources _output (- (.Amount (Utilities|Struct|BreakS_Resources _output)) Amount%20to%20Remove)))
    (Development|PrintString "Remaining: ")
    (Development|PrintString (Utilities|String|ToString(Name) (.name _structout)))
    (Development|PrintString (Utilities|String|ToString(Integer) (.amount _structout)))
    (else
      (Development|PrintString "didnt find"))))