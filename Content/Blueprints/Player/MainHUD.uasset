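; MainHUD is the player HUD Blueprint that relays game state and objective updates to on-screen widgets.
; On BeginPlay it creates the W_PinnedObjective widget and adds it to the viewport, then forwards pinned objective and resource refreshes to it.
; State, objective amount and activation events pass to a separate UI reference, which is not assigned here.
; UpdatePlayerResources does nothing because its UI call is disconnected.
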(event EventUpdateObjective
  (params (ObjectiveAmount :type String))
  (Default|UpdateObjective (Variables|Default|GetUI) ObjectiveAmount))

(event EventUpdateObjectiveState
  (params (IsActivated :type String))
  (Default|UpdateObjectiveState (Variables|Default|GetUI) IsActivated))

(event EventUpdatePlayerResources
  (params (ResourceName :type String) (ResourceAmount :type String)))

(event EventBeginPlay
  (bind _returnvalue (UserInterface|CreateWidget "/Game/UI/WidgetBlueprints/Objectives/W_PinnedObjective.W_PinnedObjective_C"))
  (bind _output_get (Variables|Default|SetPinned%20Objective _returnvalue))
  (UserInterface|Viewport|AddtoViewport _output_get 0))

(event EventUpdateState
  (params (State :type String))
  (Default|UpdateState (Variables|Default|GetUI) State))

(event EventUpdateObjective0
  ;[0.15 0.15 0.15 0.5] These are used by the pinned objective widget at the top left of the screen to feed it information when an objective is updated or a new one is pinned
  (Default|UpdatePinnedObjective (Variables|Default|GetPinned%20Objective)))

(event EventUpdateResources0
  (params (Objective :type BP%20Objective%20Base%20Object%20Reference))
  ;[0.15 0.15 0.15 0.5] These are used by the pinned objective widget at the top left of the screen to feed it information when an objective is updated or a new one is pinned
  (Default|UpdateResources (Variables|Default|GetPinned%20Objective) Objective))

(fn ConstructionScript)