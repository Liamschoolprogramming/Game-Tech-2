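; BP_MainHUD creates the player's main HUD widget and relays game state to its sub-widgets.
; On BeginPlay it builds W_HUD, caches the core health, wave timer and pinned objective widgets, adds the HUD and health bar to the viewport, and starts Bridge health full.
; Update events then forward objective, resource, pressure hazard, core health and wave timer changes, with core health handled only for the Bridge.
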(event EventUpdateCoreHealthBar
  (params (CoreName :type Name :default "None") (CurrentHealth :type Float%20%28double-precision%29) (MaxHealth :type Float%20%28double-precision%29))
  (switch name CoreName
    (:Bridge
      (bind _corehealthui (Variables|Default|GetCoreHealthUI)
        (:then
          (Default|UpdateCoreHealth _corehealthui CurrentHealth MaxHealth))
        (:else)))))

(event EventUpdateResourcesHUD
  (params (Objective :type BP%20Objective%20Base%20Object%20Reference))
  ;[0.15 0.15 0.15 0.5] These are used by the pinned objective widget at the top left of the screen to feed it information when an objective is updated or a new one is pinned
  (Default|UpdateResources (Variables|Default|GetPinned%20Objective) Objective))

(event EventUpdateObjectiveHUD
  ;[0.15 0.15 0.15 0.5] These are used by the pinned objective widget at the top left of the screen to feed it information when an objective is updated or a new one is pinned
  (Default|UpdatePinnedObjective (Variables|Default|GetPinned%20Objective)))

(event EventBeginPlay
  (bind _returnvalue (UserInterface|CreateWidget "/Game/UI/WidgetBlueprints/HUD/W_HUD.W_HUD_C"))
  (Variables|Default|SetHUD _returnvalue)
  (Variables|Default|SetCoreHealthUI (Variables|/Game/UI/WidgetBlueprints/HUD/W_HUD.W_HUD_C|GetWB_HUD_CoreHealth _returnvalue))
  (Variables|Default|SetWave%20Timer%20Text (Variables|/Game/UI/WidgetBlueprints/HUD/W_HUD.W_HUD_C|GetWaveTimerText _returnvalue))
  (Variables|Default|SetPinned%20Objective (Variables|/Game/UI/WidgetBlueprints/HUD/W_HUD.W_HUD_C|GetW_PinnedObjective _returnvalue))
  (UserInterface|Viewport|AddtoViewport _returnvalue 0)
  (UserInterface|Viewport|AddtoViewport (Variables|/Game/UI/WidgetBlueprints/HUD/W_HUD.W_HUD_C|GetWB_HUD_CoreHealth _returnvalue) 0)
  (CallFunction|UpdateCoreHealthBar "Bridge" 1e+02 1e+02))

(event EventUpdateWaveTimer
  (params (WaveTimerString :type String))
  (Rendering|Components|TextRender|SetText (Variables|Default|GetWave%20Timer%20Text) (Utilities|Text|ToText(String) WaveTimerString)))

(event EventUpdatePressureIndicator
  (params (HazardState :type E_HazardBoilerAreaStates%20Enum :default "NewEnumerator0"))
  (Default|SetPressureIndicator (Variables|Default|GetHUD) HazardState))

(fn ConstructionScript)