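; Restoration enemy, a child Blueprint that on death spawns a heal pulse and heals nearby BPI_Enemy actors by applying negative damage through a sphere trace.
; Attacks fire after a delay when its sphere overlaps the attack target or through ExecuteAttack, which also starts the ABP_Restoration attack animation.
; SpeedUp and SlowDown swap looping timers that incrementally raise or lower walk speed, with only the decrease clamped.
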(event OnComponentBeginOverlap(Sphere)
  (params (OverlappedComponent :type Primitive%20Component%20Object%20Reference) (OtherActor :type Actor%20Object%20Reference) (OtherComp :type Primitive%20Component%20Object%20Reference) (OtherBodyIndex :type Integer) (bFromSweep :type Boolean) (SweepResult :type Hit%20Result%20Structure%20%28by%20ref%29))
  (if (== OtherActor (Variables|Default|GetAttackTarget))
    (CallFunction|Attack)))

(event Custom|SpeedUp
  (Utilities|Time|ClearandInvalidateTimerbyHandle (Variables|Default|GetSlowDownTimer))
  (bind _returnvalue (Utilities|Time|SetTimerbyFunctionName 0 "AddSpeed" 0.05 true))
  (Variables|Default|SetSpeedUpTimer _returnvalue))

(event Custom|SlowDown
  (Utilities|Time|ClearandInvalidateTimerbyHandle (Variables|Default|GetSpeedUpTimer))
  (bind _returnvalue (Utilities|Time|SetTimerbyFunctionName 0 "RemoveSpeed" 0.05 true))
  (Variables|Default|SetSlowDownTimer _returnvalue))

(event EventBeginPlay
  (|CallParentFunction)
  (Variables|Default|SetCurrentHealth 9.0))

(event EventAttack
  (Utilities|FlowControl|Delay (Variables|Default|GetAttackDelay))
  (|CallParentFunction))

(fn ConstructionScript
  (|CallParentFunction))

(fn Death
  (bind _returnvalue (Transformation|GetActorLocation))
  (Niagara|SpawnSystematLocation "/Game/Blueprints/Enemy/NS_HealPulse.NS_HealPulse" (Transformation|GetActorLocation) "0, 0, 0" (Math|Conversions|ToVector(Float) 17.0))
  (bind _outhits (Collision|MultiSphereTraceByChannel _returnvalue _returnvalue 7e+02 "TraceTypeQuery1" false 0 "None"))
  (for _array_element _outhits
    (if (Utilities|DoesObjectImplementInterface (.HitActor (Collision|BreakHitResult _array_element)) "/Game/Blueprints/Enemy/BPI_Enemy.BPI_Enemy_C")
      (Game|Damage|ApplyDamage (.HitActor (Collision|BreakHitResult _array_element)) -5.0 0 0)))
  (|CallParentFunction))

(fn ExecuteAttack
  (|CallParentFunction)
  (bind _asabp_restoration (Utilities|Casting|CastToABP_Restoration (Components|SkeletalMesh|GetAnimInstance (Variables|Default|GetSkeletalMesh))))
  (Default|StartAttack _asabp_restoration)
  (CallFunction|Attack))

(fn AddSpeed
  (bind _charactermovement (Variables|Character|GetCharacterMovement))
  (Variables|/Script/Engine.CharacterMovementComponent|SetMaxWalkSpeed _charactermovement (+ (Variables|/Script/Engine.CharacterMovementComponent|GetMaxWalkSpeed _charactermovement) 16.0)))

(fn RemoveSpeed
  (Variables|/Script/Engine.CharacterMovementComponent|SetMaxWalkSpeed (Variables|Character|GetCharacterMovement) (Math|Float|Clamp(Float) (- (Variables|/Script/Engine.CharacterMovementComponent|GetMaxWalkSpeed (Variables|Character|GetCharacterMovement)) 5e+01) 0.0 1e+03)))