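; Mortar bug enemy that walks to a free stand position, locks itself in place and shells turrets from there.
; An invalid target makes it claim a stand position; sphere overlaps supply turret targets, remembered if found while still moving.
; Interactable targets start timers for facing and firing from a projectile pool spawned on BeginPlay.
; When a target's health runs out, it seeks another overlapping turret, falling back to the player pawn.
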(event OnComponentBeginOverlap(Sphere)
  (params (OverlappedComponent :type Primitive%20Component%20Object%20Reference) (OtherActor :type Actor%20Object%20Reference) (OtherComp :type Primitive%20Component%20Object%20Reference) (OtherBodyIndex :type Integer) (bFromSweep :type Boolean) (SweepResult :type Hit%20Result%20Structure%20%28by%20ref%29))
  (bind _returnvalue (Utilities|DoesObjectImplementInterface OtherActor "/Game/Blueprints/Machines/Turret/BI_Turret.BI_Turret_C"))
  (if (Variables|Default|GetInPosition?)
    (if _returnvalue
      (CallFunction|SetAttackTarget OtherActor))
    (elif _returnvalue
      (Variables|Default|SetImminentTarget OtherActor))))

(event Custom|AttackLoop
  (bind _current_health (Class|BPIMachine|GetMachineHealth(Message) (Variables|Default|GetAttackTarget)))
  (if (> _current_health 0.0)
    (CallFunction|FiringEffects)
    (else
      (bind _success_ (CallFunction|FindTarget))
      (if _success_
        _
        (else
          (CallFunction|SetAttackTarget (Game|Player|GetPlayerPawn 0))))
      (Utilities|Time|ClearandInvalidateTimerbyHandle (Variables|Default|GetAttackLoopTimer)))))

(event EventBeginPlay
  (|CallParentFunction)
  (for _index (range 0 4)
    (bind _returnvalue (Game|SpawnActorfromClass "/Game/Blueprints/Machines/Turret/BP_ProjectileMortar.BP_ProjectileMortar_C" (Math|Transform|MakeTransform "0, 0, 0" "0, 0, 0" "1.000000,1.000000,1.000000") "AlwaysSpawn" "MultiplyWithRoot" self (Utilities|Struct|MakeStruct_TurretValues 0.0 0.0 (.basedamage (Variables|Default|GetStats)) 0.0 0) 0))
    (Utilities|Array|Add (Variables|Default|GetProjectiles) _returnvalue)))

(event EventSetAttackTarget
  (params (AttackTarget :type Actor%20Object%20Reference))
  (Utilities|IsValid AttackTarget
    (:Is%20Valid
      (Variables|Default|SetAttackTarget AttackTarget)
      (CallFunction|NavigatetoAttackTarget :!label _label))
    (:Is%20Not%20Valid
      (bind _target (CallFunction|GetTargettoStandat))
      (if (Variables|Default|GetAlive?)
        (Variables|Default|SetAttackTarget _target)
        (goto _label)))))

(event EventNavigatetoAttackTarget
  (bind _charactermovement (Variables|Character|GetCharacterMovement))
  (if (Utilities|DoesObjectImplementInterface (Variables|Default|GetAttackTarget) "/Game/Blueprints/BPI_Interactable.BPI_Interactable_C")
    (Utilities|Time|SetTimerbyFunctionName 0 "FaceTarget" 0.05 true)
    (bind _returnvalue (Utilities|Time|SetTimerbyEvent (delegate Custom|AttackLoop) (Variables|Default|GetFire%20Rate) true))
    (Variables|Default|SetAttackLoopTimer _returnvalue)
    (else
      (Utilities|Time|SetTimerbyFunctionName 0 "FaceTarget" 0.05 true)
      (bind _randomlocation (Class|NavigationSystemV1|GetRandomLocationinNavigableRadius (Transformation|GetActorLocation (Variables|Default|GetAttackTarget)) 1e+01 0 0))
      (AI|AIMoveTo self _randomlocation 0 1e+01 true
        (:OnSuccess
          _)
        (:OnFail
          _))
      (Components|Movement|StopMovementImmediately _charactermovement)
      (Pawn|Components|CharacterMovement|DisableMovement _charactermovement)
      (Variables|Default|SetInPosition? true)
      (bind _imminenttarget (Variables|Default|GetImminentTarget)
        (:then
          (CallFunction|SetAttackTarget _imminenttarget))
        (:else
          (CallFunction|SetAttackTarget (Game|Player|GetPlayerPawn 0)))))))

(event EventAttack)

(fn ConstructionScript
  (|CallParentFunction))

(fn GetTargettoStandat
  (bind _outactors (Actor|GetAllActorsOfClass "/Game/Blueprints/Enemy/BP_MortarBug_StandPosition.BP_MortarBug_StandPosition_C"))
  (for _array_element _outactors
    (if (not (Variables|/Game/Blueprints/Enemy/BP_MortarBug_StandPosition.BP_MortarBug_StandPosition_C|GetInUse? _array_element))
      (Default|SetinUse _array_element true)
      (return _array_element)))
  (return 0))

(fn FiringEffects
  (bind _arrow (Variables|Default|GetArrow))
  (bind _chosen_projectile (CallFunction|FirstAvailableProjectile))
  (LocalVariables|SetL_ChosenProjectile _chosen_projectile)
  (Transformation|SetActorLocationAndRotation (LocalVariables|GetL_ChosenProjectile) (- (Transformation|GetWorldLocation _arrow) "0.000000,0.000000,100.000000") (Transformation|GetWorldRotation _arrow))
  (Variables|/Game/Blueprints/Machines/Turret/BP_ProjectileBase.BP_ProjectileBase_C|SetCharged? (LocalVariables|GetL_ChosenProjectile) false)
  (Default|SetIsActive (LocalVariables|GetL_ChosenProjectile) true))

(fn FirstAvailableProjectile
  (for _array_element (Variables|Default|GetProjectiles)
    (if (not (Variables|/Game/Blueprints/Machines/Turret/BP_ProjectileBase.BP_ProjectileBase_C|GetIsActive _array_element))
      (return _array_element))))

(fn FindTarget
  (for _array_element (Collision|GetOverlappingActors (Variables|Default|GetSphere) "/Script/Engine.Actor" :!class /Script/Engine.PrimitiveComponent)
    (if (Utilities|DoesObjectImplementInterface _array_element "/Game/Blueprints/Machines/Turret/BI_Turret.BI_Turret_C")
      (bind _current_health (Class|BPIMachine|GetMachineHealth(Message) _array_element))
      (if (> _current_health 0.0)
        (CallFunction|SetAttackTarget _array_element)
        (return true))))
  (return false))

(fn ExecuteAttack)