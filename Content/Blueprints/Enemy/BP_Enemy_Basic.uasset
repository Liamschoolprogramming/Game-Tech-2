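; BP_Enemy_Basic is a basic enemy Blueprint that extends its parent's attack behavior.
; An overlap on its Sphere component calls Attack when the entering actor is the AttackTarget.
; The ExecuteAttack override runs the parent logic, then calls StartAttack on the skeletal mesh's ABP_Enemy_Basic and calls Attack immediately afterward.
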(event OnComponentBeginOverlap(Sphere)
  (params (OverlappedComponent :type Primitive%20Component%20Object%20Reference) (OtherActor :type Actor%20Object%20Reference) (OtherComp :type Primitive%20Component%20Object%20Reference) (OtherBodyIndex :type Integer) (bFromSweep :type Boolean) (SweepResult :type Hit%20Result%20Structure%20%28by%20ref%29))
  (if (== (Variables|Default|GetAttackTarget) OtherActor)
    (CallFunction|Attack)))

(event EventBeginPlay
  (|CallParentFunction))

(fn ConstructionScript
  (|CallParentFunction))

(fn ExecuteAttack
  (|CallParentFunction)
  (bind _asabp_enemy_basic (Utilities|Casting|CastToABP_Enemy_Basic (Components|SkeletalMesh|GetAnimInstance (Variables|Default|GetSkeletalMesh))))
  (Default|StartAttack _asabp_enemy_basic)
  (CallFunction|Attack))