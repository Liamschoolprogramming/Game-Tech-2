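; Base gib explosion actor in the enemy gib effects, which bursts a Geometry Collection apart as soon as it spawns.
; BeginPlay applies a constant-falloff radial impulse at the collection's location and spawns the NS_Gib Niagara system there.
; After a short delay it destroys its Cube component, then sets a lifespan so the actor removes itself a few seconds later.
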(event EventBeginPlay
  (Physics|AddRadialImpulse (Variables|Default|GetGeometryCollection) (Transformation|GetWorldLocation (Variables|Default|GetGeometryCollection)) 1e+02 1e+04 "RIF_Constant" false)
  (Niagara|SpawnSystematLocation "/Game/Blueprints/Enemy/Gib_effect/NS_Gib.NS_Gib" (Transformation|GetWorldLocation (Variables|Default|GetGeometryCollection)))
  (Utilities|FlowControl|Delay 0.5)
  (Components|DestroyComponent (Variables|Default|GetCube))
  (Actor|SetLifeSpan 3.0))

(fn ConstructionScript)