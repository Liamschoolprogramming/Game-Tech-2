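; Strong enemy variant that can target crafting machines as well as cores.
; SetAttackTarget keeps a valid target half the time, otherwise picks a random crafting machine with health left, falling back to an active core, then navigates.
; FindNewAttackTarget flips between parent logic and any random machine, unfiltered by health, fed into SetAttackTarget.
; Sphere overlap with the target triggers Attack; ExecuteAttack also starts the ABP_Enemy_Strong attack animation.
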(event OnComponentBeginOverlap(Sphere)
  (params (OverlappedComponent :type Primitive%20Component%20Object%20Reference) (OtherActor :type Actor%20Object%20Reference) (OtherComp :type Primitive%20Component%20Object%20Reference) (OtherBodyIndex :type Integer) (bFromSweep :type Boolean) (SweepResult :type Hit%20Result%20Structure%20%28by%20ref%29))
  (if (== (Variables|Default|GetAttackTarget) OtherActor)
    (CallFunction|Attack)))

(event EventBeginPlay
  (|CallParentFunction) ; This node is disabled and will not be called.\nDrag off pins to build functionality.
)

(event EventSetAttackTarget
  (params (AttackTarget :type Actor%20Object%20Reference))
  (Utilities|IsValid AttackTarget
    (:Is%20Valid
      (if (== (Math|Random|RandomInteger 2) 0)
        (Variables|Default|SetAttackTarget AttackTarget)
        (CallFunction|NavigatetoAttackTarget)
        (else
          (bind _crafting_machine (CallFunction|GetRandomCraftingMachine :!label _label))
          (Utilities|IsValid _crafting_machine
            (:Is%20Valid
              (Variables|Default|SetAttackTarget _crafting_machine)
              (CallFunction|NavigatetoAttackTarget))
            (:Is%20Not%20Valid
              (bind _core (CallFunction|GetRandomActiveCore))
              (Variables|Default|SetAttackTarget _core)
              (CallFunction|NavigatetoAttackTarget))))))
    (:Is%20Not%20Valid
      (goto _label))))

(fn ConstructionScript
  (|CallParentFunction))

(fn ExecuteAttack
  (|CallParentFunction)
  (bind _asabp_enemy_strong (Utilities|Casting|CastToABP_Enemy_Strong (Components|SkeletalMesh|GetAnimInstance (Variables|Default|GetSkeletalMesh))))
  (Default|StartAttack _asabp_enemy_strong)
  (CallFunction|Attack))

(fn FindNewAttackTarget
  ;[0.15 0.15 0.15 0.5] 50/50 chance of finding a new core to attack or finding a machine
  (if (== (Math|Random|RandomInteger 2) 0)
    (|CallParentFunction)
    (else
      (bind _outactors (Actor|GetAllActorsOfClass "/Game/Blueprints/Machines/CraftingMachines/BP_CraftingMachine.BP_CraftingMachine_C"))
      (CallFunction|SetAttackTarget (Utilities|Array|Get(acopy) _outactors (Math|Random|RandomInteger (Utilities|Array|Length _outactors)))))))

(fn GetRandomCraftingMachine
  (bind _outactors (Actor|GetAllActorsOfClass "/Game/Blueprints/Machines/CraftingMachines/BP_CraftingMachine.BP_CraftingMachine_C"))
  (Utilities|Array|Shuffle _outactors)
  (for _array_element _outactors
    (if (> (Variables|/Game/Blueprints/Machines/MachineBaseClass/BP_Machine_Base.BP_Machine_Base_C|GetCurrentHealth _array_element) 0.0)
      (return _array_element)))
  (return 0))