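; Enemy spawn point that spawns enemies on a looping timer while spawning, registering itself and each enemy as observers of BP_LevelEventManager.
; Types come from a weighted random pick over a weight-keyed map, seeded only with Basic, and Mortar falls back to Basic without a free stand position.
; Basic and Restoration enemies target random active engine cores.
; Event notifications trigger retreat at wave end, cleanup on load, and boosting of new spawns during gauge overload.
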(event Custom|BeginSpawning
  ;[0.15 0.15 0.15 0.5] End enemy spawn cycle events
  (Variables|Default|SetSpawning true)
  (Utilities|Time|SetTimerbyFunctionName 0 "SpawnNewEnemy" (Variables|Default|GetSecondsDelayBetweenEnemies) true))

(event EventBeginPlay
  ;[0.15 0.15 0.15 0.5] Initializations
  (bind _returnvalue (Actor|GetActorOfClass "/Game/Blueprints/LevelEventManager/BP_LevelEventManager.BP_LevelEventManager_C"))
  (Variables|Default|SetLevelEventManager _returnvalue)
  (bind _asbpi_observer (Utilities|Casting|CastToBPI_Observer self))
  (Default|SubscribeObserver (Variables|Default|GetLevelEventManager) _asbpi_observer)
  (CallFunction|AddNewEnemyType "NewEnumerator0" 4e+01)
  (Variables|Default|SetSpawnTransform (Transformation|GetActorTransform self)))

(event EventOnNotify
  (params (EventType :type E_LevelEventType%20Enum :default "NewEnumerator0"))
  (switch Utilities|FlowControl|Switch|SwitchonE_LevelEventType EventType
    (:NewEnumerator3
      (CallFunction|EndSpawningandBeginRetreat))
    (:NewEnumerator7
      ;[0.15 0.15 0.15 0.5] Enemy cleanup when the game resets
      (Utilities|Time|ClearTimerbyFunctionName 0 "SpawnNewEnemy")
      (Variables|Default|SetSpawning false)
      (for _array_element (Variables|Default|GetEnemies)
        (bind _asbp_enemy (Utilities|Casting|CastToBP_Enemy _array_element))
        (Utilities|IsValid _asbp_enemy
          (:Is%20Valid
            (Default|UnsubscribeObserver (Variables|Default|GetLevelEventManager) _asbp_enemy)
            (Actor|DestroyActor _asbp_enemy)))))
    (:NewEnumerator10
      (Variables|Default|SetBoosted true))
    (:NewEnumerator11
      (Variables|Default|SetBoosted false))))

(fn ConstructionScript)

(fn SetActive
  (params (ActiveStatus :type Boolean))
  (Variables|Default|SetActive ActiveStatus))

(fn UnsubscribeObserver
  (params (Observer :type BP%20Enemy%20Object%20Reference))
  (Default|UnsubscribeObserver (Variables|Default|GetLevelEventManager) Observer))

(fn SpawnNewEnemy
  (bind _spawntransform (Variables|Default|GetSpawnTransform))
  (bind (_location _rotation _scale) (Math|Transform|BreakTransform _spawntransform))
  (if (Variables|Default|GetSpawning)
    (bind _enemytype (CallFunction|GetRandomEnemyType))
    (switch Utilities|FlowControl|Switch|SwitchonE_EnemyTypes _enemytype
      (:NewEnumerator0
        (bind _returnvalue (Game|SpawnActorfromClass "/Game/Blueprints/Enemy/BP_Enemy_Basic.BP_Enemy_Basic_C" (Variables|Default|GetSpawnTransform) "Undefined" "MultiplyWithRoot" 0 0))
        (bind _output_get (LocalVariables|SetL_NewEnemy _returnvalue))
        (bind _core (CallFunction|GetRandomActiveCore))
        (Default|SetAttackTarget _output_get _core))
      (:NewEnumerator1
        (bind _returnvalue_2 (Game|SpawnActorfromClass "/Game/Blueprints/Enemy/BP_Enemy_Strong.BP_Enemy_Strong_C" (Variables|Default|GetSpawnTransform) "Undefined" "MultiplyWithRoot" 0 0))
        (bind _output_get_2 (LocalVariables|SetL_NewEnemy _returnvalue_2))
        (Default|SetAttackTarget _output_get_2))
      (:NewEnumerator2
        (bind _returnvalue_3 (Game|SpawnActorfromClass "/Game/Blueprints/Enemy/BP_Enemy_Flying.BP_Enemy_Flying_C" (Math|Transform|MakeTransform (+ _location "0.000000,0.000000,300.000000") _rotation _scale) "Undefined" "MultiplyWithRoot" 0 0))
        (bind _output_get_3 (LocalVariables|SetL_NewEnemy _returnvalue_3))
        (Default|SetAttackTarget _output_get_3))
      (:NewEnumerator3
        (bind _returnvalue_4 (Game|SpawnActorfromClass "/Game/Blueprints/Enemy/BP_Enemy_Restoration.BP_Enemy_Restoration_C" (Variables|Default|GetSpawnTransform) "Undefined" "MultiplyWithRoot" 0 0))
        (bind _output_get_4 (LocalVariables|SetL_NewEnemy _returnvalue_4))
        (bind _core_2 (CallFunction|GetRandomActiveCore))
        (Default|SetAttackTarget _output_get_4 _core_2))
      (:NewEnumerator4
        (bind _returnvalue_5 (Game|SpawnActorfromClass "/Game/Blueprints/Enemy/BP_Enemy_Mortar.BP_Enemy_Mortar_C" (Variables|Default|GetSpawnTransform) "Undefined" "MultiplyWithRoot" 0 0))
        (bind _output_get_5 (LocalVariables|SetL_NewEnemy _returnvalue_5))
        (Default|SetAttackTarget _output_get_5)))
    (Utilities|Array|Add (Variables|Default|GetEnemies) (LocalVariables|GetL_NewEnemy))
    (Variables|/Game/Blueprints/Enemy/BP_Enemy.BP_Enemy_C|SetSpawner (LocalVariables|GetL_NewEnemy) self)
    (if (Variables|Default|GetBoosted)
      (Default|BoostAttackandSpeed (LocalVariables|GetL_NewEnemy) true 1.5))
    (bind _asbpi_observer (Utilities|Casting|CastToBPI_Observer (LocalVariables|GetL_NewEnemy)))
    (Default|SubscribeObserver (Variables|Default|GetLevelEventManager) _asbpi_observer)))

(fn EndSpawningandBeginRetreat
  (Utilities|Time|ClearTimerbyFunctionName 0 "SpawnNewEnemy")
  (Variables|Default|SetSpawning false)
  (for _array_element (Variables|Default|GetEnemies)
    (if (Utilities|IsValidInterface _array_element)
      (Default|Retreat _array_element (Transformation|GetActorTransform self)))))

(fn AddNewEnemyType
  (params (EnemyType :type E_EnemyTypes%20Enum :default "NewEnumerator0") (Weight :type Float%20%28double-precision%29))
  (Utilities|Map|Add (Variables|Default|GetEnemyTypes) Weight EnemyType))

(fn GetRandomEnemyType
  (bind _sum (CallFunction|SumOfSpawnOdds))
  (bind _chosen_index (CallFunction|DetermineSpawnIndex (Math|Random|RandomFloatinRange 0.0 _sum)))
  (if (Utilities|Enum|Equal(Enum) (.Value (Utilities|Map|GetKeyValueByIndex (Variables|Default|GetEnemyTypes) _chosen_index)) "NewEnumerator4")
    (bind _target (CallFunction|GetValidMortarStandPoints))
    (Utilities|IsValid _target
      (:Is%20Valid
        (return "NewEnumerator4"))
      (:Is%20Not%20Valid
        (return "NewEnumerator0")))
    (else
      (return (.Value (Utilities|Map|GetKeyValueByIndex (Variables|Default|GetEnemyTypes) _chosen_index))))))

(fn GetRandomActiveCore
  (bind _outactors (Actor|GetAllActorsOfClass "/Game/Blueprints/EngineCores/BP_EngineCore.BP_EngineCore_C"))
  (Utilities|Array|Shuffle _outactors)
  (for _array_element _outactors
    (if (Variables|/Game/Blueprints/EngineCores/BP_EngineCore.BP_EngineCore_C|GetIsActive _array_element)
      (if (> (Variables|/Game/Blueprints/EngineCores/BP_EngineCore.BP_EngineCore_C|GetHealth _array_element) 0.0)
        (return _array_element))))
  (return 0))

(fn SumOfSpawnOdds
  (bind _keys (Utilities|Map|Keys (Variables|Default|GetEnemyTypes)))
  (for _array_element _keys
    (LocalVariables|SetL_Sum (+ _array_element (LocalVariables|GetL_Sum))))
  (return (LocalVariables|GetL_Sum)))

(fn DetermineSpawnIndex
  (params (Random%20Value :type Float%20%28double-precision%29))
  (bind _keys (Utilities|Map|Keys (Variables|Default|GetEnemyTypes)))
  (for (_array_element _array_index) _keys
    (bind _output_get (LocalVariables|SetL_Sum (+ _array_element (LocalVariables|GetL_Sum))))
    (if (>= _output_get Random%20Value)
      (return _array_index))))

(fn GetValidMortarStandPoints
  (bind _outactors (Actor|GetAllActorsOfClass "/Game/Blueprints/Enemy/BP_MortarBug_StandPosition.BP_MortarBug_StandPosition_C"))
  (for _array_element _outactors
    (if (not (Variables|/Game/Blueprints/Enemy/BP_MortarBug_StandPosition.BP_MortarBug_StandPosition_C|GetInUse? _array_element))
      (return _array_element)))
  (return 0))