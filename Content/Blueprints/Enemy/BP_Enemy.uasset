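; Enemy character that navigates to an assigned target, faces it on a timer and damages it repeatedly once its sphere overlaps it.
; When an engine core or crafting machine target is destroyed, it switches to another active core.
; As an event observer, it retreats to a spawn point on wave end and scales speed and damage with pressure gauge overloads.
; Death unsubscribes it from its spawner and drops resources.
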(event OnComponentBeginOverlap(Sphere)
  (params (OverlappedComponent :type Primitive%20Component%20Object%20Reference) (OtherActor :type Actor%20Object%20Reference) (OtherComp :type Primitive%20Component%20Object%20Reference) (OtherBodyIndex :type Integer) (bFromSweep :type Boolean) (SweepResult :type Hit%20Result%20Structure%20%28by%20ref%29))
  ;[0.15 0.15 0.15 0.5] Attack
  (if (== (Variables|Default|GetAttackTarget) OtherActor)
    (CallFunction|Attack)))

(event Custom|NotifyOnSpawn
  (params (Event%20Type :type E_LevelEventType%20Enum :default "NewEnumerator0"))
  (switch Utilities|FlowControl|Switch|SwitchonE_LevelEventType Event%20Type
    (:NewEnumerator3
      (bind _returnvalue (Actor|GetActorOfClass "/Game/Blueprints/Enemy/BP_EnemySpawnPoint.BP_EnemySpawnPoint_C"))
      (CallFunction|Retreat (Transformation|GetActorTransform _returnvalue)))
    (:NewEnumerator10
      (CallFunction|BoostAttackandSpeed true 1.5))
    (:NewEnumerator11
      (CallFunction|BoostAttackandSpeed false 1.5))))

(event EventAttack
  ;[0.15 0.15 0.15 0.5] Attack
  (if (Variables|Default|GetAlive?)
    (Utilities|FlowControl|RetriggerableDelay 0.5)
    (CallFunction|ExecuteAttack)
    (CallFunction|Attack)))

(event EventNavigatetoAttackTarget
  ;[0.15 0.15 0.15 0.5] Moving and Navigation
  (if (Utilities|DoesObjectImplementInterface (Variables|Default|GetAttackTarget) "/Game/Team_Folders/Liam/BPI_Interactable.BPI_Interactable_C")
    (bind _location (Class|BPIInteractable|GetLocation(Message) (Variables|Default|GetAttackTarget)))
    (Utilities|Time|SetTimerbyFunctionName 0 "FaceTarget" 0.05 true)
    (AI|AIMoveTo self (.RandomLocation (AI|Navigation|GetRandomReachablePointinRadius _location 1e+01 0 0)) 0 1e+01 true)
    (else
      (Utilities|Time|SetTimerbyFunctionName 0 "FaceTarget" 0.05 true)
      (bind _randomlocation (Class|NavigationSystemV1|GetRandomLocationinNavigableRadius (Transformation|GetActorLocation (Variables|Default|GetAttackTarget)) 1e+01 0 0))
      (AI|AIMoveTo self _randomlocation 0 1e+01 true))))

(event Game|Damage|EventAnyDamage
  (params (Damage :type Float%20%28single-precision%29) (DamageType :type Damage%20Type%20Object%20Reference) (InstigatedBy :type Controller%20Object%20Reference) (DamageCauser :type Actor%20Object%20Reference))
  ;[0.15 0.15 0.15 0.5] Take Damage
  (CallFunction|OnTakeDamage Damage))

(event EventSetAttackTarget
  (params (AttackTarget :type Actor%20Object%20Reference))
  ;[0.15 0.15 0.15 0.5] Moving and Navigation
  (if (Variables|Default|GetAlive?)
    (Variables|Default|SetAttackTarget AttackTarget)
    (CallFunction|NavigatetoAttackTarget)))

(event EventRetreat
  (params (RetreatPoint :type Transform))
  ;[0.15 0.15 0.15 0.5] Retreat
  (AI|AIMoveTo self (.location RetreatPoint) 0 5.0 false
    (:then
      (Utilities|FlowControl|Delay 1.0)
      (Actor|DestroyActor))))

(event EventOnNotify
  (params (EventType :type E_LevelEventType%20Enum :default "NewEnumerator0"))
  (switch Utilities|FlowControl|Switch|SwitchonE_LevelEventType (stale Custom|NotifyOnSpawn Event%20Type)
    (:NewEnumerator3
      (bind _returnvalue (Actor|GetActorOfClass "/Game/Blueprints/Enemy/BP_EnemySpawnPoint.BP_EnemySpawnPoint_C"))
      (CallFunction|Retreat (Transformation|GetActorTransform _returnvalue)))
    (:NewEnumerator10
      (CallFunction|BoostAttackandSpeed true 1.5))
    (:NewEnumerator11
      (CallFunction|BoostAttackandSpeed false 1.5))))

(event EventBeginPlay
  (bind _returnvalue (Actor|GetActorOfClass "/Game/Blueprints/LevelEventManager/BP_LevelEventManager.BP_LevelEventManager_C"))
  (bind _output_get (Variables|Default|SetLevelEventManager _returnvalue))
  (CallFunction|NotifyonSpawn (Variables|/Game/Blueprints/LevelEventManager/BP_LevelEventManager.BP_LevelEventManager_C|GetLevelEventType _output_get)))

(fn ConstructionScript
  (Variables|Default|SetCurrentHealth (.basehp (Variables|Default|GetStats))))

(fn OnTakeDamage
  (params (DamageAmount :type Float%20%28double-precision%29))
  (if (Variables|Default|GetAlive?)
    (bind _output_get (Variables|Default|SetCurrentHealth (- (Variables|Default|GetCurrentHealth) DamageAmount)))
    (if (< _output_get 0.0)
      (CallFunction|Death))))

(fn FaceTarget
  (bind _returnvalue (Transformation|GetActorLocation))
  (bind _attacktarget (Variables|Default|GetAttackTarget))
  (bind _returnvalue_2 (Transformation|GetActorLocation _attacktarget))
  (bind _returnvalue_3 (Math|Rotator|FindLookatRotation _returnvalue _returnvalue_2))
  (bind (_roll _pitch _yaw) (Math|Rotator|BreakRotator _returnvalue_3))
  (if (Variables|Default|GetAlive?)
    (Transformation|SetWorldRotation (Variables|Collision|GetCapsuleComponent) (Math|Rotator|MakeRotator _roll 0.0 _yaw) false false)))

(fn Death
  (bind _resource_drop (Variables|Default|GetResource%20Drop))
  (Components|Movement|StopMovementImmediately (Variables|Character|GetCharacterMovement))
  (Variables|Default|SetAlive? false)
  (Default|UnsubscribeObserver (Variables|Default|GetSpawner) self)
  (for _index (range 1 (.amount _resource_drop))
    (Game|SpawnActorfromClass :Class "/Game/Blueprints/BP_ResourceDrop.BP_ResourceDrop_C" :SpawnTransform (Transformation|GetActorTransform) :CollisionHandlingOverride "Undefined" :TransformScaleMethod "MultiplyWithRoot" :Resouce%20Name (.name _resource_drop) :Instigator 0))
  (Actor|DestroyActor))

(fn BoostAttackandSpeed
  (params (boost? :type Boolean) (Amplifier :type Float%20%28double-precision%29))
  (bind _charactermovement (Variables|Character|GetCharacterMovement))
  (if boost?
    (Variables|/Script/Engine.CharacterMovementComponent|SetMaxWalkSpeed _charactermovement (* (Class|MovementComponent|GetMaxSpeed _charactermovement) Amplifier))
    (Variables|Default|SetStats (Utilities|Struct|MakeStruct_EnemyStats (.basehp (Variables|Default|GetStats)) (* (.basedamage (Variables|Default|GetStats)) Amplifier)))
    (else
      (Variables|/Script/Engine.CharacterMovementComponent|SetMaxWalkSpeed _charactermovement (/ (Class|MovementComponent|GetMaxSpeed _charactermovement) Amplifier))
      (Variables|Default|SetStats (Utilities|Struct|MakeStruct_EnemyStats (.basehp (Variables|Default|GetStats)) (/ (.basedamage (Variables|Default|GetStats)) Amplifier))))))

(fn ExecuteAttack
  (bind _attacktarget (Variables|Default|GetAttackTarget))
  (Game|Damage|ApplyDamage (Variables|Default|GetAttackTarget) (.basedamage (Variables|Default|GetStats)) 0 0)
  (bind _asbp_engine_core (Utilities|Casting|CastToBP_EngineCore _attacktarget)
    (:then
      (if (<= (Variables|/Game/Blueprints/EngineCores/BP_EngineCore.BP_EngineCore_C|GetHealth _asbp_engine_core) 0.0)
        (CallFunction|FindNewAttackTarget :!label _label)))
    (:CastFailed
      (bind _asbp_crafting_machine (Utilities|Casting|CastToBP_CraftingMachine _attacktarget))
      (if (<= (Variables|/Game/Blueprints/Machines/MachineBaseClass/BP_Machine_Base.BP_Machine_Base_C|GetCurrentHealth _asbp_crafting_machine) 0.0)
        (goto _label)))))

(fn FindNewAttackTarget
  (bind _outactors (Actor|GetAllActorsOfClass "/Game/Blueprints/EngineCores/BP_EngineCore.BP_EngineCore_C"))
  (for _array_element _outactors
    (if (Variables|/Game/Blueprints/EngineCores/BP_EngineCore.BP_EngineCore_C|GetIsActive _array_element)
      (if (!= _array_element (Variables|Default|GetAttackTarget))
        (CallFunction|SetAttackTarget _array_element)
        (return)))))

(fn GetEnemyCurrentHP
  (return (Variables|Default|GetCurrentHealth)))