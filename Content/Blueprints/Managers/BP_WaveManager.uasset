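; BP_WaveManager is a manager that alternates timed enemy waves with countdown breaks between them.
; On BeginPlay it spawns a save manager, creates the wave timer widget, and activates and registers only the "bridge" spawn point.
; Self-rescheduling timers drive the cycle, starting and ending spawning on registered points while updating the widget.
; Each break autosaves inside the spawn-point loop and, after a short delay, alerts the level event manager.
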(event Custom|SetWaveActive
  (Default|SetWaveActiveText (Variables|Default|GetTimerWidget))
  (for _array_element (Variables|Default|GetEnemySpawnPoints)
    (Utilities|IsValid _array_element
      (:Is%20Valid
        (Default|BeginSpawning _array_element))))
  (Utilities|Time|SetTimerbyEvent (delegate Custom|StartWaveTimer) (Math|Conversions|ToFloat(Integer) (Variables|Default|GetWaveDurationSeconds))))

(event Custom|StartWaveTimer
  (for _array_element (Variables|Default|GetEnemySpawnPoints)
    (Utilities|IsValid _array_element
      (:Is%20Valid
        (Default|EndSpawning _array_element)
        ;[0.15 0.15 0.15 0.5] Autosave
        (Default|SavetheGame (Variables|Default|GetSaveManager)))))
  (Default|SetWaveNotActiveText (Variables|Default|GetTimerWidget) (Variables|Default|GetSecondsBetweenWaves))
  (Variables|Default|SetTimeRemaining (Variables|Default|GetSecondsBetweenWaves))
  (Utilities|FlowControl|Delay 1.0)
  (CallFunction|CountdowntoWave)
  (Default|AlertWaveEnded (Variables|Default|GetLevelEventManager)))

(event Custom|CountdownToWave
  (bind _output_get (Variables|Default|SetTimeRemaining (- (Variables|Default|GetTimeRemaining) 1)))
  (if (<= _output_get 0)
    (CallFunction|SetWaveActive)
    (else
      (Default|SetTimeRemainingValue (Variables|Default|GetTimerWidget) _output_get)
      (Utilities|Time|SetTimerbyEvent (delegate Custom|CountdownToWave) 1.0))))

(event EventBeginPlay
  (bind _returnvalue (Game|SpawnActorfromClass "/Game/Blueprints/Managers/BP_SaveManager.BP_SaveManager_C" (Transformation|GetActorTransform) "Undefined" "MultiplyWithRoot" 0 0))
  (Variables|Default|SetSaveManager _returnvalue)
  (bind _returnvalue_2 (UserInterface|CreateWidget "/Game/UI/WidgetBlueprints/W_WaveTimer.W_WaveTimer_C"))
  (UserInterface|Viewport|AddtoViewport _returnvalue_2 0)
  (Class|UserWidget|SetPositioninViewport _returnvalue_2 (Math|Vector2D|MakeVector2D (* (.x (Viewport|GetViewportSize)) 0.75) 1e+01) true)
  (Variables|Default|SetTimerWidget _returnvalue_2)
  (bind _returnvalue_3 (Actor|GetActorOfClass "/Game/Blueprints/LevelEventManager/BP_LevelEventManager.BP_LevelEventManager_C"))
  (Variables|Default|SetLevelEventManager _returnvalue_3)
  (bind _outactors (Actor|GetAllActorsOfClass "/Game/Blueprints/Enemy/BP_EnemySpawnPoint.BP_EnemySpawnPoint_C"))
  (for _array_element _outactors
    ;[0.15 0.15 0.15 0.5] INITIALIZATION: Set all spawn points to inactive except for bridge spawn point, add ref to bridge spawn point to EnemySpawnPoints array
    (Default|SetActive _array_element (== (Variables|/Game/Blueprints/Enemy/BP_EnemySpawnPoint.BP_EnemySpawnPoint_C|GetName _array_element) (Utilities|Name|MakeLiteralName "bridge")))
    (if (== (Variables|/Game/Blueprints/Enemy/BP_EnemySpawnPoint.BP_EnemySpawnPoint_C|GetName _array_element) (Utilities|Name|MakeLiteralName "bridge"))
      (Utilities|Array|Add (Variables|Default|GetEnemySpawnPoints) _array_element)))
  (CallFunction|StartWaveTimer))

(fn ConstructionScript)