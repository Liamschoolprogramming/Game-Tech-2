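; BP_SaveManager handles saving and loading the game to a slot named by the FileName held in BP_GameInstance.
; LoadTheGame stores the loaded BP_SaveGame in the GameInstance's SaveVar, or calls SaveTheGame when no file exists.
; SaveTheGame creates a save object if SaveVar is invalid, records each BP_EngineCore's health in a map keyed by actor name, then writes it to the slot.
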(event Custom|SaveTheGame
  ;[0.15 0.15 0.15 0.5] Save
  ;;[0.15 0.15 0.15 0.5] Save File differentiation
  (bind _asbp_game_instance (Utilities|Casting|CastToBP_GameInstance (Game|GetGameInstance)))
  (bind _output_get (Variables|Default|SetFile%20Name (Variables|/Game/Blueprints/Managers/BP_GameInstance.BP_GameInstance_C|GetFile%20Name _asbp_game_instance)))
  (Utilities|FlowControl|Sequence
    (:then_0
      (Utilities|IsValid (Variables|/Game/Blueprints/Managers/BP_GameInstance.BP_GameInstance_C|GetSaveVar _asbp_game_instance)
        (:Is%20Not%20Valid
          (bind _returnvalue (SaveGame|CreateSaveGameObject "/Game/Team_Folders/Gordon/BP_SaveGame.BP_SaveGame_C"))
          (Variables|/Game/Blueprints/Managers/BP_GameInstance.BP_GameInstance_C|SetSaveVar _asbp_game_instance _returnvalue))))
    (:then_1
      ;;[0.15 0.15 0.15 0.5] Save Core Health
      (bind _outactors (Actor|GetAllActorsOfClass "/Game/Blueprints/EngineCores/BP_EngineCore.BP_EngineCore_C"))
      ;;;[0.15 0.15 0.15 0.5] Loop through all 3 Cores
      (for _array_element _outactors
        (Utilities|Map|Add (Variables|Default|GetCoreHealths) (Variables|/Game/Blueprints/EngineCores/BP_EngineCore.BP_EngineCore_C|GetName _array_element) (Variables|/Game/Blueprints/EngineCores/BP_EngineCore.BP_EngineCore_C|GetHealth _array_element)))
      (Variables|/Game/Team_Folders/Gordon/BP_SaveGame.BP_SaveGame_C|SetCoreHealths (Variables|/Game/Blueprints/Managers/BP_GameInstance.BP_GameInstance_C|GetSaveVar _asbp_game_instance) (Variables|Default|GetCoreHealths)))
    (:then_2
      (SaveGame|SaveGametoSlot (Variables|/Game/Blueprints/Managers/BP_GameInstance.BP_GameInstance_C|GetSaveVar _asbp_game_instance) _output_get))))

(event Custom|LoadTheGame
  ;[0.15 0.15 0.15 0.5] Load
  ;;[0.15 0.15 0.15 0.5] Save File Differentiation
  (bind _asbp_game_instance (Utilities|Casting|CastToBP_GameInstance (Game|GetGameInstance)))
  (bind _output_get (Variables|Default|SetFile%20Name (Variables|/Game/Blueprints/Managers/BP_GameInstance.BP_GameInstance_C|GetFile%20Name _asbp_game_instance)))
  (bind _returnvalue (SaveGame|DoesSaveGameExist _output_get))
  (if _returnvalue
    (bind _returnvalue_2 (SaveGame|LoadGamefromSlot _output_get))
    (bind _asbp_game_instance_2 (Utilities|Casting|CastToBP_GameInstance (Game|GetGameInstance)))
    (bind _asbp_save_game (Utilities|Casting|CastToBP_SaveGame _returnvalue_2))
    (Variables|/Game/Blueprints/Managers/BP_GameInstance.BP_GameInstance_C|SetSaveVar _asbp_game_instance_2 _asbp_save_game)
    (else
      (CallFunction|SavetheGame))))

(fn ConstructionScript)