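; Manager for overgrown-area hazards, prototyping an oxygen-depletion event tied to destroyed walls.
; StartHazardEvent prints warnings and starts a looping timer, while GameOver stops it and prints a message once oxygen is depleted.
; Functions count destroyed walls, register entry points, recalculate oxygen from the wall count and pick random attack or spawn locations.
; An event spawns enemy spawn points at hazards; much other wiring is disconnected, with empty StartEvent and OnNotify handlers.
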(event Custom|StartEvent)

(event Custom|SpawnEnemySpawnPoint
  (params (OvergrownAreaHazard :type BP%20Hazard%20Over%20Grown%20Area%20Object%20Reference))
  (Game|SpawnActorfromClass "/Game/Blueprints/Enemy/BP_EnemySpawnPoint.BP_EnemySpawnPoint_C" (Transformation|GetActorTransform OvergrownAreaHazard) "Undefined" "MultiplyWithRoot" 0 0))

(event Custom|StartHazardEvent
  (Development|PrintString "WARNING" true true "(R=1.000000,G=0.000000,B=0.000000,A=1.000000)")
  (Development|PrintString "OXYGEN IS DEPLETING" true true "(R=1.000000,G=0.512895,B=0.000000,A=1.000000)")
  (bind _returnvalue (Utilities|Time|SetTimerbyEvent (EventDispatchers|CreateEvent :!event DepletefromMeter) (Variables|Default|GetReductionSpeed) true))
  (Variables|Default|SetTimer _returnvalue))

(event Custom|GameOver
  (if (Variables|Default|GetIsOxygenDepleted)
    (Utilities|Time|ClearandInvalidateTimerbyHandle (Variables|Default|GetTimer))
    (Development|PrintString "Game over")))

(event EventOnNotify
  (params (EventType :type E_LevelEventType%20Enum :default "NewEnumerator0"))
  (switch Utilities|FlowControl|Switch|SwitchonE_LevelEventType EventType))

(event EventBeginPlay
  (|CallParentFunction))

(fn ConstructionScript)

(fn WallHazard
  (Math|Integer|IncrementInt (Variables|Default|GetDestroyedWalls)
    (:%20%20
      (Development|PrintString (Utilities|String|Append (Utilities|String|ToString(Integer) (Variables|Default|GetDestroyedWalls)) " walls"))
      (if (== (Variables|Default|GetDestroyedWalls) (Variables|Default|GetStartEventAmount))
        _))))

(fn AddtoArray
  (params (Object :type BP%20Hazard%20Over%20Grown%20Area%20Object%20Reference))
  (bind _returnvalue (Utilities|Array|Add (Variables|Default|GetEntryPoints) Object))
  (Utilities|IsValid (Utilities|Array|Get(acopy) (Variables|Default|GetEntryPoints) _returnvalue)
    (:Is%20Valid
      (Development|PrintString (Utilities|GetDisplayName (Utilities|Array|Get(acopy) (Variables|Default|GetEntryPoints) _returnvalue))))))

(fn GetAttackPointLocation
  (bind _returnvalue (Transformation|GetWorldLocation (Variables|/Game/Blueprints/Hazards/BP_Hazard_OverGrownArea.BP_Hazard_OverGrownArea_C|GetAttackPoint (Utilities|Array|Get(acopy) (Variables|Default|GetEntryPoints) (Math|Random|RandomInteger (Utilities|Array|Length (Variables|Default|GetEntryPoints)))))))
  (return _returnvalue))

(fn GetEnemySpawnPoint
  (bind _returnvalue (Transformation|GetWorldLocation (Variables|/Game/Blueprints/Hazards/BP_Hazard_OverGrownArea.BP_Hazard_OverGrownArea_C|GetEnemySpawnPointLocation (Utilities|Array|Get(acopy) (Variables|Default|GetEntryPoints) (Math|Random|RandomInteger (Utilities|Array|Length (Variables|Default|GetEntryPoints)))))))
  (return _returnvalue))

(fn DepletefromMeter
  (if (!= (Variables|Default|GetDestroyedWalls) 0)
    (Variables|Default|SetOxygenAmount (- (* 1 (Variables|Default|GetDestroyedWalls)) (Variables|Default|GetOxygenAmount)))
    (Development|PrintString (Utilities|String|ToString(Integer) (Variables|Default|GetOxygenAmount)))
    (if (== (Variables|Default|GetOxygenAmount) 0)
      (Utilities|Time|ClearandInvalidateTimerbyHandle (Variables|Default|GetTimer))
      (CallFunction|GameOver))
    (else
      (Variables|Default|SetOxygenAmount (Variables|Default|GetMaxOxygen))
      (Utilities|Time|ClearandInvalidateTimerbyHandle (Variables|Default|GetTimer)))))