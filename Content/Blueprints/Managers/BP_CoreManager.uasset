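; BP_CoreManager is a manager that sets up the engine cores and triggers game over when too many are inactive.
; On BeginPlay it activates only the BP_EngineCore named "bridge" and stores it in EngineCores.
; CoreStatusCheck rescans all cores, adding inactive ones to InactiveCores without resetting it, and shows the GameOverWidget once that count reaches the threshold of three.
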(event Custom|CoreStatusCheck
  (bind _outactors (Actor|GetAllActorsOfClass "/Game/Blueprints/EngineCores/BP_EngineCore.BP_EngineCore_C"))
  (for _array_element _outactors
    (if (not (Variables|/Game/Blueprints/EngineCores/BP_EngineCore.BP_EngineCore_C|GetIsActive _array_element))
      (Variables|Default|SetInactiveCores (+ (Variables|Default|GetInactiveCores) 1))))
  (if (>= (Variables|Default|GetInactiveCores) 3)
    (bind _returnvalue (UserInterface|CreateWidget "/Game/Team_Folders/Gordon/GameOverWidget.GameOverWidget_C"))
    (UserInterface|Viewport|AddtoViewport _returnvalue 0)))

(event EventBeginPlay
  (bind _outactors (Actor|GetAllActorsOfClass "/Game/Blueprints/EngineCores/BP_EngineCore.BP_EngineCore_C"))
  (for _array_element _outactors
    ;[0.15 0.15 0.15 0.5] INITIALIZATION: Set all cores to inactive except for bridge core, add ref to bridge core to EngineCores array
    (Default|SetActive _array_element (Utilities|Enum|Equal(Enum) (Variables|/Game/Blueprints/EngineCores/BP_EngineCore.BP_EngineCore_C|GetName _array_element) "bridge"))
    (if (Utilities|Enum|Equal(Enum) (Variables|/Game/Blueprints/EngineCores/BP_EngineCore.BP_EngineCore_C|GetName _array_element) "bridge")
      (Utilities|Array|Add (Variables|Default|GetEngineCores) _array_element))))

(fn ConstructionScript)