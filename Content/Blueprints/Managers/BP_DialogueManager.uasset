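; Dialogue manager that runs the game's opening tutorial aboard the Synthera, in either a full cutscene or simplified version.
; Writes line arrays into WB_DialogueBox while locking player movement, then uses a numbered stage switch on text completion to trigger the next step.
; The full version steers attention with camera moves, an indicator arrow and look-at rotation, and polls timers for Gel crafting, Furnace repair and Astral Ingot possession.
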(event Custom|WaitForPlayerToCraftGel
  (if (> (.Value (Utilities|Map|Find (Variables|/Game/Blueprints/Components/BP_Inventory.BP_Inventory_C|GetResource%20Inventory (Variables|/Game/Blueprints/Player/BP_FPCharacter.BP_FPCharacter_C|GetBP_Inventory (Variables|Default|GetPlayer))) "Gel")) 0)
    (if (Widget|IsVisible (Variables|/Game/Blueprints/Player/BP_FPCharacter.BP_FPCharacter_C|GetReticle (Variables|Default|GetPlayer)))
      (CallFunction|DisplayDialogue (Utilities|Array|MakeArray "Now that you have Gel, walk up to the Furnace and apply it by holding R.") false 8)
      (Utilities|Time|ClearandInvalidateTimerbyHandle (Variables|Default|GetWaitingTimer)))))

(event Custom|WaitForPlayerToRepairFurnace
  (bind _tutorial_furnace (CallFunction|GetTutorialFurnace))
  (if (> (Variables|/Game/Blueprints/Machines/MachineBaseClass/BP_Machine_Base.BP_Machine_Base_C|GetCurrentHealth _tutorial_furnace) 0.0)
    (if (Widget|IsVisible (Variables|/Game/Blueprints/Player/BP_FPCharacter.BP_FPCharacter_C|GetReticle (Variables|Default|GetPlayer)))
      (CallFunction|DisplayDialogue (Utilities|Array|MakeArray "Excellent! Now the Furnace should be up and running again." "To use the Furnace, press E to open the machine terminal. Deposit resources into the Furnace to craft new resources, such as Astral Ingots." "Celestial Ore can be hand crafted, like Gel. It can also be produced in a Compressor.") false 9)
      (Utilities|FlowControl|Delay 0.1)
      (CallFunction|HideInputPrompt)
      (Utilities|Time|ClearandInvalidateTimerbyHandle (Variables|Default|GetWaitingTimer)))))

(event Custom|Add%20All%20Recipes%20%28Gold%29
  (bind _outrownames (DataTable|GetDataTableRowNames "/Game/Blueprints/DT_Recipes.DT_Recipes"))
  (for _array_element _outrownames
    (switch name _array_element
      (:Default
        (Class|BPIGameInstance|AddorRemovePlayerRecipe(Message) (Game|GetGameInstance) _array_element true)))))

(event Custom|DisplayDialogue
  (params (TextToWrite :type Array%20of%20Strings) (EnableMovement? :type Boolean) (CutsceneStage :type Integer))
  (Variables|Default|SetText%20to%20Write TextToWrite)
  (Variables|Default|SetCutSceneStages CutsceneStage)
  (Variables|Default|SetIndex 0)
  (CallFunction|HideInputPrompt)
  (CallFunction|AddtoView)
  (CallFunction|EnableMovement EnableMovement?)
  (Default|WriteOutText (Variables|Default|GetDialogueBox) (Utilities|Array|Get(acopy) (Variables|Default|GetText%20to%20Write) (Variables|Default|GetIndex))))

(event Custom|WaitForPlayerToHaveAstralIngot
  (if (> (.Value (Utilities|Map|Find (Variables|/Game/Blueprints/Components/BP_Inventory.BP_Inventory_C|GetResource%20Inventory (Variables|/Game/Blueprints/Player/BP_FPCharacter.BP_FPCharacter_C|GetBP_Inventory (Variables|Default|GetPlayer))) "Astral Ingot")) 0)
    (bind _tutorial_furnace (CallFunction|GetTutorialFurnace))
    (if (> (Variables|/Game/Blueprints/Machines/MachineBaseClass/BP_Machine_Base.BP_Machine_Base_C|GetCurrentHealth _tutorial_furnace) 0.0)
      (if (not (or (UserInterface|Viewport|IsinViewport (Variables|/Game/Blueprints/Machines/MachineBaseClass/BP_Machine_Base.BP_Machine_Base_C|GetMenu%20Widget _tutorial_furnace)) (UserInterface|Viewport|IsinViewport (Variables|/Game/Blueprints/Player/BP_FPCharacter.BP_FPCharacter_C|GetInventoryUI (Variables|Default|GetPlayer)))))
        (bind _tutorial_objective (CallFunction|GetTutorialObjective))
        (Transformation|SetActorLocation (Variables|Default|GetArrow) (+ (Transformation|GetActorLocation _tutorial_objective) "0.000000,0.000000,350.000000") false false)
        (CallFunction|DisplayDialogue (Utilities|Array|MakeArray "Now you have the means to procure all the necessary resources to repair the Main Core.") false 10)
        (Utilities|FlowControl|Delay 0.1)
        (CallFunction|HideInputPrompt)
        (Utilities|Time|ClearandInvalidateTimerbyHandle (Variables|Default|GetWaitingTimer))))))

(event Custom|Start%20Tutorial%20Cutscene
  (bind _tutorial_furnace (CallFunction|GetTutorialFurnace))
  (Variables|/Game/Blueprints/Machines/MachineBaseClass/BP_Machine_Base.BP_Machine_Base_C|SetCurrentHealth _tutorial_furnace 0.0)
  (Variables|/Game/Blueprints/Machines/MachineBaseClass/BP_Machine_Base.BP_Machine_Base_C|SetOperational%20State _tutorial_furnace "NewEnumerator1")
  (Default|UpdateStatus _tutorial_furnace)
  (bind _returnvalue (UserInterface|CreateWidget "/Game/UI/WidgetBlueprints/WB_DialogueBox.WB_DialogueBox_C" (Game|GetPlayerController 0)))
  (Variables|Default|SetDialogueBox _returnvalue)
  (bind _asbp_fpcharacter (Utilities|Casting|CastToBP_FPCharacter (Game|Player|GetPlayerPawn 0)))
  (Variables|Default|SetPlayer _asbp_fpcharacter)
  (Utilities|FlowControl|DelayUntilNextTick)
  (CallFunction|DisplayDialogue (Utilities|Array|MakeArray "Welcome aboard the Synthera. I am the Synthera Interactive Diagnostics Emergecy Response System, your assistant, and your only hope of survival." "To speak in the plainest of terms, you are the only significant life form remaining on this ship." "The ship has suffered major damage. Main Core Power remaining: 10% - Alternate Core Power 0% - Synthera Condition: CRITICAL" "But not all hope is lost. I will guide you through the steps to repairing this vessel." "Let's start with the basics. Do you see that core over there?") false 1)
  (bind _bp_game_instance (Class|BPIGameInstance|GetBPGameInstanceRef(Message) (Game|GetGameInstance)))
  (EventDispatchers|BindEventtoOnTextCompleted _bp_game_instance (delegate Custom|TextCompleted)))

(event Custom|Move%20Camera
  (params (MoveDistance :type Vector))
  (bind _zoomy (Timeline|Zoom%20Camera PlayFromStart)
    (:Update
      (Transformation|SetWorldLocation (Variables|/Game/Blueprints/Player/BP_FPCharacter.BP_FPCharacter_C|GetFirstPersonCamera (Variables|Default|GetPlayer)) (+ (* _zoomy MoveDistance) (Transformation|GetWorldLocation (Variables|/Game/Blueprints/Player/BP_FPCharacter.BP_FPCharacter_C|GetFirstPersonCamera (Variables|Default|GetPlayer)))) false false))))

(event Custom|Simple%20Text%20Completed
  (if (Variables|Default|GetSimplified%20Tutorial)
    (switch int (Variables|Default|GetCutSceneStages)
      (:1
        (Camera|SetFieldOfView (Variables|/Game/Blueprints/Player/BP_FPCharacter.BP_FPCharacter_C|GetFirstPersonCamera (Variables|Default|GetPlayer)) 3e+01)
        (CallFunction|DisplayDialogue (Utilities|Array|MakeArray "This is the Main Core of the Synthera. It is absolutely vital to your survival! Without it, all systems will fail, and the ship will likely explode." " Your chances of survival would be reduced to 0%. You must defend the Main Core at all costs.") false 2))
      (:2
        (Camera|SetFieldOfView (Variables|/Game/Blueprints/Player/BP_FPCharacter.BP_FPCharacter_C|GetFirstPersonCamera (Variables|Default|GetPlayer)) 9e+01)
        (Default|SetImageVisibility (Variables|Default|GetDialogueBox) true "/Game/UI/Tutorial/ObjectiveImage.ObjectiveImage")
        (CallFunction|DisplayDialogue (Utilities|Array|MakeArray "The Synthera has undergone Lockdown Protocol. In order to access the rest of the ship and restore it to an operation state, you must deliver the requested materials to each of the ship's terminals." "Unlocking these terminals will also make new crafting recipes available to you.") false 3))
      (:3
        (Default|SetImageVisibility (Variables|Default|GetDialogueBox) false)
        (CallFunction|DisplayDialogue (Utilities|Array|MakeArray "There is one other crucial detail. " "You are not alone out here in space. My sensors detect lifeforms approaching." "You have two and a half minutes.") false 4)
        (CallFunction|AddAllRecipes(Gold)))
      (:4
        (CallFunction|EnableMovement true)
        (CallFunction|ReDisplayInputPrompt)
        (Default|TutorialCompleted (Variables|Default|GetLevel%20Event%20Manager))))))

(event Custom|Begin%20Tutorial
  (bind _returnvalue (Actor|GetActorOfClass "/Game/Blueprints/LevelEventManager/BP_LevelEventManager.BP_LevelEventManager_C"))
  (Variables|Default|SetLevel%20Event%20Manager _returnvalue)
  (if (Variables|Default|GetSimplified%20Tutorial)
    (CallFunction|StartSimplifiedTutorial)
    (else
      (CallFunction|StartTutorialCutscene)
      (bind _returnvalue_2 (Game|SpawnActorfromClass "/Game/Blueprints/BP_IndicatorArrow.BP_IndicatorArrow_C" (Math|Transform|MakeTransform "0, 0, 0" "0, 0, 0" "1.000000,1.000000,1.000000") "Undefined" "MultiplyWithRoot" 0 0))
      (bind _output_get (Variables|Default|SetArrow _returnvalue_2))
      (Rendering|SetVisibility (Variables|/Game/Blueprints/BP_IndicatorArrow.BP_IndicatorArrow_C|GetCone _output_get) false false))))

(event Custom|Start%20Simplified%20Tutorial
  (bind _returnvalue (UserInterface|CreateWidget "/Game/UI/WidgetBlueprints/WB_DialogueBox.WB_DialogueBox_C" (Game|GetPlayerController 0)))
  (Variables|Default|SetDialogueBox _returnvalue)
  (bind _asbp_fpcharacter (Utilities|Casting|CastToBP_FPCharacter (Game|Player|GetPlayerPawn 0)))
  (Variables|Default|SetPlayer _asbp_fpcharacter)
  (Utilities|FlowControl|DelayUntilNextTick)
  (CallFunction|DisplayDialogue (Utilities|Array|MakeArray "Welcome aboard the Synthera. I am the Synthera Interactive Diagnostics Emergecy Response System, your assistant, and your only hope of survival." "To speak in the plainest of terms, you are the only significant life form remaining on this ship." "The ship has suffered major damage. Main Core Power remaining: 10% - Alternate Core Power 0% - Synthera Condition: CRITICAL" "But not all hope is lost. I will guide you through the steps to repairing this vessel." "Let's start with the basics. Do you see that core over there?") false 1)
  (bind _bp_game_instance (Class|BPIGameInstance|GetBPGameInstanceRef(Message) (Game|GetGameInstance)))
  (EventDispatchers|BindEventtoOnTextCompleted _bp_game_instance (delegate Custom|Simple%20Text%20Completed)))

(event Custom|TextCompleted
  (bind _arrow (Variables|Default|GetArrow))
  (if (not (Variables|Default|GetSimplified%20Tutorial))
    (switch int (Variables|Default|GetCutSceneStages)
      (:1
        (CallFunction|MoveCamera "0.000000,-85.000000,0.000000")
        (Utilities|FlowControl|Delay 1.5)
        (CallFunction|DisplayDialogue (Utilities|Array|MakeArray "This is the Main Core of the Synthera. It is absolutely vital to your survival! Without it, all systems will fail, and the ship will likely explode. Your chances of survival would be reduced to 0%." "At the moment, the Main Core is operating at 50% output speed. To begin your repairs of the ship, your first goal should be to repair the Main Core.") false 2))
      (:2
        (CallFunction|MoveCamera "-20.000000,-35.000000,0.000000")
        (Utilities|FlowControl|Delay 1.5)
        (CallFunction|DisplayDialogue (Utilities|Array|MakeArray "That terminal over there is the Backup Generator. It possess the power you need to restore the Main Core to a self-reliant state." "You'll have to procure the resources it needs and deposit them into the Generator." "Examine the Generator to see what resources must be procured. Press E to interact with machines, cores,  and devices.") false 3))
      (:3
        (CallFunction|MoveCamera "20.000000,120.000000,0.000000")
        (Utilities|FlowControl|Delay 2.0)
        (CallFunction|EnableMovement true)
        (CallFunction|ReDisplayInputPrompt)
        (bind _tutorial_objective (CallFunction|GetTutorialObjective))
        (Transformation|SetActorLocation _arrow (+ (Transformation|GetActorLocation _tutorial_objective) "0.000000,0.000000,350.000000") false false)
        (Rendering|SetVisibility (Variables|/Game/Blueprints/BP_IndicatorArrow.BP_IndicatorArrow_C|GetCone _arrow) true false))
      (:4
        (bind _location (CallFunction|GetMainCore))
        (Transformation|SetActorLocation (Variables|Default|GetArrow) (+ _location "0.000000,0.000000,350.000000") false false)
        (bind _returnvalue (Utilities|Time|SetTimerbyFunctionName 0 "RotateToArrow" 0.01 true))
        (Variables|Default|SetLookAtTimer _returnvalue)
        (Utilities|FlowControl|Delay 1.0)
        (CallFunction|DisplayDialogue (Utilities|Array|MakeArray "The Main Core produces Star Dust as a waste product when it generates power." "Even in the state it's in, it will still be producing Star Dust as we speak." "Gather Star Dust from the Main Core and deposit it into the Backup Generator terminal.") false 5))
      (:5
        (CallFunction|EnableMovement true)
        (CallFunction|ReDisplayInputPrompt))
      (:6
        (bind _tutorial_furnace (CallFunction|GetTutorialFurnace))
        (Transformation|SetActorLocation (Variables|Default|GetArrow) (+ (Transformation|GetActorLocation _tutorial_furnace) "0.000000,0.000000,350.000000") false false)
        (bind _returnvalue_2 (Utilities|Time|SetTimerbyFunctionName 0 "RotateToArrow" 0.01 true))
        (Variables|Default|SetLookAtTimer _returnvalue_2)
        (Utilities|FlowControl|Delay 1.0)
        (CallFunction|DisplayDialogue (Utilities|Array|MakeArray "This Furnace appears to be badly damaged. It will need to be repaired before it can be used." "Most machines can be mended by using Gel." "You can craft Gel yourself. Press I to open your inventory and craft Gel.") false 7))
      (:7
        (CallFunction|EnableMovement true)
        (bind _returnvalue_3 (Utilities|Time|SetTimerbyEvent (delegate Custom|WaitForPlayerToCraftGel) 0.2 true))
        (Variables|Default|SetWaitingTimer _returnvalue_3)
        (CallFunction|ReDisplayInputPrompt))
      (:8
        (CallFunction|EnableMovement true)
        (bind _returnvalue_4 (Utilities|Time|SetTimerbyEvent (delegate Custom|WaitForPlayerToRepairFurnace) 0.2 true))
        (Variables|Default|SetWaitingTimer _returnvalue_4)
        (CallFunction|ReDisplayInputPrompt))
      (:9
        (CallFunction|EnableMovement true)
        (CallFunction|ReDisplayInputPrompt)
        (bind _returnvalue_5 (Utilities|Time|SetTimerbyEvent (delegate Custom|WaitForPlayerToHaveAstralIngot) 0.2 true))
        (Variables|Default|SetWaitingTimer _returnvalue_5))
      (:10
        (CallFunction|EnableMovement true)
        (CallFunction|ReDisplayInputPrompt)
        (bind _tutorial_objective_2 (CallFunction|GetTutorialObjective))
        (Transformation|SetActorLocation (Variables|Default|GetArrow) (+ (Transformation|GetActorLocation _tutorial_objective_2) "0.000000,0.000000,350.000000") false false))
      (:11
        (Rendering|SetVisibility (Variables|/Game/Blueprints/BP_IndicatorArrow.BP_IndicatorArrow_C|GetCone (Variables|Default|GetArrow)) false false)
        (bind _tutorial_objective_3 (CallFunction|GetTutorialObjective))
        (Transformation|SetActorLocation (Variables|Default|GetArrow) (+ (Transformation|GetActorLocation (Variables|/Game/Blueprints/Objective/ObjectiveBase/BP_Objective_Base.BP_Objective_Base_C|GetObjective%20Dependent _tutorial_objective_3)) "0.000000,0.000000,350.000000") false false)
        (bind _returnvalue_6 (Utilities|Time|SetTimerbyFunctionName 0 "RotateToArrow" 0.01 true))
        (Variables|Default|SetLookAtTimer _returnvalue_6)
        (Utilities|FlowControl|Delay 1.0)
        (Class|BPIInteractable|ObjectiveActivate(Message) (Variables|/Game/Blueprints/Objective/ObjectiveBase/BP_Objective_Base.BP_Objective_Base_C|GetObjective%20Dependent _tutorial_objective_3))
        (bind _main_core (CallFunction|GetMainCore))
        (Variables|/Game/Blueprints/EngineCores/BP_EngineCore.BP_EngineCore_C|SetResourceGenDelay _main_core (* (Variables|/Game/Blueprints/EngineCores/BP_EngineCore.BP_EngineCore_C|GetResourceGenDelay _main_core) 0.5))
        (CallFunction|DisplayDialogue (Utilities|Array|MakeArray "It seems the doors to the other wings of the Synthera have been jammed." " With their cores offline, the only way to open the doors is to deposit the appropriate resources into the terminals by each door.") false 12))
      (:12
        (CallFunction|EnableMovement true)
        (CallFunction|ReDisplayInputPrompt)))))

(fn ConstructionScript)

(fn AddtoView
  (UserInterface|Viewport|AddtoViewport (Variables|Default|GetDialogueBox) 0))

(fn RemovefromView
  (Widget|RemovefromParent (Variables|Default|GetDialogueBox))
  (Rendering|Components|TextRender|SetText (Variables|/Game/UI/WidgetBlueprints/WB_DialogueBox.WB_DialogueBox_C|GetTextBox (Variables|Default|GetDialogueBox)) ""))

(fn ProceedThroughTextInput
  (if (Widget|IsVisible (Variables|Default|GetDialogueBox))
    (if (Variables|/Game/UI/WidgetBlueprints/WB_DialogueBox.WB_DialogueBox_C|GetCompletedTyping? (Variables|Default|GetDialogueBox))
      (bind _result (Math|Integer|IncrementInt (Variables|Default|GetIndex))
        (:%20%20
          (if (>= _result (Utilities|Array|Length (Variables|Default|GetText%20to%20Write)))
            (CallFunction|RemovefromView)
            (return true)
            (else
              (Default|WriteOutText (Variables|Default|GetDialogueBox) (Utilities|Array|Get(acopy) (Variables|Default|GetText%20to%20Write) (Variables|Default|GetIndex)))
              (return false)))))
      (else
        (Default|SkiptoEnd (Variables|Default|GetDialogueBox))
        (return false)))
    (else
      (return false))))

(fn EnableMovement
  (params (Enable? :type Boolean))
  (if Enable?
    (Input|SetInputModeGameOnly (Game|GetPlayerController 0) false)
    (Variables|/Script/Engine.PlayerController|SetbShowMouseCursor (Game|GetPlayerController 0) false)
    (Variables|/Game/Blueprints/Player/BP_FPCharacter.BP_FPCharacter_C|SetMovementEnabled (Variables|Default|GetPlayer) true)
    (Variables|/Game/Blueprints/Player/BP_FPCharacter.BP_FPCharacter_C|SetMenuOpen (Variables|Default|GetPlayer) false)
    (Variables|/Game/Blueprints/Player/BP_FPCharacter.BP_FPCharacter_C|SetInteractEnabled (Variables|Default|GetPlayer) true)
    (CallFunction|SetHotbarVisibility true)
    (else
      (Input|SetInputModeGameandUI (Game|GetPlayerController 0) (Variables|Default|GetDialogueBox) "DoNotLock" true true)
      (Variables|/Script/Engine.PlayerController|SetbShowMouseCursor (Game|GetPlayerController 0) false)
      (Variables|/Game/Blueprints/Player/BP_FPCharacter.BP_FPCharacter_C|SetMovementEnabled (Variables|Default|GetPlayer) false)
      (Variables|/Game/Blueprints/Player/BP_FPCharacter.BP_FPCharacter_C|SetMenuOpen (Variables|Default|GetPlayer) true)
      (Variables|/Game/Blueprints/Player/BP_FPCharacter.BP_FPCharacter_C|SetInteractEnabled (Variables|Default|GetPlayer) false)
      (CallFunction|SetHotbarVisibility false))))

(fn RotatetoArrow
  (bind _player (Variables|Default|GetPlayer))
  (bind _player_2 (Variables|Default|GetPlayer))
  (Pawn|SetControlRotation (Game|GetPlayerController 0) (Math|Interpolation|RInterpTo (Pawn|GetControlRotation _player :!class /Script/Engine.Pawn) (Math|Rotator|FindLookatRotation (Transformation|GetActorLocation _player) (Transformation|GetActorLocation (Variables|Default|GetArrow))) (Utilities|Time|GetWorldDeltaSeconds) 5.0))
  (if (Utilities|Operators|EqualEqual (Pawn|GetControlRotation _player_2 :!class /Script/Engine.Pawn) (Math|Rotator|FindLookatRotation (Transformation|GetActorLocation _player_2) (Transformation|GetActorLocation (Variables|Default|GetArrow))) 1.0)
    (Utilities|Time|ClearandInvalidateTimerbyHandle (Variables|Default|GetLookAtTimer))))

(fn ReDisplayInputPrompt
  (if (UserInterface|Viewport|IsinViewport (Variables|/Game/Blueprints/Player/BP_FPCharacter.BP_FPCharacter_C|GetInputPromptWidget (Variables|Default|GetPlayer)))
    (Widget|SetVisibility (Variables|/Game/Blueprints/Player/BP_FPCharacter.BP_FPCharacter_C|GetInputPromptWidget (Variables|Default|GetPlayer)) "Visible")))

(fn HideInputPrompt
  (bind _player (Variables|Default|GetPlayer))
  (bind _inputpromptwidget (Variables|/Game/Blueprints/Player/BP_FPCharacter.BP_FPCharacter_C|GetInputPromptWidget _player))
  (Utilities|IsValid _inputpromptwidget
    (:Is%20Valid
      (if (UserInterface|Viewport|IsinViewport _inputpromptwidget)
        (Widget|SetVisibility (Variables|/Game/Blueprints/Player/BP_FPCharacter.BP_FPCharacter_C|GetInputPromptWidget (Variables|Default|GetPlayer)) "Hidden")
        (else
          (Default|HideInputPrompt (Variables|Default|GetPlayer)))))))

(fn GetMainCore
  (bind _outactors (Actor|GetAllActorsOfClass "/Game/Blueprints/EngineCores/BP_EngineCore.BP_EngineCore_C"))
  (for _array_element _outactors
    (bind _name (Class|BPIInteractable|GetName(Message) _array_element))
    (if (== _name "Bridge")
      (return _array_element (Transformation|GetActorLocation _array_element)))))

(fn GetTutorialObjective
  (bind _outactors (Actor|GetAllActorsOfClass "/Game/Blueprints/Objective/ObjectiveBase/BP_Objective_Base.BP_Objective_Base_C"))
  (for _array_element _outactors
    (bind _name (Class|BPIInteractable|GetName(Message) _array_element))
    (if (== _name "Tutorial")
      (return _array_element))))

(fn GetTutorialFurnace
  (bind _returnvalue (Actor|GetActorOfClass "/Game/Blueprints/Machines/CraftingMachines/BP_Machine_Furnace.BP_Machine_Furnace_C"))
  (return _returnvalue))

(fn SetHotbarVisibility
  (params (Visible? :type Boolean))
  (bind _player (Variables|Default|GetPlayer))
  (bind _inventoryui (Variables|/Game/Blueprints/Player/BP_FPCharacter.BP_FPCharacter_C|GetInventoryUI _player))
  (bind _w_hotbar (Variables|/Game/UI/WidgetBlueprints/CraftingSystemMenus/W_Inventory.W_Inventory_C|GetW_Hotbar _inventoryui))
  (if Visible?
    (Widget|SetVisibility _w_hotbar "Visible")
    (else
      (Widget|SetVisibility _w_hotbar "Hidden"))))