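; Base manager Blueprint that connects managers to the level's event system through an observer pattern.
; On BeginPlay it finds and stores the LevelEventManager actor by class, then subscribes itself if it casts to BPI_Observer.
; Its query functions for tags, location, name, machine data and resources are stubs returning empty or default values.
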(event EventBeginPlay
  (bind _returnvalue (Actor|GetActorOfClass (Variables|Default|GetLevelEventManagerClass)))
  (Variables|Default|SetLevelEventManager _returnvalue)
  (bind _asbpi_observer (Utilities|Casting|CastToBPI_Observer self))
  (Default|SubscribeObserver (Variables|Default|GetLevelEventManager) _asbpi_observer))

(fn ConstructionScript)

(fn GameplayTag
  (return ""))

(fn GetGameplayTags
  (return ""))

(fn GetLocation
  (return "0, 0, 0"))

(fn GetMachine
  (return 0))

(fn GetMachineClass
  (return 0))

(fn GetMachineMesh
  (return 0))

(fn GetName
  (return "None"))

(fn HasResource
  (params (Resource%20Name :type Name :default "None"))
  (return 0 false))