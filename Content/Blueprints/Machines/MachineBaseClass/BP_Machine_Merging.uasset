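; Work-in-progress factory machine actor that draws power from engine cores and can be picked up, placed, repaired and queried by robots.
; An EventChange state machine registers it with the nearest core in horizontal range and updates colored status text, which timers turn toward the camera.
; Resources live in an array indexed by a name-to-index map for recipe crafting, though StartTimer is empty and several setup chains are disconnected.
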(event OnComponentBeginOverlap(InputInteractionBox)
  (params (OverlappedComponent :type Primitive%20Component%20Object%20Reference) (OtherActor :type Actor%20Object%20Reference) (OtherComp :type Primitive%20Component%20Object%20Reference) (OtherBodyIndex :type Integer) (bFromSweep :type Boolean) (SweepResult :type Hit%20Result%20Structure%20%28by%20ref%29))
  ;[0.15 0.15 0.15 0.5] Interactions with other actors
  (if (not (Utilities|DoesObjectImplementInterface OtherActor "/Game/Blueprints/Robot/BPI_Robot.BPI_Robot_C"))
    (if (< (Variables|Default|GetCurrentHealth) (.maxhealth (Variables|Default|GetMachine%20Info)))
      (bind _asbp_fpcharacter (Utilities|Casting|CastToBP_FPCharacter OtherActor))
      (Default|DisplayInputPrompt _asbp_fpcharacter "Press E to Interact & R to Repair")
      (else
        (bind _asbp_fpcharacter_2 (Utilities|Casting|CastToBP_FPCharacter OtherActor))
        (Default|DisplayInputPrompt _asbp_fpcharacter_2 "Press E to Interact")))))

(event OnComponentEndOverlap(InputInteractionBox)
  (params (OverlappedComponent :type Primitive%20Component%20Object%20Reference) (OtherActor :type Actor%20Object%20Reference) (OtherComp :type Primitive%20Component%20Object%20Reference) (OtherBodyIndex :type Integer))
  ;[0.15 0.15 0.15 0.5] Interactions with other actors
  (if (not (Utilities|DoesObjectImplementInterface OtherActor "/Game/Blueprints/Robot/BPI_Robot.BPI_Robot_C"))
    (bind _asbp_fpcharacter (Utilities|Casting|CastToBP_FPCharacter OtherActor))
    (Default|HideInputPrompt _asbp_fpcharacter)))

(event Custom|Start%20Timer
  ;[0.15 0.15 0.15 0.5] Crafting An Item
)

(event Custom|Timer
  (bind (_resource_name _resource_index) (CallFunction|GetResourceAmount (Variables|Containers|GetResourceIndex) (Variables|Default|Getname)))
  (CallFunction|CraftItem (Variables|Default|GetActiveRecipe) (Variables|Containers|GetResourceInventory) _resource_name _resource_index))

(event Custom|UpdateWidget
  (bind _textrender (Variables|Default|GetTextRender))
  (bind _poweredbytext (Variables|Default|GetPoweredByText))
  (Transformation|SetWorldRotation _textrender (Math|Rotator|FindLookatRotation (Transformation|GetWorldLocation _textrender) (Transformation|GetWorldLocation (Variables|/Script/Engine.PlayerCameraManager|GetTransformComponent (Game|GetPlayerCameraManager 0)))) false false)
  (Transformation|SetWorldRotation _poweredbytext (Math|Rotator|FindLookatRotation (Transformation|GetWorldLocation _poweredbytext) (Transformation|GetWorldLocation (Variables|/Script/Engine.PlayerCameraManager|GetTransformComponent (Game|GetPlayerCameraManager 0)))) false false))

(event Custom|Stop%20Timer
  ;[0.15 0.15 0.15 0.5] Crafting An Item
  (Utilities|Time|ClearandInvalidateTimerbyHandle (Variables|Default|GetCraftingTimer)))

(event Custom|TimerReset
  (bind _recipeinventory (Variables|Containers|GetRecipeInventory))
  (bind _machinerecipeslot (Variables|Enum|GetMachineRecipeSlot))
  (bind _machinerecipeslot_2 (Variables|Enum|GetMachineRecipeSlot))
  (bind _returnvalue (Math|Conversions|ToInteger(Byte) _machinerecipeslot))
  (bind _output (Utilities|Array|Get(acopy) _recipeinventory _returnvalue))
  (bind _output_2 (Utilities|Array|Get(acopy) _recipeinventory _returnvalue))
  (bind _output_3 (Utilities|Array|Get(acopy) _recipeinventory _returnvalue))
  (bind _output_4 (Utilities|Array|Get(acopy) _recipeinventory _returnvalue))
  (bind _returnvalue_2 (Utilities|Select :Index _machinerecipeslot :NewEnumerator0 _output :NewEnumerator1 _output_2 :NewEnumerator2 _output_3 :NewEnumerator3 _output_4))
  (switch Utilities|FlowControl|Switch|SwitchonE_MachineRecipeSlot _machinerecipeslot_2
    (:NewEnumerator0
      (Development|PrintString (Utilities|String|EnumtoString _machinerecipeslot_2))
      (Variables|Default|SetActiveRecipe _returnvalue_2))
    (:NewEnumerator1
      (Development|PrintString (Utilities|String|EnumtoString _machinerecipeslot_2))
      (Variables|Default|SetActiveRecipe _returnvalue_2)))
  (Utilities|Time|ClearandInvalidateTimerbyHandle (Variables|Default|GetCraftingTimer))
  (bind _returnvalue_3 (Utilities|Time|SetTimerbyFunctionName 0 "Timer" (.productionrate (Variables|Default|GetMachine%20Info%20Defaults)) true))
  (Variables|Default|SetCraftingTimer _returnvalue_3))

(event Custom|RepairLoop
  (bind _machine_info (Variables|Default|GetMachine%20Info))
  ;[0.15 0.15 0.15 0.5] Start repair timer when holding R and stop when R is released - Set player state to repairing if health isn't full, otherise cancel this event - Also stop if repairing finishes
  (if (< (Variables|Default|GetCurrentHealth) (.maxhealth _machine_info))
    (bind _output_get (Variables|Default|SetCurrentHealth (Math|Float|Clamp(Float) (+ (Variables|Default|GetCurrentHealth) 1.0) 0.0 (.maxhealth _machine_info))))
    (Default|DisplayRepairing (stale EventRepair Player) _output_get (.maxhealth _machine_info) true)
    (if (Utilities|Enum|Equal(Enum) (Variables|Enum|GetOperational%20State) "NewEnumerator1")
      (CallFunction|EventChange))
    (else
      (Utilities|Time|ClearandInvalidateTimerbyHandle (Variables|Default|GetRepair%20Timer))
      (Default|DisplayRepairing (stale EventRepair Player) (Variables|Default|GetCurrentHealth) (.maxhealth _machine_info) false))))

(event Custom|Upgrade
  (bind _output_get (Variables|Default|SetMachine%20Info%20Defaults (Utilities|Struct|MakeStruct_MachineValues 0.0 0.0 0 (- (.productionrate (Variables|Default|GetMachine%20Info%20Defaults)) 0.2))))
  (Development|PrintString (Utilities|String|ToString(Float) (.ProductionRate (Utilities|Struct|BreakStruct_MachineValues _output_get)))))

(event Custom|EventChange
  ;[0.15 0.15 0.15 0.5] Event Logic
  (CallFunction|SetCorePoweredby)
  (switch Utilities|FlowControl|Switch|SwitchonE_MachineState (Variables|Enum|GetMachineStates)
    (:NewEnumerator0
      (Utilities|FlowControl|DoOnce false
        (:Completed
          (Development|PrintString "In the default state")
          (Variables|Enum|SetMachineStates "NewEnumerator3")
          (Development|PrintString "Switching to crafting")
          (CallFunction|EventChange))))
    (:NewEnumerator3
      (CallFunction|SetPoweredbyText)
      (switch Utilities|FlowControl|Switch|SwitchonE_OperationalState (Variables|Enum|GetOperational%20State)
        (:NewEnumerator0
          (CallFunction|SetCorePoweredby))
        (:NewEnumerator2
          (switch Utilities|FlowControl|Switch|SwitchonE_MachineSubState (Variables|Enum|GetMachineSubStates)
            (:NewEnumerator0
              (CallFunction|StartTimer)
              (Development|PrintString " Started crafting"))))))))

(event Custom|Set%20Powered%20By%20Text
  (bind _poweredbytext (Variables|Default|GetPoweredByText))
  (bind _operational_state (Variables|Enum|GetOperational%20State))
  ;[0.15 0.15 0.15 0.5] Set Text Render PoweredByText and Color (temp)
  (Rendering|Components|TextRender|SetText _poweredbytext (|GenerictoText _operational_state))
  (Rendering|Components|TextRender|SetTextRenderColor _poweredbytext (Utilities|Select :Index _operational_state :NewEnumerator0 (Class|KismetMathLibrary|LinearColortoRGBE "(R=0.679543,G=0.005182,B=0.040915,A=1.000000)") :NewEnumerator1 (Class|KismetMathLibrary|LinearColortoRGBE) :NewEnumerator2 (Class|KismetMathLibrary|LinearColortoRGBE "(R=0.000000,G=1.000000,B=0.327778,A=1.000000)"))))

(event EventRenameMachine
  (Rendering|Components|TextRender|SetText (Variables|Default|GetTextRender) (Utilities|Text|ToText(String) (Utilities|String|Append (Utilities|String|ToString(Name) (Variables|Default|GetMachineName)) (Utilities|String|ToString(Integer) (Math|Random|RandomInteger 100)))))
  (Variables|Enum|SetMachineRecipeSlot (Utilities|Enum|ByteToEnumE_MachineRecipeSlot (Math|Conversions|ToByte(Integer) 1))))

(event EventSelection
  (params (Player :type BP%20FP%20Character%20Object%20Reference))
  ;[0.15 0.15 0.15 0.5] BPI Logic
)

(event EventBeginPlay
  ;[0.15 0.15 0.15 0.5] Initialization
  (Utilities|Time|SetTimerbyEvent (delegate Custom|UpdateWidget) 0.01 true)
  (CallFunction|EventChange))

(event EventPickupMachine
  (params (Player :type BP%20FP%20Character%20Object%20Reference))
  ;[0.15 0.15 0.15 0.5] BPI Logic
  (Transformation|AttachComponentToComponent 0 "None" "SnapToTarget" "KeepRelative" "KeepRelative" true)
  (Variables|Enum|SetMachineStates "NewEnumerator2")
  (CallFunction|StopTimer)
  (Development|PrintString "Is picked up")
  (CallFunction|EventChange))

(event EventPlaceMachine
  ;[0.15 0.15 0.15 0.5] BPI Logic
  (Transformation|DetachFromActor "KeepRelative" "KeepRelative" "KeepRelative")
  (Transformation|SetActorTransform self (Math|Conversions|ToTransform(Vector) (.HitLocation (Utilities|Struct|BreakS_Linetrace (Variables|/Game/Blueprints/Player/BP_FPCharacter.BP_FPCharacter_C|GetLineTraceInfo (stale EventSelection Player))))))
  (Variables|Enum|SetMachineStates "NewEnumerator3")
  (Development|PrintString "Is placed")
  (CallFunction|EventChange))

(event EventRecieveEnergy
  (params (Sending%20Core :type BP%20Engine%20Core%20Object%20Reference) (Operational? :type Boolean))
  ;[0.15 0.15 0.15 0.5] Recieving Energy From the Core
  (if Operational?
    (switch Utilities|FlowControl|Switch|SwitchonE_OperationalState (Variables|Enum|GetOperational%20State)
      (:NewEnumerator0
        _)
      (:NewEnumerator2
        _))
    (Variables|Enum|SetOperational%20State "NewEnumerator2")
    (CallFunction|EventChange)
    (CallFunction|SetPoweredbyText)
    (else
      (switch Utilities|FlowControl|Switch|SwitchonE_OperationalState (Variables|Enum|GetOperational%20State)
        (:NewEnumerator0
          _)
        (:NewEnumerator2
          _))
      (Variables|Enum|SetOperational%20State "NewEnumerator0")
      (CallFunction|SetPoweredbyText))))

(event EventRepair
  (params (Player :type BP%20FP%20Character%20Object%20Reference) (Repairing? :type Boolean))
  (bind _machine_info (Variables|Default|GetMachine%20Info))
  ;[0.15 0.15 0.15 0.5] Start repair timer when holding R and stop when R is released - Set player state to repairing if health isn't full, otherise cancel this event - Also stop if repairing finishes
  (if Repairing?
    (if (< (Variables|Default|GetCurrentHealth) (.maxhealth _machine_info))
      (Variables|/Game/Blueprints/Player/BP_FPCharacter.BP_FPCharacter_C|SetPlayerStates Player "NewEnumerator6")
      (Utilities|Time|ClearandInvalidateTimerbyHandle (Variables|Default|GetRepair%20Timer))
      (bind _returnvalue (Utilities|Time|SetTimerbyEvent (delegate Custom|RepairLoop) 0.2 true))
      (Variables|Default|SetRepair%20Timer _returnvalue))
    (else
      (Utilities|Time|ClearandInvalidateTimerbyHandle (Variables|Default|GetRepair%20Timer))
      (Default|DisplayRepairing Player (Variables|Default|GetCurrentHealth) (.maxhealth _machine_info) false))))

(event EventRemoveResource1
  (params (Resource%20Name :type Name :default "None") (Amount%20To%20Remove :type Integer) (Resource%20Index :type Integer))
  ;[0.15 0.15 0.15 0.5] BPI Logic
  (CallFunction|SetResourceAmount Resource%20Index Amount%20To%20Remove (Variables|Containers|GetResourceInventory)))

(event EventInteract
  (params (Player :type BP%20FP%20Character%20Object%20Reference))
  (Development|PrintString (Utilities|GetDisplayName self)))

(fn ConstructionScript
  (bind _machine_info_defaults (Variables|Default|GetMachine%20Info%20Defaults))
  (Variables|Default|SetMachineName (Utilities|String|StringToName (Utilities|GetDisplayName self)))
  (bind _output_get (Variables|Default|SetMachine%20Info (Utilities|Struct|MakeStruct_MachineValues (.maxhealth _machine_info_defaults) (.distancefromcore _machine_info_defaults) (.energycost _machine_info_defaults) (.productionrate _machine_info_defaults))))
  (Variables|Default|SetCurrentHealth (.maxhealth _output_get))
  (CallFunction|InventoryMap (Variables|Containers|GetResourceInventory) (Variables|Containers|GetResourceIndex)))

(fn ResourceUpdate
  (params (TargetMap :type Map%20of%20Strings%20to%20Structs) (Resource%20Name :type String))
  (bind _value (Utilities|Map|Find TargetMap Resource%20Name))
  (return 0 _value ""))

(fn AddtoInventory
  (params (ResourceInventory :type Array%20of%20S%20Resources%20Structures) (Item :type S%20Resources%20Structure%20%28by%20ref%29))
  (bind (_name _mesh _amount) (Utilities|Struct|BreakS_Resources Item))
  (if (Utilities|Array|IsEmpty ResourceInventory)
    (Utilities|Array|Add ResourceInventory Item)
    (return)
    (else
      (for (_array_element _array_index) ResourceInventory
        (if (== (.Name (Utilities|Struct|BreakS_Resources _array_element)) _name)
          (bind _structout (Utilities|Struct|SetmembersinS_Resources (Utilities|Array|Get(acopy) ResourceInventory _array_index) (+ _amount (.Amount (Utilities|Struct|BreakS_Resources _array_element)))))
          (Development|PrintString (Utilities|String|ToString(Name) (.Name (Utilities|Struct|BreakS_Resources _structout))))
          (else
            (Utilities|Array|Add ResourceInventory Item)))))))

(fn InventoryMap
  (params (Resource%20Inventory :type Array%20of%20S%20Resources%20Structures) (ResourceIndex :type Map%20of%20Names%20to%20Integers))
  (for (_array_element _array_index) Resource%20Inventory
    (Utilities|Map|Add ResourceIndex (.Name (Utilities|Struct|BreakS_Resources _array_element)) _array_index)))

(fn GetResourceAmount
  (params (TargetMap :type Map%20of%20Names%20to%20Integers) (name :type Name))
  (bind _value (Utilities|Map|Find TargetMap name))
  (bind _resourceinventory (Variables|Containers|GetResourceInventory))
  (bind _output (Utilities|Array|Get(acopy) _resourceinventory _value))
  (bind (_name _mesh _amount) (Utilities|Struct|BreakS_Resources _output))
  (return _name _value _amount))

(fn CraftItem
  (params (Recipe :type S%20Recipes%20Structure%20%28by%20ref%29) (Resource%20Inventory :type Array%20of%20S%20Resources%20Structures) (Item%20Name :type Name) (Item%20Index :type Integer))
  (bind _requiredresources (Utilities|Struct|BreakS_Recipes Recipe))
  (bind _output (Utilities|Array|Get(acopy) Resource%20Inventory Item%20Index))
  (bind _amount (Utilities|Struct|BreakS_Resources _output))
  (bind _value (Utilities|Map|Find _requiredresources Item%20Name))
  (if (>= _amount _value)
    (Utilities|Struct|SetmembersinS_Resources _output (- _amount _value))
    (Development|PrintString "Item crafted")
    (return)
    (else
      (return))))

(fn RemoveResource
  (params (Resource%20Inventory :type Array%20of%20S%20Resources%20Structures) (Resource%20Index :type Map%20of%20Names%20to%20Integers) (Name :type Name) (Item%20Index :type Integer)))

(fn SetResourceAmount
  (params (Index :type Integer) (Amount%20To%20Remove :type Integer) (Array :type Array%20of%20S%20Resources%20Structures))
  (bind _output (Utilities|Array|Get(acopy) Array Index))
  (Utilities|Struct|SetmembersinS_Resources _output (- (.Amount (Utilities|Struct|BreakS_Resources _output)) Amount%20To%20Remove)))

(fn AddingRecipes
  (params (Recipes :type Data%20Table%20Object%20Reference%20%28by%20ref%29) (Recipe%20Inventory :type Array%20of%20S%20Recipes%20Structures))
  (for _array_element (Variables|Containers|GetRecipeNames)
    (bind _returnvalue (Utilities|GetDataTableRow Recipes _array_element)
      (:then
        (Utilities|Array|Add Recipe%20Inventory _returnvalue)))))

(fn SetCorePoweredby
  (bind _self self)
  (bind _machine_info (Variables|Default|GetMachine%20Info))
  (LocalVariables|SetDistance 9999.0)
  (bind _outactors (Actor|GetAllActorsOfClass "/Game/Blueprints/EngineCores/BP_EngineCore.BP_EngineCore_C"))
  (for _array_element _outactors
    (if (and (< (Transformation|GetHorizontalDistanceTo _array_element self) (LocalVariables|GetDistance)) (<= (Transformation|GetHorizontalDistanceTo _array_element self) (.distancefromcore (Variables|Default|GetMachine%20Info))))
      (LocalVariables|SetTemp%20Core _array_element)
      (LocalVariables|SetDistance (Transformation|GetHorizontalDistanceTo _array_element self))))
  (bind _temp_core (LocalVariables|GetTemp%20Core)
    (:then
      (Variables|Default|SetCore%20Powered%20By _temp_core)
      (Variables|Enum|SetOperational%20State "NewEnumerator2")
      (Development|PrintString "in range")
      (Default|VerifyDependentMachine (Variables|Default|GetCore%20Powered%20By) _self (.energycost _machine_info) true))
    (:else
      (Development|PrintString "Not in range of core!" true true "(R=1.000000,G=0.000000,B=0.077756,A=1.000000)")
      (Variables|Enum|SetOperational%20State "NewEnumerator0")
      (bind _core_powered_by (Variables|Default|GetCore%20Powered%20By)
        (:then
          (Default|VerifyDependentMachine _core_powered_by _self (.energycost _machine_info) false))
        (:else)))))

(fn ResetTimer
  (Development|PrintString "Timer reset"))

(fn GameplayTag
  (return "(TagName=\"Interactable\")"))

(fn GetMachineHealth
  (return (Variables|Default|GetCurrentHealth) (.maxhealth (Variables|Default|GetMachine%20Info))))

(fn GetLocation1
  (return (Transformation|GetActorLocation)))

(fn GetGameplayTags
  (return (Variables|Default|GetGameplayTags_0)))

(fn GetLocation
  (return (Transformation|GetActorLocation)))

(fn GetMachine
  (return self))

(fn GetName
  (return (Variables|Default|Getname)))

(fn HasResource1
  (params (Resource%20Robot%20Is%20Looking%20For :type Name :default "None"))
  (bind (_resource_name _resource_index _resourceamount) (CallFunction|GetResourceAmount (Variables|Containers|GetResourceIndex) Resource%20Robot%20Is%20Looking%20For))
  (return _resource_name _resource_index _resourceamount))

(fn HasResource
  (params (Resource%20Robot%20Is%20Looking%20For :type Name :default "None"))
  (return "None" 0 0))