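; BP_Machine_Barricade is the barricade variant of the machine base class, a machine that players can place, pick up and rotate.
; Begin play, construction, placement and pickup defer to the parent, while rotation adds the given degrees to a stored value.
; Interact and the input box overlap events are empty, so interacting does nothing here.
; Getter functions expose health, mesh, name, class, location, rotation and the Machine tag.
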(event OnComponentBeginOverlap(InputInteractionBox)
  (params (OverlappedComponent :type Primitive%20Component%20Object%20Reference) (OtherActor :type Actor%20Object%20Reference) (OtherComp :type Primitive%20Component%20Object%20Reference) (OtherBodyIndex :type Integer) (bFromSweep :type Boolean) (SweepResult :type Hit%20Result%20Structure%20%28by%20ref%29)))

(event OnComponentEndOverlap(InputInteractionBox)
  (params (OverlappedComponent :type Primitive%20Component%20Object%20Reference) (OtherActor :type Actor%20Object%20Reference) (OtherComp :type Primitive%20Component%20Object%20Reference) (OtherBodyIndex :type Integer)))

(event EventBeginPlay
  (|CallParentFunction))

(event EventRotateObject
  (params (Degrees :type Float%20%28double-precision%29))
  (Variables|Default|SetRotation (+ Degrees (Variables|Default|GetRotation))))

(event EventPickupMachine
  (params (Player :type BP%20FP%20Character%20Object%20Reference))
  (|CallParentFunction Player))

(event EventPlaceMachine
  (params (Player :type BP%20FP%20Character%20Object%20Reference))
  (|CallParentFunction Player))

(event EventInteract
  (params (Player :type BP%20FP%20Character%20Object%20Reference)))

(fn ConstructionScript
  (|CallParentFunction))

(fn GetMachineHealth
  (return (Variables|Default|GetCurrentHealth) (.maxhealth (Variables|Default|GetMachine%20Info))))

(fn GetMachine
  (return self))

(fn GetLocation
  (return (Transformation|GetActorLocation)))

(fn GetMachineMesh
  (return (Variables|Character|GetMesh)))

(fn GetName
  (return (Variables|Default|GetName)))

(fn GetMachineClass
  (return "BP_Machine_Barricade_C"))

(fn GetGameplayTags
  (return "(GameplayTags=((TagName=\"Machine\"),(TagName=\"Interactable\")))"))

(fn GetRotation
  (return (Variables|Default|GetRotation)))