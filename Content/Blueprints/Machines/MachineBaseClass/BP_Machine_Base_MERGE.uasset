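; Base class for player-placeable machines that can be picked up, placed, damaged, repaired with Gel and given unique names.
; UpdateStatus links the machine to the nearest BP_EngineCore in range, registering it on that grid, while core Energy events toggle power on the diegetic details widget.
; An overlap box shows interact prompts and a looping timer drives hold-to-repair.
; Most specific upgrade functions raise errors so child classes override them.
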(event OnComponentBeginOverlap(InputInteractionBox)
  (params (OverlappedComponent :type Primitive%20Component%20Object%20Reference) (OtherActor :type Actor%20Object%20Reference) (OtherComp :type Primitive%20Component%20Object%20Reference) (OtherBodyIndex :type Integer) (bFromSweep :type Boolean) (SweepResult :type Hit%20Result%20Structure%20%28by%20ref%29))
  ;[0.15 0.15 0.15 0.5] Interactions with other actors
  (bind _asbp_fpcharacter (Utilities|Casting|CastToBP_FPCharacter OtherActor))
  (switch Utilities|FlowControl|Switch|SwitchonE_PlayerState (Variables|/Game/Blueprints/Player/BP_FPCharacter.BP_FPCharacter_C|GetPlayerStates _asbp_fpcharacter)
    (:NewEnumerator0
      (CallFunction|DisplayInteract OtherActor))))

(event OnComponentEndOverlap(InputInteractionBox)
  (params (OverlappedComponent :type Primitive%20Component%20Object%20Reference) (OtherActor :type Actor%20Object%20Reference) (OtherComp :type Primitive%20Component%20Object%20Reference) (OtherBodyIndex :type Integer))
  ;[0.15 0.15 0.15 0.5] Interactions with other actors
  (CallFunction|HideInteract OtherActor))

(event Custom|Interact_1_1
  (params (Player :type BP%20FP%20Character%20Object%20Reference))
  (CallFunction|ActionInteract Player))

(event Custom|Upgrade
  (params (Upgrades :type E_Upgrades%20Enum :default "NewEnumerator0"))
  (CallFunction|UpgradeMachine))

(event Custom|UpdateWidgets
  ;[0.15 0.15 0.15 0.5] Initialize Text Widgets
  (CallFunction|SetWidgetRotation (Variables|Default|GetMachineDetailsWidget)))

(event EventEnergy
  (params (Sending%20Core :type BP%20Engine%20Core%20Object%20Reference) (Operational? :type Boolean))
  ;[0.15 0.15 0.15 0.5] Recieving Energy From the Core
  (Default|SetPowered (Variables|Default|GetDetailsWidget) Operational?)
  (if Operational?
    (switch Utilities|FlowControl|Switch|SwitchonE_OperationalState (Variables|Enum|GetOperational%20State)
      (:NewEnumerator0
        _)
      (:NewEnumerator2
        _))
    (Variables|Enum|SetOperational%20State "NewEnumerator2")
    (CallFunction|UpdateStatus)
    (Default|SetPowered (Variables|Default|GetDetailsWidget) true)
    (else
      (switch Utilities|FlowControl|Switch|SwitchonE_OperationalState (Variables|Enum|GetOperational%20State)
        (:NewEnumerator0
          _)
        (:NewEnumerator2
          _))
      (Variables|Enum|SetOperational%20State "NewEnumerator0")
      (Default|SetPowered (Variables|Default|GetDetailsWidget) false))))

(event EventDropOffResource
  (params (ResourceName :type Name :default "None") (ResourceAmount :type Integer))
  (CallFunction|DropOffResourceAction ResourceName ResourceAmount))

(event Game|Damage|EventAnyDamage
  (params (Damage :type Float%20%28single-precision%29) (DamageType :type Damage%20Type%20Object%20Reference) (InstigatedBy :type Controller%20Object%20Reference) (DamageCauser :type Actor%20Object%20Reference))
  ;[0.15 0.15 0.15 0.5] When Takes Damage and runs out of health, set state to destroyed and remove machine from power grid
  (if (> (Variables|Default|GetCurrentHealth) 0.0)
    (bind _output_get (Variables|Default|SetCurrentHealth (- (Variables|Default|GetCurrentHealth) Damage)))
    (if (<= _output_get 0.0)
      (Variables|Enum|SetOperational%20State "NewEnumerator1")
      (CallFunction|UpdateStatus))))

(event EventOnNotify
  (params (EventType :type E_LevelEventType%20Enum :default "NewEnumerator0"))
  (switch Utilities|FlowControl|Switch|SwitchonE_LevelEventType EventType
    (:NewEnumerator7
      (CallFunction|UpdateStatus))))

(event EventPickupMachine
  (params (Player :type BP%20FP%20Character%20Object%20Reference))
  ;[0.15 0.15 0.15 0.5] BPI Logic
  (CallFunction|HideInteract (Game|GetPlayerCharacter 0))
  (Rendering|SetVisibility (Variables|Default|GetMesh) false false)
  (Rendering|SetVisibility (Variables|Default|GetMachineDetailsWidget) false false)
  (CallFunction|AttachtoComponet)
  (CallFunction|UpdateStatus))

(event EventPlaceMachine
  (params (Player :type BP%20FP%20Character%20Object%20Reference))
  ;[0.15 0.15 0.15 0.5] BPI Logic
  (CallFunction|PlaceMachineDown Player)
  (CallFunction|UpdateStatus)
  (Transformation|SetActorRotation (Math|Rotator|MakeRotator 0.0 0.0 (Variables|/Game/Blueprints/Player/BP_FPCharacter.BP_FPCharacter_C|GetBuildRotation Player))))

(event EventRotateObject
  (params (Degrees :type Float%20%28double-precision%29))
  ;[0.15 0.15 0.15 0.5] Rotate Machine When Placing
  (Variables|Default|SetRotation (+ Degrees (Variables|Default|GetRotation))))

(event EventRepair
  (params (Player :type BP%20FP%20Character%20Object%20Reference) (Repairing? :type Boolean))
  ;[0.15 0.15 0.15 0.5] Start repair timer when holding R and stop when R is released - Set player state to repairing if health isn't full, otherise cancel this event - Also stop if repairing finishes
  (CallFunction|RepairMachine Player Repairing?))

(fn ConstructionScript
  (bind _machine_info_defaults (Variables|Default|GetMachine%20Info%20Defaults))
  (bind _output_get (Variables|Default|SetMachine%20Info (Utilities|Struct|MakeStruct_MachineValues (.maxhealth _machine_info_defaults) (.distancefromcore _machine_info_defaults) (.energycost _machine_info_defaults) (.productionrate _machine_info_defaults))))
  (Variables|Default|SetCurrentHealth (.maxhealth _output_get)))

(fn ResourceUpdate
  (params (TargetMap :type Map%20of%20Strings%20to%20Structs) (Resource%20Name :type String))
  (bind _value (Utilities|Map|Find TargetMap Resource%20Name))
  (return 0 _value ""))

(fn SetCorePoweredby
  (if (> (Variables|Default|GetCurrentHealth) 0.0)
    (LocalVariables|SetL_Distance 9999.0)
    (bind _outactors (Actor|GetAllActorsOfClass "/Game/Blueprints/EngineCores/BP_EngineCore.BP_EngineCore_C"))
    (for _array_element _outactors
      (LocalVariables|SetL_CoreArrayItem _array_element)
      (if (and (< (Transformation|GetHorizontalDistanceTo (LocalVariables|GetL_CoreArrayItem) self) (LocalVariables|GetL_Distance)) (<= (Transformation|GetHorizontalDistanceTo (LocalVariables|GetL_CoreArrayItem) self) (.distancefromcore (Variables|Default|GetMachine%20Info))))
        (LocalVariables|SetL_TempCore (LocalVariables|GetL_CoreArrayItem))
        (LocalVariables|SetL_Distance (Transformation|GetHorizontalDistanceTo (LocalVariables|GetL_CoreArrayItem) self))))
    (bind _l_tempcore (LocalVariables|GetL_TempCore)
      (:then
        (Variables|Default|SetCore%20Powered%20By _l_tempcore)
        (Variables|Enum|SetOperational%20State "NewEnumerator2")
        (Default|VerifyDependentMachine (Variables|Default|GetCore%20Powered%20By) self (.energycost (Variables|Default|GetMachine%20Info)) true))
      (:else
        (bind _asbp_fpcharacter (Utilities|Casting|CastToBP_FPCharacter (Game|GetPlayerCharacter 0)))
        (Default|DisplayAlert _asbp_fpcharacter "Machine not in range of core!")
        (Variables|Enum|SetOperational%20State "NewEnumerator0")
        (bind _core_powered_by (Variables|Default|GetCore%20Powered%20By)
          (:then
            (Default|VerifyDependentMachine _core_powered_by self (.energycost (Variables|Default|GetMachine%20Info)) false))
          (:else))))
    (else
      (bind _core_powered_by_2 (Variables|Default|GetCore%20Powered%20By)
        (:then
          (Default|VerifyDependentMachine _core_powered_by_2 self (.energycost (Variables|Default|GetMachine%20Info)) false))
        (:else)))))

(fn SetPoweredbyText)

(fn ChangeCoreState
  (CallFunction|SetCorePoweredby)
  (switch Utilities|FlowControl|Switch|SwitchonE_MachineState (Variables|Enum|GetMachineStates)
    (:NewEnumerator0
      (Variables|Enum|SetMachineStates "NewEnumerator3"))
    (:NewEnumerator3
      (CallFunction|SetPoweredbyText)
      (switch Utilities|FlowControl|Switch|SwitchonE_OperationalState (Variables|Enum|GetOperational%20State)
        (:NewEnumerator0
          (CallFunction|SetCorePoweredby)
          (Default|SetPowered (Variables|Default|GetDetailsWidget) false))
        (:NewEnumerator2
          (Default|SetPowered (Variables|Default|GetDetailsWidget) true))))))

(fn AttachtoComponet
  (Transformation|AttachComponentToComponent 0 "None" "SnapToTarget" "KeepRelative" "KeepRelative" true)
  (Variables|Enum|SetMachineStates "NewEnumerator2"))

(fn PlaceMachineDown
  (params (Player :type BP%20FP%20Character%20Object%20Reference))
  (Variables|Default|SetPlayer Player)
  (Rendering|SetVisibility (Variables|Default|GetMesh) true false)
  (Rendering|SetVisibility (Variables|Default|GetMachineDetailsWidget) true false)
  (Transformation|DetachFromActor "KeepRelative" "KeepRelative" "KeepRelative")
  (Transformation|SetActorTransform self (Math|Conversions|ToTransform(Vector) (.hitlocation (Variables|/Game/Blueprints/Player/BP_FPCharacter.BP_FPCharacter_C|GetLineTraceInfo (Variables|Default|GetPlayer)))))
  (Variables|Enum|SetMachineStates "NewEnumerator3"))

(fn CalculateWidgetRotation
  (params (Widget :type Scene%20Component%20Object%20Reference))
  (return (Math|Rotator|FindLookatRotation (Transformation|GetWorldLocation Widget) (Transformation|GetWorldLocation (Variables|/Script/Engine.PlayerCameraManager|GetTransformComponent (Game|GetPlayerCameraManager 0))))))

(fn SetWidgetRotation
  (params (Widget :type Scene%20Component%20Object%20Reference))
  (bind _returnvalue (Transformation|GetWorldRotation Widget))
  (bind (_roll _pitch) (Math|Rotator|BreakRotator _returnvalue))
  (Transformation|SetWorldRotation Widget (Math|Rotator|MakeRotator _roll _pitch (.Yaw (Math|Rotator|BreakRotator (CallFunction|CalculateWidgetRotation Widget)))) false false))

(fn ReceiveBeginPlay
  (CallFunction|SetUniqueName "None")
  (bind _returnvalue (UserInterface|CreateWidget "/Game/UI/Machines/W_MachineDetailsDiagetic.W_MachineDetailsDiagetic_C"))
  (bind _output_get (Variables|Default|SetDetailsWidget _returnvalue))
  (UserInterface|SetWidget (Variables|Default|GetMachineDetailsWidget) _output_get)
  (bind _returnvalue_2 (Actor|GetActorOfClass "/Game/Blueprints/LevelEventManager/BP_LevelEventManager.BP_LevelEventManager_C"))
  (Variables|Default|SetLevelEventManager _returnvalue_2)
  (bind _returnvalue_3 (Actor|GetActorOfClass "/Game/Blueprints/Managers/BP_CoreManager.BP_CoreManager_C"))
  (Variables|Default|SetCoreManager _returnvalue_3)
  (CallFunction|UpdateStatus))

(fn UpgradeMachine
  (bind _output_get (Variables|Default|SetMachine%20Info%20Defaults (Utilities|Struct|MakeStruct_MachineValues 0.0 0.0 0 (- (.productionrate (Variables|Default|GetMachine%20Info%20Defaults)) 0.2))))
  (Development|PrintString (Utilities|String|ToString(Float) (.ProductionRate (Utilities|Struct|BreakStruct_MachineValues _output_get)))))

(fn DisplayInteract
  (params (Actor :type Actor%20Object%20Reference))
  (if (not (Utilities|DoesObjectImplementInterface Actor "/Game/Blueprints/Robot/BPI_Robot.BPI_Robot_C"))
    (if (< (Variables|Default|GetCurrentHealth) (.maxhealth (Variables|Default|GetMachine%20Info)))
      (bind _asbp_fpcharacter (Utilities|Casting|CastToBP_FPCharacter Actor))
      (Default|DisplayInputPrompt _asbp_fpcharacter "Press E to Interact & R to Repair")
      (else
        (bind _asbp_fpcharacter_2 (Utilities|Casting|CastToBP_FPCharacter Actor))
        (Default|DisplayInputPrompt _asbp_fpcharacter_2 "Press E to Interact")))))

(fn HideInteract
  (params (Object :type Object%20Object%20Reference))
  (if (not (Utilities|DoesObjectImplementInterface Object "/Game/Blueprints/Robot/BPI_Robot.BPI_Robot_C"))
    (bind _asbp_fpcharacter (Utilities|Casting|CastToBP_FPCharacter Object))
    (Default|HideInputPrompt _asbp_fpcharacter)))

(fn RepairMachine
  (params (Player :type BP%20FP%20Character%20Object%20Reference) (Condition :type Boolean))
  (Variables|Default|SetPlayer Player)
  (if Condition
    (if (< (Variables|Default|GetCurrentHealth) (.maxhealth (Variables|Default|GetMachine%20Info)))
      (Variables|/Game/Blueprints/Player/BP_FPCharacter.BP_FPCharacter_C|SetPlayerStates (Variables|Default|GetPlayer) "NewEnumerator6")
      (Utilities|Time|ClearandInvalidateTimerbyHandle (Variables|Default|GetRepair%20Timer))
      (bind _returnvalue (Utilities|Time|SetTimerbyEvent (EventDispatchers|CreateEvent :!event RepairAction) 0.2 true))
      (Variables|Default|SetRepair%20Timer _returnvalue))
    (else
      (Utilities|Time|ClearandInvalidateTimerbyHandle (Variables|Default|GetRepair%20Timer))
      (Default|DisplayRepairing (Variables|Default|GetPlayer) (Variables|Default|GetCurrentHealth) (.maxhealth (Variables|Default|GetMachine%20Info)) false))))

(fn RepairAction
  (if (< (Variables|Default|GetCurrentHealth) (.maxhealth (Variables|Default|GetMachine%20Info)))
    (if (> (.Value (Utilities|Map|Find (Variables|/Game/Blueprints/Components/BP_Inventory.BP_Inventory_C|GetResource%20Inventory (Variables|/Game/Blueprints/Player/BP_FPCharacter.BP_FPCharacter_C|GetBP_Inventory (Variables|Default|GetPlayer))) "Gel")) 0)
      (Variables|Default|SetCurrentHealth (Math|Float|Clamp(Float) (+ (Variables|Default|GetCurrentHealth) 2e+01) 0.0 (.maxhealth (Variables|Default|GetMachine%20Info))))
      (Default|DisplayRepairing (Variables|Default|GetPlayer) (Math|Float|Clamp(Float) (+ (Variables|Default|GetCurrentHealth) 2e+01) 0.0 (.maxhealth (Variables|Default|GetMachine%20Info))) (.maxhealth (Variables|Default|GetMachine%20Info)) true)
      (Default|RemoveResourcefromInventory (Variables|/Game/Blueprints/Player/BP_FPCharacter.BP_FPCharacter_C|GetBP_Inventory (Variables|Default|GetPlayer)) "Gel" 1)
      (if (Utilities|Enum|Equal(Enum) (Variables|Enum|GetOperational%20State) "NewEnumerator1")
        (CallFunction|UpdateStatus))
      (else
        (Default|DisplayAlert (Variables|Default|GetPlayer) "You must have Gel in order to repair!")
        (Utilities|Time|ClearandInvalidateTimerbyHandle (Variables|Default|GetRepair%20Timer) :!label _label)
        (Default|DisplayRepairing (Variables|Default|GetPlayer) (Variables|Default|GetCurrentHealth) (.maxhealth (Variables|Default|GetMachine%20Info)) false)))
    (else
      (goto _label))))

(fn ActionInteract
  (params (Player :type BP%20FP%20Character%20Object%20Reference))
  (Default|HideInputPrompt Player))

(fn DropOffResourceAction
  (params (ResourceName :type Name) (Amount :type Integer))
  (Default|AddResourcetoInventory (Variables|Default|GetBP_Inventory) ResourceName Amount))

(fn UpdateStatus
  (CallFunction|SetCorePoweredby)
  (switch Utilities|FlowControl|Switch|SwitchonE_MachineState (Variables|Enum|GetMachineStates)
    (:NewEnumerator0
      (Variables|Enum|SetMachineStates "NewEnumerator3"))
    (:NewEnumerator3
      (CallFunction|SetPoweredbyText)
      (switch Utilities|FlowControl|Switch|SwitchonE_OperationalState (Variables|Enum|GetOperational%20State)
        (:NewEnumerator0
          (CallFunction|SetCorePoweredby))
        (:NewEnumerator2
          (switch Utilities|FlowControl|Switch|SwitchonE_MachineSubState (Variables|Enum|GetMachineSubStates)))))))

(fn MachineReceiveEnergy
  (params (Operational? :type Boolean))
  (if Operational?
    (switch Utilities|FlowControl|Switch|SwitchonE_OperationalState (Variables|Enum|GetOperational%20State)
      (:NewEnumerator0
        _)
      (:NewEnumerator2
        _))
    (Variables|Enum|SetOperational%20State "NewEnumerator2")
    (CallFunction|SetPoweredbyText)
    (else
      (switch Utilities|FlowControl|Switch|SwitchonE_OperationalState (Variables|Enum|GetOperational%20State)
        (:NewEnumerator0
          _)
        (:NewEnumerator2
          _))
      (Variables|Enum|SetOperational%20State "NewEnumerator0")
      (CallFunction|SetPoweredbyText))))

(fn UpgradeCraftingSpeed
  (CallFunction|UpgradeError))

(fn UpgradeRobotStationInventorySize
  (CallFunction|UpgradeError))

(fn UpgradeConvertorExtraResource
  (CallFunction|UpgradeError))

(fn UpgradeError
  (Utilities|Debugging|RaiseScriptError "Upgrade is being called from the baseclass. Please over ride the functionality of this upgrade in the child class of the machine that will use it"))

(fn UpgradeConvertorDamage
  (CallFunction|UpgradeError))

(fn UpgradeConverterDoubleCraftingSpeed
  (CallFunction|UpgradeError))

(fn UpgradeRobotStationTurboCharge
  (CallFunction|UpgradeRobotStationTurboCharge))

(fn SetUniqueName
  (params (NewName :type Name))
  (if (== NewName "")
    (bind _asbp_game_instance (Utilities|Casting|CastToBP_GameInstance (Game|GetGameInstance)))
    (bind _output_get (Variables|Default|SetName (Utilities|String|StringToName (Utilities|String|Append (Utilities|String|ToString(Name) (Variables|Default|GetMachineType)) (Utilities|String|ToString(Integer) (+ (.Value (Utilities|Map|Find (Variables|/Game/Blueprints/Managers/BP_GameInstance.BP_GameInstance_C|GetMachineHistogram _asbp_game_instance) (Variables|Default|GetMachineType))) 1))))))
    (Utilities|Map|Add (Variables|/Game/Blueprints/Managers/BP_GameInstance.BP_GameInstance_C|GetMachineHistogram _asbp_game_instance) (Variables|Default|GetMachineType) (+ (.Value (Utilities|Map|Find (Variables|/Game/Blueprints/Managers/BP_GameInstance.BP_GameInstance_C|GetMachineHistogram _asbp_game_instance) (Variables|Default|GetMachineType))) 1))
    (Utilities|Array|Add (Variables|/Game/Blueprints/Managers/BP_GameInstance.BP_GameInstance_C|GetMachineNames _asbp_game_instance) _output_get)
    (return true)
    (else
      (bind _asbp_game_instance_2 (Utilities|Casting|CastToBP_GameInstance (Game|GetGameInstance)))
      (if (== (Utilities|Array|FindItem (Variables|/Game/Blueprints/Managers/BP_GameInstance.BP_GameInstance_C|GetMachineNames _asbp_game_instance_2) NewName) -1)
        ;[0.15 0.15 0.15 0.5] UNIQUE NAME
        (Utilities|Array|SetArrayElem (Variables|/Game/Blueprints/Managers/BP_GameInstance.BP_GameInstance_C|GetMachineNames _asbp_game_instance_2) (Utilities|Array|FindItem (Variables|/Game/Blueprints/Managers/BP_GameInstance.BP_GameInstance_C|GetMachineNames _asbp_game_instance_2) (Variables|Default|GetName)) NewName)
        (Variables|Default|SetName NewName)
        (return true)
        (else
          (Development|PrintString "NOT UNIQUE")
          (return false))))))

(fn GameplayTag
  (return "(TagName=\"Interactable\")"))

(fn GetMachineHealth
  (return 0.0 0.0))

(fn GetGameplayTags
  (return (Variables|Default|GetGameplayTags)))

(fn GetIndicatorMesh
  (return 0))

(fn GetLocation
  (return (Transformation|GetActorLocation)))

(fn GetMachine
  (return self))

(fn GetMachineClass
  (return 0))

(fn GetMachineMesh
  (return 0))

(fn GetMachineTypeName
  (return (Variables|Default|GetMachineType)))

(fn GetName
  (return (Variables|Default|GetName)))

(fn GetRotation
  (return (Variables|Default|GetRotation)))

(fn HasResource
  (params (Resource%20Name :type Name :default "None"))
  (return 0 false))

(fn Interact
  (params (Player :type BP%20FP%20Character%20Object%20Reference))
  (return 0))