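; BP_Trap is a placeable trap machine that the first-person player character can build, pick up and place.
; Machine interface events attach it to the player's item socket or pickup component, then detach it at the line-trace hit location, updating machine and player states.
; It caches the player character on BeginPlay and revalidates it on placement.
; Selection and the interface getters are empty stubs, and no trap effect is implemented.
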(event EventSelection
  (params (Player :type BP%20FP%20Character%20Object%20Reference))
  ;[0.15 0.15 0.15 0.5] BPI Logic
)

(event EventPickupMachine
  (params (Player :type BP%20FP%20Character%20Object%20Reference))
  ;[0.15 0.15 0.15 0.5] BPI Logic
  (Transformation|AttachComponentToComponent (.ItemSocket (Utilities|Struct|BreakS_Linetrace (Variables|/Game/Blueprints/Player/BP_FPCharacter.BP_FPCharacter_C|GetLineTraceInfo (stale EventSelection Player)))) "None" "SnapToTarget" "KeepRelative" "KeepRelative" true)
  (Variables|Default|SetMachineState "NewEnumerator2"))

(event EventPlaceMachine
  (params (Player :type BP%20FP%20Character%20Object%20Reference))
  ;[0.15 0.15 0.15 0.5] BPI Logic
  (CallFunction|ValidatePlayerRef)
  (Transformation|DetachFromActor "KeepRelative" "KeepRelative" "KeepRelative")
  (Transformation|SetActorTransform self (Math|Transform|MakeTransform (.hitlocation (Variables|/Game/Blueprints/Player/BP_FPCharacter.BP_FPCharacter_C|GetLineTraceInfo Player)) "0, 0, 0" "1.000000,1.000000,1.000000"))
  (Variables|Default|SetMachineState "NewEnumerator3")
  (Variables|/Game/Blueprints/Player/BP_FPCharacter.BP_FPCharacter_C|SetPlayerStates (Variables|Default|GetPlayerRef) "NewEnumerator0"))

(event EventBeginPlay
  (bind _asbp_fpcharacter (Utilities|Casting|CastToBP_FPCharacter (Game|GetPlayerCharacter 0)))
  (Variables|Default|SetPlayerRef _asbp_fpcharacter))

(event EventBuildMachine
  (params (Player :type BP%20FP%20Character%20Object%20Reference))
  ;[0.15 0.15 0.15 0.5] BPI Logic
  (Variables|/Game/Blueprints/Player/BP_FPCharacter.BP_FPCharacter_C|SetBuildMachine Player self)
  (Transformation|AttachComponentToComponent (Variables|/Game/Blueprints/Player/BP_FPCharacter.BP_FPCharacter_C|GetObjectPickup Player) "None" "SnapToTarget" "KeepRelative" "KeepRelative" true)
  (Variables|Default|SetMachineState "NewEnumerator2"))

(fn ConstructionScript)

(fn ValidatePlayerRef
  (Utilities|IsValid (Variables|Default|GetPlayerRef)
    (:Is%20Not%20Valid
      (bind _asbp_fpcharacter (Utilities|Casting|CastToBP_FPCharacter (Game|GetPlayerCharacter 0)))
      (Variables|Default|SetPlayerRef _asbp_fpcharacter))))

(fn GameplayTag
  (return ""))

(fn GetGameplayTags
  (return ""))

(fn GetLocation
  (return "0, 0, 0"))

(fn GetMachine
  (return 0))

(fn GetMachineClass
  (return 0))

(fn GetMachineMesh
  (return 0))

(fn GetName
  (return "None"))

(fn HasResource
  (params (Resource%20Name :type Name :default "None"))
  (return 0 false))