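; Mini black hole trap that pulls enemies toward itself when they enter its sphere.
; Overlapping BP_Enemy actors are recorded once in EnemiesInTrap and told to pull into the trap's transform.
; It starts a Lifespan timer and, after a short delay, subscribes as an observer to BP_LevelEventManager.
; A Died notification triggers Destroy, which sends trapped enemies back to their attack targets before removing the actor.
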(event OnComponentBeginOverlap(Sphere1)
  (params (OverlappedComponent :type Primitive%20Component%20Object%20Reference) (OtherActor :type Actor%20Object%20Reference) (OtherComp :type Primitive%20Component%20Object%20Reference) (OtherBodyIndex :type Integer) (bFromSweep :type Boolean) (SweepResult :type Hit%20Result%20Structure%20%28by%20ref%29))
  (if (Utilities|DoesObjectImplementInterface OtherActor "/Game/Blueprints/Enemy/BPI_Enemy.BPI_Enemy_C")
    (bind _asbp_enemy (Utilities|Casting|CastToBP_Enemy OtherActor))
    (if (not (Utilities|Array|ContainsItem (Variables|Default|GetEnemiesInTrap) _asbp_enemy))
      (Utilities|Array|Add (Variables|Default|GetEnemiesInTrap) _asbp_enemy)
      (Default|PullIntoTrap _asbp_enemy (Transformation|GetActorTransform)))))

(event EventBeginPlay
  (|CallParentFunction)
  (Utilities|Time|SetTimerbyEvent (EventDispatchers|CreateEvent :!event Destroy) (Variables|Default|GetLifespan))
  (Utilities|FlowControl|Delay 0.2)
  (bind _returnvalue (Actor|GetActorOfClass "/Game/Blueprints/LevelEventManager/BP_LevelEventManager.BP_LevelEventManager_C"))
  (Default|SubscribeObserver _returnvalue self))

(event EventOnNotify
  (params (EventType :type E_LevelEventType%20Enum :default "NewEnumerator0"))
  (switch Utilities|FlowControl|Switch|SwitchonE_LevelEventType EventType
    (:NewEnumerator13
      (CallFunction|Destroy))))

(fn ConstructionScript
  (|CallParentFunction))

(fn Destroy
  (for _array_element (Variables|Default|GetEnemiesInTrap)
    (Default|NavigatetoAttackTarget _array_element))
  (Actor|DestroyActor))