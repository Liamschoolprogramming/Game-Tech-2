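; BP_Machine_RefineryTutorial is a tutorial variant of the refinery machine that starts play with zero health.
; On BeginPlay it runs the parent logic, then overrides health and operational state and refreshes its status.
; It supplies its name, Machine gameplay tag, arrow-based location and mesh through simple getters.
; Construction and player interaction defer entirely to the parent class.
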(event EventBeginPlay
  (|CallParentFunction)
  (Variables|Default|SetCurrentHealth 0.0)
  (Variables|Default|SetOperational%20State "NewEnumerator1")
  (CallFunction|UpdateStatus))

(fn ConstructionScript
  (|CallParentFunction))

(fn GetName
  (return (Variables|Default|GetName)))

(fn GameplayTag
  (return "(TagName=\"Machine\")"))

(fn GetLocation
  (return (Transformation|GetWorldLocation (Variables|Default|GetArrow))))

(fn GetMachineMesh
  (return (Variables|Character|GetMesh)))

(fn ActionInteract
  (params (Player :type BP%20FP%20Character%20Object%20Reference))
  (|CallParentFunction Player))