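; Refinery machine Blueprint, a child of a base machine class that supplies most of its behavior.
; BeginPlay and construction defer to the parent, and the Upgrade event calls UpgradeMachine, which prints a debug string before running the parent upgrade.
; Getters expose its name, Machine gameplay tag, arrow location and mesh.
; A CelestialOre recipe lookup meant to override the base RecipeInventory is disconnected and never runs.
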(event EventBeginPlay
  (|CallParentFunction))

(event EventUpgrade
  (CallFunction|UpgradeMachine))

(fn ConstructionScript
  (|CallParentFunction))

(fn GetName
  (return (Variables|Default|Getname)))

(fn GameplayTag
  (return "(TagName=\"Machine\")"))

(fn GetLocation
  (return (Transformation|GetWorldLocation (Variables|Default|GetArrow))))

(fn GetMachineMesh
  (return (Variables|Character|GetMesh)))

(fn UpgradeMachine
  (Development|PrintString "1")
  (|CallParentFunction))