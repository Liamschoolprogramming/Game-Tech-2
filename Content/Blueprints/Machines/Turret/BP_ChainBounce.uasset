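; BP_ChainBounce is one link of a turret's chain lightning, damaging its hit actor on a looping timer over a short lifespan.
; SetSpawnInfo attaches it to the parent actor and spawns a Niagara lightning effect using the hit actor's mesh as Origin.
; It usually spawns another link recursively on the first other BP_Enemy passing a distance check, with the current target as parent.
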(event Custom|SetSpawnInfo
  (params (Hit%20Actor :type Actor%20Object%20Reference) (Damage :type Float%20%28double-precision%29) (Causer :type Actor%20Object%20Reference) (Parent :type Actor%20Object%20Reference))
  (bind _output_get (Variables|Default|SetHit%20Actor Hit%20Actor))
  (bind _static_mesh (Class|BPIEnemy|GetStaticMesh(Message) _output_get))
  (Variables|Default|SetHit%20Mesh _static_mesh)
  (Variables|Default|SetDamage Damage)
  (Variables|Default|SetCauser Causer)
  (Utilities|IsValid Parent
    (:Is%20Valid
      (Transformation|AttachActorToActor Parent "None" "SnapToTarget" "KeepRelative" "KeepRelative" true)
      (bind _returnvalue (Niagara|SpawnSystemAttached "/Game/Blueprints/Machines/Turret/NS_LightningAttach.NS_LightningAttach" (Variables|Default|GetCube) "" "0, 0, 0" "0, 0, 0" "KeepRelativeOffset" false))
      (Class|NiagaraFunctionLibrary|OverrideSystemUserVariableStaticMeshComponent _returnvalue "Origin" (Variables|Default|GetHit%20Mesh))
      (Utilities|Time|SetTimerbyEvent (delegate Custom|Apply%20Damage) 0.2 true false 0.5)
      (Actor|SetLifeSpan 2.0)
      (if (< (Math|Random|RandomIntegerinRange 1 10) 10)
        (bind _enemy (CallFunction|IsEnemyinChainRange))
        (Utilities|IsValid _enemy
          (:Is%20Valid
            (bind _returnvalue_2 (Game|SpawnActorfromClass "BP_ChainBounce_C" (Math|Transform|MakeTransform "0, 0, 0" "0, 0, 0" "1.000000,1.000000,1.000000") "Undefined" "MultiplyWithRoot" 0 0))
            (CallFunction|SetSpawnInfo _returnvalue_2 _enemy (Variables|Default|GetDamage) (Variables|Default|GetCauser) (Variables|Default|GetHit%20Actor))))))
    (:Is%20Not%20Valid
      (Actor|DestroyActor))))

(event Custom|Apply%20Damage
  (Game|Damage|ApplyDamage (Variables|Default|GetHit%20Actor) (Variables|Default|GetDamage) 0 (Variables|Default|GetCauser))
  (Utilities|IsValid (Variables|Default|GetHit%20Actor)
    (:Is%20Not%20Valid
      (Actor|DestroyActor))))

(fn ConstructionScript)

(fn ChainBounce
  (params (Niagara%20System :type Niagara%20Component%20Object%20Reference)))

(fn IsEnemyinChainRange
  (bind _outactors (Actor|GetAllActorsOfClass "/Game/Blueprints/Enemy/BP_Enemy.BP_Enemy_C"))
  (for _array_element _outactors
    (if (and (!= (Variables|Default|GetHit%20Actor) _array_element) (< (Math|Vector|Distance(Vector) (Transformation|GetActorLocation) (Transformation|GetActorLocation)) 2e+03))
      (return _array_element)))
  (return 0))