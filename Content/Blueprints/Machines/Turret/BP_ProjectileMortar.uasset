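; BP_ProjectileMortar is a mortar turret projectile that overrides SetIsActive to launch and shut down rather than spawn or destroy itself.
; Activation sets velocity along its forward vector and deactivates it after a fixed delay, while deactivation zeroes velocity; both enlarge it when Charged.
; Overlapping a static mesh component on a BPI_Interactable actor applies the turret's base damage and stops movement.
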(event OnComponentBeginOverlap(Collision)
  (params (OverlappedComponent :type Primitive%20Component%20Object%20Reference) (OtherActor :type Actor%20Object%20Reference) (OtherComp :type Primitive%20Component%20Object%20Reference) (OtherBodyIndex :type Integer) (bFromSweep :type Boolean) (SweepResult :type Hit%20Result%20Structure%20%28by%20ref%29))
  (if (Utilities|DoesObjectImplementInterface OtherActor "/Game/Blueprints/BPI_Interactable.BPI_Interactable_C")
    (if (== (Utilities|GetClass OtherComp) "/Script/Engine.StaticMeshComponent")
      (Game|Damage|ApplyDamage OtherActor (.basedamage (Variables|Default|GetTurret%20Stats)) 0 (Components|GetOwner) "/Script/Engine.DamageType")
      (Components|Movement|StopMovementImmediately (Variables|Default|GetProjectileMovement)))))

(event EventBeginPlay
  (|CallParentFunction) ; This node is disabled and will not be called.\nDrag off pins to build functionality.
)

(event EventSetIsActive
  (params (IsActive :type Boolean))
  (|CallParentFunction IsActive)
  (if (Variables|Default|GetIsActive)
    (Variables|/Script/Engine.MovementComponent|SetVelocity (Variables|Default|GetProjectileMovement) (* (Transformation|GetActorForwardVector) (Variables|Default|GetSpeed)))
    (if (Variables|Default|GetCharged?)
      (Transformation|SetActorScale3D "6.000000,6.000000,6.000000")
      (else
        (Transformation|SetActorScale3D "1.000000,1.000000,1.000000")))
    (Utilities|FlowControl|Delay 2.0)
    (CallFunction|SetIsActive false)
    (else
      (Variables|/Script/Engine.MovementComponent|SetVelocity (Variables|Default|GetProjectileMovement) "0, 0, 0")
      (if (Variables|Default|GetCharged?)
        (Transformation|SetActorScale3D "6.000000,6.000000,6.000000")
        (else
          (Transformation|SetActorScale3D "1.000000,1.000000,1.000000"))))))

(fn ConstructionScript
  (|CallParentFunction))