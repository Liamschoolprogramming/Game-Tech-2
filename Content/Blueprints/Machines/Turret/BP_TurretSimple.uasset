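; BP_TurretSimple is a turret machine that uses BP_ProjectileSimple as its projectile.
; On BeginPlay it runs the parent logic, then pre-spawns a small batch of projectiles owned by itself, passing in its TurretInfo stats and storing them in the Projectiles array.
; It overrides GetIndicatorMesh to supply the TurretSimplePreview mesh, leaving other behavior to the parent class.
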(event EventBeginPlay
  (|CallParentFunction)
  (for _index (range 0 4)
    (bind _returnvalue (Game|SpawnActorfromClass "/Game/Blueprints/Machines/Turret/BP_ProjectileSimple.BP_ProjectileSimple_C" (Math|Transform|MakeTransform "0, 0, 0" "0, 0, 0" "1.000000,1.000000,1.000000") "AlwaysSpawn" "MultiplyWithRoot" self (Variables|Default|GetTurret%20Info) self))
    (Utilities|Array|Add (Variables|Default|GetProjectiles) _returnvalue)))

(fn ConstructionScript
  (|CallParentFunction))

(fn GetIndicatorMesh
  (return "/Game/Assets/Turrets/TurretSimplePreview.TurretSimplePreview"))