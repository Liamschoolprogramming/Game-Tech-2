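; BP_ProjectileSimple is a turret projectile that damages actors implementing BPI_Enemy on overlap.
; Activation launches it along its forward vector, then deactivates it after a short delay, zeroing velocity, rather than destroying it.
; The Charged flag enlarges the projectile, yet selects plain turret base damage, while uncharged shots deal triple.
; Hits leave it active, and damage credits the first player controller as instigator.
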(event OnComponentBeginOverlap(Collision)
  (params (OverlappedComponent :type Primitive%20Component%20Object%20Reference) (OtherActor :type Actor%20Object%20Reference) (OtherComp :type Primitive%20Component%20Object%20Reference) (OtherBodyIndex :type Integer) (bFromSweep :type Boolean) (SweepResult :type Hit%20Result%20Structure%20%28by%20ref%29))
  (bind _turret_stats (Variables|Default|GetTurret%20Stats))
  ;[0.15 0.15 0.15 0.5] If projectile comes in contact with an ememy, deal damage
  (if (Utilities|DoesObjectImplementInterface OtherActor "/Game/Blueprints/Enemy/BPI_Enemy.BPI_Enemy_C")
    (Game|Damage|ApplyDamage OtherActor (Math|Float|SelectFloat (.basedamage _turret_stats) (* (.basedamage _turret_stats) 3.0) (Variables|Default|GetCharged?)) (Game|GetPlayerController 0) (Components|GetOwner) "/Script/Engine.DamageType")))

(event EventBeginPlay
  (|CallParentFunction))

(event EventSetIsActive
  (params (IsActive :type Boolean))
  ;[0.15 0.15 0.15 0.5] Projectile Fired / Stopped
  (|CallParentFunction IsActive)
  (if (Variables|Default|GetIsActive)
    (Variables|/Script/Engine.MovementComponent|SetVelocity (Variables|Default|GetProjectileMovement) (* (Transformation|GetActorForwardVector) (Variables|Default|GetSpeed)))
    (if (Variables|Default|GetCharged?)
      (Transformation|SetActorScale3D "6.000000,6.000000,6.000000")
      (else
        (Transformation|SetActorScale3D "1.000000,1.000000,1.000000")))
    (Utilities|FlowControl|Delay 0.2)
    (CallFunction|SetIsActive false)
    (else
      (Variables|/Script/Engine.MovementComponent|SetVelocity (Variables|Default|GetProjectileMovement) "0, 0, 0")
      (if (Variables|Default|GetCharged?)
        (Transformation|SetActorScale3D "6.000000,6.000000,6.000000")
        (else
          (Transformation|SetActorScale3D "1.000000,1.000000,1.000000"))))))

(fn ConstructionScript
  (|CallParentFunction))