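; Base turret machine that automatically tracks and shoots enemies entering its sight range.
; Overlap events maintain a target list and pick one by targeting mode (distance or health), with the lowest-health comparison never reading the candidate's health.
; Looping timers drive head yaw, return to rest and line-trace damage that ignores other machines; the firing timer is never cleared.
; Interact moves the player to the turret and disables their movement.
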(event OnComponentBeginOverlap(SightRange)
  (params (OverlappedComponent :type Primitive%20Component%20Object%20Reference) (OtherActor :type Actor%20Object%20Reference) (OtherComp :type Primitive%20Component%20Object%20Reference) (OtherBodyIndex :type Integer) (bFromSweep :type Boolean) (SweepResult :type Hit%20Result%20Structure%20%28by%20ref%29))
  ;[0.15 0.15 0.15 0.5] Sets target when an enemy enters turret sight radius
  (if (Utilities|DoesObjectImplementInterface OtherActor "/Game/Blueprints/Enemy/BPI_Enemy.BPI_Enemy_C")
    (Utilities|Array|AddUnique (Variables|Default|GetAvailableTargets) OtherActor)
    (bind _target (CallFunction|DetermineTarget))
    (if (Utilities|IsValid _target)
      (CallFunction|Attack)
      ;[0.15 0.15 0.15 0.5] Rotates the Head of the turret towards the designated target enemy
      (Utilities|Time|ClearandInvalidateTimerbyHandle (Variables|Default|GetReturn%20Rotate%20Timer))
      (bind _returnvalue (Utilities|Time|SetTimerbyEvent (delegate Custom|Rotate%20To%20Target) 0.01 true true))
      (Variables|Default|SetAttack%20Rotate%20Timer _returnvalue)
      (else
        (CallFunction|ReturntoRest)))))

(event OnComponentEndOverlap(SightRange)
  (params (OverlappedComponent :type Primitive%20Component%20Object%20Reference) (OtherActor :type Actor%20Object%20Reference) (OtherComp :type Primitive%20Component%20Object%20Reference) (OtherBodyIndex :type Integer))
  ;[0.15 0.15 0.15 0.5] Resets target when enemy leaves turret sight radius, and goes back to forward facing if no target exists
  (if (Utilities|DoesObjectImplementInterface OtherActor "/Game/Blueprints/Enemy/BPI_Enemy.BPI_Enemy_C")
    (Utilities|Array|RemoveItem (Variables|Default|GetAvailableTargets) OtherActor)
    (bind _target (CallFunction|DetermineTarget))
    (if (Utilities|IsValid _target)
      (CallFunction|Attack)
      ;[0.15 0.15 0.15 0.5] Rotates the Head of the turret towards the designated target enemy
      (Utilities|Time|ClearandInvalidateTimerbyHandle (Variables|Default|GetReturn%20Rotate%20Timer))
      (bind _returnvalue (Utilities|Time|SetTimerbyEvent (delegate Custom|Rotate%20To%20Target) 0.01 true true))
      (Variables|Default|SetAttack%20Rotate%20Timer _returnvalue)
      (else
        (CallFunction|ReturntoRest)))))

(event Custom|Rotate%20To%20Target
  (bind _head (Variables|Default|GetHead))
  ;[0.15 0.15 0.15 0.5] Rotates the Head of the turret towards the designated target enemy
  (Utilities|IsValid (Variables|Default|GetTarget)
    (:Is%20Valid
      (Transformation|SetWorldRotation (Variables|Default|GetHead) (Math|Rotator|MakeRotator 0.0 0.0 (.yaw (Math|Interpolation|RInterpTo (Transformation|GetWorldRotation _head) (Math|Rotator|FindLookatRotation (Transformation|GetWorldLocation _head) (Transformation|GetActorLocation (Variables|Default|GetTarget))) (Utilities|Time|GetGameTimeinSeconds) 0.5))) false false))
    (:Is%20Not%20Valid
      (CallFunction|ReturntoRest))))

(event Custom|Return%20To%20Rest
  ;[0.15 0.15 0.15 0.5] Returns turret Head back to resting 0,0,0 rotation when no enemies are targeted
  (Utilities|Time|ClearandInvalidateTimerbyHandle (Variables|Default|GetAttack%20Rotate%20Timer))
  (bind _returnvalue (Utilities|Time|SetTimerbyEvent (delegate Custom|Go%20Back) 0.01 true true))
  (Variables|Default|SetReturn%20Rotate%20Timer _returnvalue))

(event Custom|Go%20Back
  ;[0.15 0.15 0.15 0.5] Returns turret Head back to resting 0,0,0 rotation when no enemies are targeted
  (Transformation|SetWorldRotation (Variables|Default|GetHead) (Math|Rotator|MakeRotator 0.0 0.0 (.yaw (Math|Interpolation|RInterpTo (Transformation|GetWorldRotation (Variables|Default|GetHead)) "0, 0, 0" (Utilities|Time|GetGameTimeinSeconds) 0.01))) false false))

(event Custom|Attack
  ;[0.15 0.15 0.15 0.5] Attack target
  (bind _returnvalue (Utilities|Time|SetTimerbyEvent (delegate Custom|Shoot) (.FireRate (Utilities|Struct|BreakStruct_TurretValues (Variables|Default|GetTurret%20Info))) true))
  (Variables|Default|SetShooting%20Timer _returnvalue))

(event Custom|Shoot
  (bind _target (Variables|Default|GetTarget))
  ;[0.15 0.15 0.15 0.5] Attack target
  (bind _outactors (Actor|GetAllActorswithInterface "/Game/Blueprints/Machines/BPI_Machine.BPI_Machine_C"))
  (Utilities|IsValid _target
    (:Is%20Valid
      (bind (_outhit _returnvalue) (Collision|LineTraceByChannel (Transformation|GetWorldLocation (Variables|Default|GetBarrel)) (Transformation|GetActorLocation _target) "TraceTypeQuery3" false _outactors "ForDuration"))
      (if _returnvalue
        (if (Utilities|DoesObjectImplementInterface (.HitActor (Collision|BreakHitResult _outhit)) "/Game/Blueprints/Enemy/BPI_Enemy.BPI_Enemy_C")
          (Game|Damage|ApplyDamage (.HitActor (Collision|BreakHitResult _outhit)) (.BaseDamage (Utilities|Struct|BreakStruct_TurretValues (Variables|Default|GetTurret%20Info))) 0 self))))))

(event EventInteract
  (params (Player :type BP%20FP%20Character%20Object%20Reference))
  (bind _returnvalue (Transformation|GetActorTransform))
  (bind _charactermovement (Variables|/Script/Engine.Character|GetCharacterMovement Player))
  (Development|PrintString "interact")
  (Transformation|SetActorTransform Player (Math|Transform|MakeTransform (+ (.location _returnvalue) "-200.000000,0.000000,0.000000") (.rotation _returnvalue) "1.000000,1.000000,1.000000") true)
  (Components|Movement|StopMovementImmediately _charactermovement)
  (Pawn|Components|CharacterMovement|DisableMovement _charactermovement))

(event EventBeginPlay)

(fn ConstructionScript)

(fn DetermineTarget
  (switch Utilities|FlowControl|Switch|SwitchonEnum_TargetingMode (Variables|Default|GetTargeting%20Mode)
    (:NewEnumerator0
      (bind _target (CallFunction|TargetClosestEnemy))
      (return _target))
    (:NewEnumerator1
      (bind _target_2 (CallFunction|TargetFarthestEnemy))
      (return _target_2))
    (:NewEnumerator2
      (bind _target_3 (CallFunction|TargetHighestHealthEnemy))
      (return _target_3))
    (:NewEnumerator3
      (bind _target_4 (CallFunction|TargetLowestHealthEnemy))
      (return _target_4))))

(fn TargetClosestEnemy
  (LocalVariables|SetDistance 99999.0)
  (for _array_element (Variables|Default|GetAvailableTargets)
    (if (< (Transformation|GetDistanceTo _array_element) (LocalVariables|GetDistance))
      (LocalVariables|SetTemp%20Target _array_element)
      (LocalVariables|SetDistance (Transformation|GetDistanceTo _array_element))))
  (bind _output_get (Variables|Default|SetTarget (LocalVariables|GetTemp%20Target)))
  (return _output_get))

(fn TargetFarthestEnemy
  (LocalVariables|SetDistance 0.0)
  (for _array_element (Variables|Default|GetAvailableTargets)
    (if (> (Transformation|GetDistanceTo _array_element) (LocalVariables|GetDistance))
      (LocalVariables|SetTemp%20Target _array_element)
      (LocalVariables|SetDistance (Transformation|GetDistanceTo _array_element))))
  (bind _output_get (Variables|Default|SetTarget (LocalVariables|GetTemp%20Target)))
  (return _output_get))

(fn TargetLowestHealthEnemy
  (LocalVariables|SetEnemyHealth 9999.0)
  (for _array_element (Variables|Default|GetAvailableTargets)
    (bind _currenthealth (Class|BPIEnemy|GetEnemyCurrentHP(Message) _array_element))
    (if (< 0.0 (LocalVariables|GetEnemyHealth))
      (LocalVariables|SetTemp%20Target _array_element)
      (LocalVariables|SetEnemyHealth _currenthealth)))
  (bind _output_get (Variables|Default|SetTarget (LocalVariables|GetTemp%20Target)))
  (return _output_get))

(fn TargetHighestHealthEnemy
  (for _array_element (Variables|Default|GetAvailableTargets)
    (bind _currenthealth (Class|BPIEnemy|GetEnemyCurrentHP(Message) _array_element))
    (if (> _currenthealth (LocalVariables|GetEnemyHealth))
      (LocalVariables|SetTemp%20Target _array_element)
      (LocalVariables|SetEnemyHealth _currenthealth)))
  (bind _output_get (Variables|Default|SetTarget (LocalVariables|GetTemp%20Target)))
  (return _output_get))

(fn GameplayTag
  (return ""))

(fn GetMachineHealth
  (return (Variables|Default|GetCurrent%20Health) (.MaxHealth (Utilities|Struct|BreakStruct_TurretValues (Variables|Default|GetTurret%20Info)))))

(fn HasResource
  (params (Resource%20Robot%20Is%20Looking%20For :type Name :default "None"))
  (return "None" 0 0))