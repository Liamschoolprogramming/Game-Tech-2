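; Pooled turret projectile that fires a bubble forward, which expands and deals area damage over time to enemies inside it.
; Activation sets velocity and a timeline grows it from tiny to full size, larger when charged.
; Once expanded, a looping timer sphere-traces at a scale-based radius, damaging BPI_Enemy actors, with triple damage when charged.
; After a fixed lifetime it deactivates itself, clearing the timer and stopping movement.
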(event Custom|Damage%20Tick
  (bind _returnvalue (Transformation|GetActorLocation))
  (bind _turret_stats (Variables|Default|GetTurret%20Stats))
  (bind _outhits (Collision|MultiSphereTraceByChannel _returnvalue _returnvalue (* (.x (Transformation|GetActorScale3D)) 25.0) "TraceTypeQuery3" false 0 "None"))
  (for _array_element _outhits
    (if (Utilities|DoesObjectImplementInterface (.HitActor (Collision|BreakHitResult _array_element)) "/Game/Blueprints/Enemy/BPI_Enemy.BPI_Enemy_C")
      (Game|Damage|ApplyDamage (.HitActor (Collision|BreakHitResult _array_element)) (Math|Float|SelectFloat (* (.basedamage _turret_stats) 3.0) (.basedamage _turret_stats) (Variables|Default|GetCharged?)) 0 self))))

(event EventBeginPlay
  (|CallParentFunction))

(event EventSetIsActive
  (params (IsActive :type Boolean))
  (|CallParentFunction IsActive)
  (if (Variables|Default|GetIsActive)
    (Variables|/Script/Engine.MovementComponent|SetVelocity (Variables|Default|GetProjectileMovement) (* (Transformation|GetActorForwardVector) (Variables|Default|GetSpeed)))
    (Transformation|SetActorScale3D (Math|Conversions|ToVector(Float) 0.01))
    (if (Variables|Default|GetCharged?)
      (Variables|Default|SetScale (Math|Conversions|ToVector(Float) 11.0))
      (bind _newtrack_1 (Timeline|Expand%20Timelines PlayFromStart)
        (:Update
          (Transformation|SetActorScale3D (* (Variables|Default|GetScale) _newtrack_1)))
        (:Finished
          (bind _returnvalue (Utilities|Time|SetTimerbyEvent (delegate Custom|Damage%20Tick) 0.25 true))
          (Variables|Default|SetTickDamageTimer _returnvalue)
          (Utilities|FlowControl|Delay 1e+01)
          (CallFunction|SetIsActive false)))
      (else
        (Variables|Default|SetScale (Math|Conversions|ToVector(Float) 7.0))
        (Timeline|Expand%20Timelines PlayFromStart)))
    (else
      (Variables|Default|SetSpeed 1.5e+02)
      (Variables|/Script/Engine.MovementComponent|SetVelocity (Variables|Default|GetProjectileMovement) "0, 0, 0")
      (Utilities|Time|ClearandInvalidateTimerbyHandle (Variables|Default|GetTickDamageTimer)))))

(fn ConstructionScript
  (|CallParentFunction))