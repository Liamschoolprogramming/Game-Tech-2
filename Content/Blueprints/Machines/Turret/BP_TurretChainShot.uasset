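; Chain-shot turret Blueprint that shows a Niagara lightning effect on enemies in front of its barrel, extending a parent turret.
; The overridden shooting loop gets a target when automated, line traces from the barrel and passes enemy hits to FiringChainShot, which feeds the actor to the lightning.
; Without a target it returns to rest.
; Manual mode only traces and calls the empty FiringEffects, and no damage is applied here.
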(event Custom|CustomEvent
  (bind _ns_lightning (Variables|Default|GetNS_Lightning))
  (Transformation|SetWorldLocation _ns_lightning (+ (Transformation|GetWorldLocation _ns_lightning) "10.000000,10.000000,0.000000") false false))

(event EventBeginPlay
  (bind _ns_lightning (Variables|Default|GetNS_Lightning))
  (|CallParentFunction)
  (Components|Activation|Activate _ns_lightning false)
  (Class|NiagaraFunctionLibrary|OverrideSystemUserVariableStaticMesh _ns_lightning "Source Actor" (Variables|/Script/Engine.StaticMeshComponent|GetStaticMesh (Variables|Default|GetHead))))

(fn ConstructionScript
  (|CallParentFunction))

(fn ShootatTargetLoop
  (bind _head (Variables|Default|GetHead))
  (bind _returnvalue (Transformation|GetSocketLocation _head "barrel"))
  ;[0.15 0.15 0.15 0.5] If chooses to shoot and able to shoot, fire a line trace - if the line trace hits an enemy shoot a projectile - if there is no target, return to resting position
  (if (Variables|Default|GetWants%20to%20Fire?)
    (if (Variables|Default|GetCan%20fire?)
      (bind _outactors (Actor|GetAllActorswithInterface "/Game/Team_Folders/Liam/BPI_Interactable.BPI_Interactable_C"))
      (LocalVariables|SetL_ActorsToIgnore _outactors)
      (LocalVariables|SetL_StartTrace _returnvalue)
      (LocalVariables|SetL_EndTrace (+ _returnvalue (* (Math|Vector|GetForwardVector (Variables|Default|GetHead)) 4e+03)))
      (if (not (Variables|Default|GetManually%20Operated?))
        (bind _target (CallFunction|DetermineTarget))
        (Utilities|IsValid _target
          (:Is%20Valid
            (bind (_outhit _returnvalue_2) (Collision|LineTraceByChannel (LocalVariables|GetL_StartTrace) (LocalVariables|GetL_EndTrace) "TraceTypeQuery3" false (LocalVariables|GetL_ActorsToIgnore) "None"))
            (if _returnvalue_2
              (if (Utilities|DoesObjectImplementInterface (.HitActor (Collision|BreakHitResult _outhit)) "/Game/Blueprints/Enemy/BPI_Enemy.BPI_Enemy_C")
                (bind _static_mesh (Class|BPIEnemy|GetStaticMesh(Message) (.HitActor (Collision|BreakHitResult _outhit))))
                (Development|PrintString (Utilities|String|Append "Static mesh: " (Utilities|GetDisplayName _static_mesh)))
                (CallFunction|FiringChainShot true _static_mesh (.HitActor (Collision|BreakHitResult _outhit))))))
          (:Is%20Not%20Valid
            (switch Utilities|FlowControl|Switch|SwitchonE_OperationalState (Variables|Default|GetOperational%20State)
              (:NewEnumerator0
                _)
              (:NewEnumerator2
                _))
            (CallFunction|ReturntoRest)))
        (else
          (Collision|LineTraceByChannel (LocalVariables|GetL_StartTrace) (LocalVariables|GetL_EndTrace) "TraceTypeQuery3" false (LocalVariables|GetL_ActorsToIgnore) "None")
          (CallFunction|FiringEffects)))
      (else
        (Utilities|Time|ClearandInvalidateTimerbyHandle (Variables|Default|GetShooting%20Timer) :!label _label)))
    (else
      (goto _label))))

(fn FiringEffects)

(fn FiringChainShot
  (params (Activate? :type Boolean) (Hit%20Mesh :type Static%20Mesh%20Object%20Reference) (Hit%20Actor :type Actor%20Object%20Reference))
  (if Activate?
    (Effects|Components|ParticleSystem|SetActorParameter (Variables|Default|GetNS_Lightning) "TargetStaticMesh" Hit%20Actor)
    (Components|Activation|Activate (Variables|Default|GetNS_Lightning) false)))