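; BP_ProjectileTemp is a turret projectile that is toggled on and off through SetIsActive rather than spawned or destroyed in its own graph.
; It starts inactive, with its sphere hidden and velocity zeroed.
; Activation shows the sphere and launches it along the actor's forward vector at high speed through ProjectileMovement.
; After a brief delay it calls SetIsActive again to hide and stop itself.
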(event Custom|Set%20IsActive
  (params (IsActive :type Boolean))
  (bind _projectilemovement (Variables|Default|GetProjectileMovement))
  (bind _output_get (Variables|Default|SetIsActive IsActive))
  (Rendering|SetVisibility (Variables|Default|GetSphere) _output_get false)
  (if (Variables|Default|GetIsActive)
    (Variables|/Script/Engine.MovementComponent|SetVelocity _projectilemovement (* (Transformation|GetActorForwardVector) 2e+04))
    (Utilities|FlowControl|Delay 0.1)
    (CallFunction|SetIsActive false)
    (else
      (Variables|/Script/Engine.MovementComponent|SetVelocity _projectilemovement "0, 0, 0"))))

(event EventBeginPlay
  (CallFunction|SetIsActive false))

(fn ConstructionScript)