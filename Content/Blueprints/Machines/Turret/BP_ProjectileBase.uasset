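; Base turret projectile actor that toggles between active and inactive states, starting inactive on BeginPlay.
; SetIsActive stores the flag and switches sphere visibility and actor collision to match, so the actor can be toggled without being destroyed.
; Logic for forward launch velocity, larger charged-shot scale and timed auto-deactivation exists in the graph but is disconnected, so it never runs.
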(event Custom|Set%20IsActive
  (params (IsActive :type Boolean))
  ;[0.15 0.15 0.15 0.5] Sets projectile viisble and gives it velocity if it is active, and sets it invisible and removes velocity when inactive
  (Variables|Default|SetIsActive IsActive)
  (Rendering|SetVisibility (Variables|Default|GetSphere) (Variables|Default|GetIsActive) false)
  (Collision|SetActorEnableCollision (Variables|Default|GetIsActive)))

(event EventBeginPlay
  ;[0.15 0.15 0.15 0.5] Auto set to inactive when created
  (CallFunction|SetIsActive false))

(fn ConstructionScript)