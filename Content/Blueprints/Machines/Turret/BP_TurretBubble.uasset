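; Bubble turret machine, a child turret Blueprint that shoots bubble projectiles either automatically or under manual control.
; BeginPlay pre-spawns a small projectile pool, which firing functions reposition and reactivate.
; Attack starts a looping timer that fires off cooldown: automatic mode needs a target and an enemy trace hit, manual mode ignores the trace result.
; Charged shots multiply projectile speed and launch from the camera when manually operated.
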(event EventBeginPlay
  (|CallParentFunction)
  (for _index (range 0 2)
    (bind _returnvalue (Game|SpawnActorfromClass "/Game/Blueprints/Machines/Turret/BP_ProjectileBubble.BP_ProjectileBubble_C" (Math|Transform|MakeTransform "0, 0, 0" "0, 0, 0" "1.000000,1.000000,1.000000") "AlwaysSpawn" "MultiplyWithRoot" self (Variables|Default|GetTurret%20Info) self))
    (Utilities|Array|Add (Variables|Default|GetProjectiles) _returnvalue)))

(fn ConstructionScript
  (|CallParentFunction))

(fn FiringEffects
  (bind _turret_info (Variables|Default|GetTurret%20Info))
  (bind _firerate (Utilities|Struct|BreakStruct_TurretValues _turret_info))
  (bind _returnvalue (* _firerate 0.75))
  (bind _returnvalue_2 (select false _returnvalue _firerate))
  (bind _chosen_projectile (CallFunction|FirstAvailableProjectile))
  (LocalVariables|SetL_ChosenProjectile _chosen_projectile)
  (Transformation|SetActorLocationAndRotation (LocalVariables|GetL_ChosenProjectile) (Transformation|GetSocketLocation (Variables|Default|GetHead) "barrel") (Variables|Default|GetSocket%20Rotation))
  (Variables|/Game/Blueprints/Machines/Turret/BP_ProjectileBase.BP_ProjectileBase_C|SetCharged? (LocalVariables|GetL_ChosenProjectile) false)
  (Default|SetIsActive (LocalVariables|GetL_ChosenProjectile) true)
  (bind _hud_other (Variables|Default|GetHUD%20Other)
    (:then
      (if (Variables|Default|GetManually%20Operated?)
        (Default|SetTimer _hud_other _returnvalue_2)))
    (:else
      _))
  (Utilities|Time|SetTimerbyFunctionName 0 "LowerCooldown" _returnvalue_2))

(fn Attack
  (if (not (Utilities|Time|IsTimerActivebyHandle (Variables|Default|GetShooting%20Timer)))
    (bind _returnvalue (Utilities|Time|SetTimerbyFunctionName 0 "Shoot At Target Loop" 0.2 true true))
    (Variables|Default|SetShooting%20Timer _returnvalue)))

(fn LowerCooldown
  (Variables|Default|SetOffCooldown? true))

(fn ShootatTargetLoop
  (bind _head (Variables|Default|GetHead))
  (bind _returnvalue (Transformation|GetSocketLocation _head "barrel"))
  ;[0.15 0.15 0.15 0.5] If chooses to shoot and able to shoot, fire a line trace - if the line trace hits an enemy shoot a projectile - if there is no target, return to resting position
  (if (Variables|Default|GetWants%20to%20Fire?)
    (if (Variables|Default|GetCan%20fire?)
      (bind _outactors (Actor|GetAllActorswithInterface "/Game/Blueprints/BPI_Interactable.BPI_Interactable_C"))
      (LocalVariables|SetL_ActorsToIgnore _outactors)
      (LocalVariables|SetL_StartTrace _returnvalue)
      (LocalVariables|SetL_EndTrace (+ _returnvalue (* (Math|Vector|GetForwardVector (Variables|Default|GetSocket%20Rotation)) 4e+03)))
      (if (not (Variables|Default|GetManually%20Operated?))
        (bind _target (CallFunction|DetermineTarget))
        (Utilities|IsValid _target
          (:Is%20Valid
            (bind (_outhit _returnvalue_2) (Collision|LineTraceByChannel (LocalVariables|GetL_StartTrace) (LocalVariables|GetL_EndTrace) "TraceTypeQuery3" false (LocalVariables|GetL_ActorsToIgnore) "None"))
            (if _returnvalue_2
              (if (Utilities|DoesObjectImplementInterface (.HitActor (Collision|BreakHitResult _outhit)) "/Game/Blueprints/Enemy/BPI_Enemy.BPI_Enemy_C")
                (if (Variables|Default|GetOffCooldown?)
                  (Variables|Default|SetOffCooldown? false)
                  (CallFunction|FiringEffects)))))
          (:Is%20Not%20Valid
            (switch Utilities|FlowControl|Switch|SwitchonE_OperationalState (Variables|Default|GetOperational%20State)
              (:NewEnumerator0
                _)
              (:NewEnumerator2
                _))
            (CallFunction|ReturntoRest)))
        (else
          (Collision|LineTraceByChannel (LocalVariables|GetL_StartTrace) (LocalVariables|GetL_EndTrace) "TraceTypeQuery3" false (LocalVariables|GetL_ActorsToIgnore) "None")
          (if (Variables|Default|GetOffCooldown?)
            (Variables|Default|SetOffCooldown? false)
            (CallFunction|FiringEffects))))
      (else
        (Utilities|Time|ClearandInvalidateTimerbyHandle (Variables|Default|GetShooting%20Timer) :!label _label)))
    (else
      (goto _label))))

(fn FiringChargedProjectile
  (bind _chosen_projectile (CallFunction|FirstAvailableProjectile))
  (LocalVariables|SetL_ChosenProjectile _chosen_projectile)
  (Transformation|SetActorLocationAndRotation (LocalVariables|GetL_ChosenProjectile) (Math|Vector|SelectVector (Transformation|GetWorldLocation (Variables|Default|GetCamera)) (Transformation|GetSocketLocation (Variables|Default|GetHead) "barrel") (Variables|Default|GetManually%20Operated?)) (Variables|Default|GetSocket%20Rotation))
  (Variables|/Game/Blueprints/Machines/Turret/BP_ProjectileBase.BP_ProjectileBase_C|SetCharged? (LocalVariables|GetL_ChosenProjectile) true)
  (Variables|/Game/Blueprints/Machines/Turret/BP_ProjectileBase.BP_ProjectileBase_C|SetSpeed (LocalVariables|GetL_ChosenProjectile) (* (Variables|/Game/Blueprints/Machines/Turret/BP_ProjectileBase.BP_ProjectileBase_C|GetSpeed (LocalVariables|GetL_ChosenProjectile)) 5.0))
  (Default|SetIsActive (LocalVariables|GetL_ChosenProjectile) true))

(fn GetIndicatorMesh
  (return "/Game/Assets/Levels/MainLevel/Bubble_Turret_Body.Bubble_Turret_Body"))

(fn GetMachineMesh
  (return 0))