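; Flamethrower turret, a child of a base turret, that burns enemies automatically or under manual player control.
; The overridden shooting loop sphere-traces from the barrel, damages BPI_Enemy hits and toggles a Niagara flame.
; Left mouse fires, with a looping timer meant as a click cooldown.
; Space runs a charge skill check, where success grants a temporary larger, stronger super flame before recharging and failure just incurs a cooldown.
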(event EventBeginPlay
  (|CallParentFunction))

(event EventResetCanManuallyFire
  ;[0.15 0.15 0.15 0.5] Attack when possessing and player presses shoot button - the timer functions as a cooldown for when the player clicks, so the turret can't shoot faster than the fire rate
  (Variables|Default|SetCan%20Manually%20Fire? true))

(event Input|MouseEvents|LeftMouseButton
  (params (Key :type Key%20Structure))
  ;[0.15 0.15 0.15 0.5] Attack when possessing and player presses shoot button - the timer functions as a cooldown for when the player clicks, so the turret can't shoot faster than the fire rate
  (:Pressed
    (Variables|Default|SetWants%20to%20Fire? true)
    (Variables|Default|SetCan%20Manually%20Fire? false)
    (CallFunction|Attack)
    (bind _returnvalue (Utilities|Time|SetTimerbyEvent (delegate EventResetCanManuallyFire) (* (.firerate (Variables|Default|GetTurret%20Info)) 0.75) true))
    (Variables|Default|SetFireCooldownTimer _returnvalue))
  (:Released
    (Variables|Default|SetWants%20to%20Fire? false)
    (Utilities|Time|ClearandInvalidateTimerbyHandle (Variables|Default|GetFireCooldownTimer))
    (CallFunction|ActivateFlame false)))

(event Input|KeyboardEvents|SpaceBar
  (params (Key :type Key%20Structure))
  ;[0.15 0.15 0.15 0.5] Charge Shot Input
  (:Pressed
    (if (Variables|Default|GetCanCharge?)
      (if (not (Variables|Default|GetCharging?))
        (Variables|Default|SetCan%20fire? false)
        (Variables|Default|SetCharging? true)
        (Variables|Default|SetCanCharge? false)
        (Default|BeginCharge (Variables|Default|GetSkillCheckWidget)))))
  (:Released
    (if (Variables|Default|GetCharging?)
      (Variables|Default|SetCharging? false)
      (Variables|Default|SetCan%20fire? true)
      (bind _success_ (Default|PlayerReleasesCharge (Variables|Default|GetSkillCheckWidget)))
      (if _success_
        (CallFunction|SuperFlame true)
        (Utilities|FlowControl|Delay 5.0)
        (CallFunction|SuperFlame false)
        (Utilities|FlowControl|Delay 2.0)
        (Variables|Default|SetCanCharge? true)
        (else
          (Utilities|FlowControl|Delay 4.0)
          (Variables|Default|SetCanCharge? true))))))

(fn ConstructionScript
  (|CallParentFunction))

(fn FiringEffects)

(fn ShootatTargetLoop
  (bind _head (Variables|Default|GetHead))
  (bind _returnvalue (Transformation|GetSocketLocation _head "barrel"))
  ;[0.15 0.15 0.15 0.5] If chooses to shoot and able to shoot, fire a line trace - if the line trace hits an enemy shoot a projectile - if there is no target, return to resting position
  (if (Variables|Default|GetWants%20to%20Fire?)
    (if (Variables|Default|GetCan%20fire?)
      (bind _outactors (Actor|GetAllActorswithInterface "/Game/Blueprints/BPI_Interactable.BPI_Interactable_C"))
      (LocalVariables|SetL_ActorsToIgnore _outactors)
      (LocalVariables|SetL_StartTrace _returnvalue)
      (LocalVariables|SetL_EndTrace (+ _returnvalue (* (Math|Vector|GetForwardVector (Variables|Default|GetHead)) 1e+03)))
      (if (not (Variables|Default|GetManually%20Operated?))
        (bind _target (CallFunction|DetermineTarget))
        (Utilities|IsValid _target
          (:Is%20Valid
            (bind _outhits (Collision|MultiSphereTraceByChannel (LocalVariables|GetL_StartTrace) (LocalVariables|GetL_EndTrace) 2e+01 "TraceTypeQuery3" false (LocalVariables|GetL_ActorsToIgnore) "ForDuration"))
            (for _array_element _outhits
              (if (Utilities|DoesObjectImplementInterface (.HitActor (Collision|BreakHitResult _array_element)) "/Game/Blueprints/Enemy/BPI_Enemy.BPI_Enemy_C")
                (CallFunction|ActivateFlame (Utilities|DoesObjectImplementInterface (.HitActor (Collision|BreakHitResult _array_element)) "/Game/Blueprints/Enemy/BPI_Enemy.BPI_Enemy_C"))
                (Game|Damage|ApplyDamage (.HitActor (Collision|BreakHitResult _array_element)) (.basedamage (Variables|Default|GetTurret%20Info)) 0 self))))
          (:Is%20Not%20Valid
            (switch Utilities|FlowControl|Switch|SwitchonE_OperationalState (Variables|Default|GetOperational%20State)
              (:NewEnumerator0
                _)
              (:NewEnumerator2
                _))
            (CallFunction|ReturntoRest)))
        (else
          (bind _outhits_2 (Collision|MultiSphereTraceByChannel (LocalVariables|GetL_StartTrace) (LocalVariables|GetL_EndTrace) 2e+01 "TraceTypeQuery3" false (LocalVariables|GetL_ActorsToIgnore) "None"))
          (CallFunction|ActivateFlame true)
          (for _array_element_2 _outhits_2
            (if (Utilities|DoesObjectImplementInterface (.HitActor (Collision|BreakHitResult _array_element_2)) "/Game/Blueprints/Enemy/BPI_Enemy.BPI_Enemy_C")
              (Game|Damage|ApplyDamage (.HitActor (Collision|BreakHitResult _array_element_2)) (.basedamage (Variables|Default|GetTurret%20Info)) 0 self)))))
      (else
        (Utilities|Time|ClearandInvalidateTimerbyHandle (Variables|Default|GetShooting%20Timer) :!label _label)))
    (else
      (goto _label))))

(fn ActivateFlame
  (params (Activate? :type Boolean))
  (if Activate?
    (if (not (Components|Activation|IsActive (Variables|Default|GetNS_Flame)))
      (Components|Activation|Activate (Variables|Default|GetNS_Flame) false))
    (elif (Components|Activation|IsActive (Variables|Default|GetNS_Flame))
      (Components|Activation|Deactivate (Variables|Default|GetNS_Flame)))))

(fn ReturntoRest
  (|CallParentFunction)
  (CallFunction|ActivateFlame false))

(fn SuperFlame
  (params (Activate? :type Boolean))
  (if Activate?
    (Variables|Default|SetWants%20to%20Fire? true)
    (Variables|Default|SetCan%20fire? true)
    (Variables|Default|SetTurret%20Info (Utilities|Struct|MakeStruct_TurretValues 0.0 0.0 (* (.basedamage (Variables|Default|GetTurret%20Info)) 1.5) 0.0 0))
    (CallFunction|Attack)
    (Transformation|SetWorldScale3D (Variables|Default|GetNS_Flame) "35.000000,35.000000,35.000000")
    (Components|Activation|Activate (Variables|Default|GetNS_Flame) false)
    (else
      (Variables|Default|SetTurret%20Info (Utilities|Struct|MakeStruct_TurretValues 0.0 0.0 (/ (.basedamage (Variables|Default|GetTurret%20Info)) 1.5) 0.0 0))
      (Utilities|Time|ClearandInvalidateTimerbyHandle (Variables|Default|GetShooting%20Timer))
      (Transformation|SetWorldScale3D (Variables|Default|GetNS_Flame) "10.000000,10.000000,10.000000")
      (Components|Activation|Deactivate (Variables|Default|GetNS_Flame)))))