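; Compressor crafting machine that extends a parent machine class with pickup and placement behavior.
; The visible machine lives in the CompressorObject child actor, which is messaged to hide on pickup and show on placement, along with the current operational state.
; It supplies Compressor_Static as its indicator mesh, while GetMachineMesh returns nothing.
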(event EventBeginPlay
  (|CallParentFunction) ; This node is disabled and will not be called.\nDrag off pins to build functionality.
)

(event Collision|EventActorBeginOverlap
  (params (OtherActor :type Actor%20Object%20Reference)))

(event EventTick
  (params (DeltaSeconds :type Float%20%28single-precision%29)))

(event EventPickupMachine
  (params (Player :type BP%20FP%20Character%20Object%20Reference))
  (|CallParentFunction Player)
  (Class|BPIMachineVisual|SetMachineVisbility(Message) (Variables|/Script/Engine.ChildActorComponent|GetChildActor (Variables|Default|GetCompressor_Object)) false (Variables|Default|GetOperational%20State)))

(event EventPlaceMachine
  (params (Player :type BP%20FP%20Character%20Object%20Reference))
  (|CallParentFunction Player)
  (Class|BPIMachineVisual|SetMachineVisbility(Message) (Variables|/Script/Engine.ChildActorComponent|GetChildActor (Variables|Default|GetCompressor_Object)) true (Variables|Default|GetOperational%20State)))

(fn ConstructionScript
  (|CallParentFunction))

(fn GetIndicatorMesh
  (return "/Game/Assets/Machines/Compressor/Compressor_Static.Compressor_Static"))

(fn GetMachineMesh
  (return 0))