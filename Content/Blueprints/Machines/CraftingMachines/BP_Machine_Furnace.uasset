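; Furnace crafting machine, a child Blueprint that leaves most machine behavior to its parent class.
; Its input interaction box shows and hides the interact prompt on overlap.
; Pickup, placement, destroyed and not-destroyed overrides call the parent, then message the ForgeObject child actor with visibility and operational state, hiding it only on pickup.
; Heating_Machine serves as the indicator mesh, while the machine mesh getter returns nothing.
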(event OnComponentBeginOverlap(InputInteractionBox)
  (params (OverlappedComponent :type Primitive%20Component%20Object%20Reference) (OtherActor :type Actor%20Object%20Reference) (OtherComp :type Primitive%20Component%20Object%20Reference) (OtherBodyIndex :type Integer) (bFromSweep :type Boolean) (SweepResult :type Hit%20Result%20Structure%20%28by%20ref%29))
  (CallFunction|DisplayInteract OtherActor))

(event OnComponentEndOverlap(InputInteractionBox)
  (params (OverlappedComponent :type Primitive%20Component%20Object%20Reference) (OtherActor :type Actor%20Object%20Reference) (OtherComp :type Primitive%20Component%20Object%20Reference) (OtherBodyIndex :type Integer))
  (CallFunction|HideInteract OtherActor))

(event EventBeginPlay
  (|CallParentFunction))

(event EventPickupMachine
  (params (Player :type BP%20FP%20Character%20Object%20Reference))
  (|CallParentFunction Player)
  (Class|BPIMachineVisual|SetMachineVisbility(Message) (Variables|/Script/Engine.ChildActorComponent|GetChildActor (Variables|Default|GetForge_Object)) false (Variables|Default|GetOperational%20State)))

(event EventPlaceMachine
  (params (Player :type BP%20FP%20Character%20Object%20Reference))
  (|CallParentFunction Player)
  (Class|BPIMachineVisual|SetMachineVisbility(Message) (Variables|/Script/Engine.ChildActorComponent|GetChildActor (Variables|Default|GetForge_Object)) true (Variables|Default|GetOperational%20State)))

(fn ConstructionScript
  (|CallParentFunction))

(fn GetMachineMesh
  (return 0))

(fn GetIndicatorMesh
  (return "/Game/Assets/Machines/HeatingMachine/Forge_Components/Heating_Machine.Heating_Machine"))

(fn SetMachineDestroyed
  (|CallParentFunction)
  (Class|BPIMachineVisual|SetMachineVisbility(Message) (Variables|/Script/Engine.ChildActorComponent|GetChildActor (Variables|Default|GetForge_Object)) true (Variables|Default|GetOperational%20State)))

(fn OnMachineNotDestroyed
  (|CallParentFunction)
  (Class|BPIMachineVisual|SetMachineVisbility(Message) (Variables|/Script/Engine.ChildActorComponent|GetChildActor (Variables|Default|GetForge_Object)) true (Variables|Default|GetOperational%20State)))