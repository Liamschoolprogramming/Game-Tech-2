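; BP_Machine_Refinery is the refinery Blueprint among the crafting machines, deferring its BeginPlay and construction script to its parent class.
; It adds no processing logic in its graphs, only getters that return its name, a Machine gameplay tag and its mesh.
; GetLocation reports the world position of an Arrow component rather than the actor origin.
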(event EventBeginPlay
  (|CallParentFunction))

(fn ConstructionScript
  (|CallParentFunction))

(fn GetName
  (return (Variables|Default|GetName)))

(fn GameplayTag
  (return "(TagName=\"Machine\")"))

(fn GetLocation
  (return (Transformation|GetWorldLocation (Variables|Default|GetArrow))))

(fn GetMachineMesh
  (return (Variables|Character|GetMesh)))