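; Placeable crafting machine that turns resources in its inventory into the selected recipe's item on a looping timer.
; Recipes load from DT_Recipes; crafting halts when ingredients run short and restarts on resource drop-off or when operational again.
; A world timer widget shows progress, and interacting toggles a recipe, upgrade and inventory menu.
; The extra-resource upgrade adds random bonus output; the speed upgrade only scales the mesh, and converter damage is empty.
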(event Custom|OnCraftingTimer
  (bind _menu_widget (Variables|Default|GetMenu%20Widget))
  (CallFunction|Craft)
  (Utilities|IsValid _menu_widget
    (:Is%20Valid
      (if (UserInterface|Viewport|IsinViewport _menu_widget)
        (Default|RefreshInventory (Variables|Default|GetMenu%20Widget))))))

(event EventBeginPlay
  (bind _returnvalue (UserInterface|CreateWidget "/Game/UI/WidgetBlueprints/WB_CraftingTimer.WB_CraftingTimer_C" 0 self))
  (bind _output_get (Variables|Default|SetProgressRef _returnvalue))
  (UserInterface|SetWidget (Variables|Default|GetTimerWidget) _output_get)
  (|CallParentFunction)
  (Utilities|Time|SetTimerbyEvent (EventDispatchers|CreateEvent :!event UpdateWidgets) 0.01 true)
  (CallFunction|AddingRecipes)
  (CallFunction|SwitchRecipe (Utilities|Array|Get(acopy) (Variables|Default|GetRecipeInventory))))

(event EventOnNotify
  (params (EventType :type E_LevelEventType%20Enum :default "NewEnumerator0"))
  (bind _menu_widget (Variables|Default|GetMenu%20Widget))
  (bind _menu_widget_2 (Variables|Default|GetMenu%20Widget))
  (switch Utilities|FlowControl|Switch|SwitchonE_LevelEventType EventType
    (:NewEnumerator7
      (if (UserInterface|Viewport|IsinViewport _menu_widget_2)
        (Widget|RemovefromParent _menu_widget_2)))
    (:NewEnumerator13
      (if (UserInterface|Viewport|IsinViewport _menu_widget)
        (Widget|RemovefromParent _menu_widget)))))

(event EventUpdateWidgets
  (|CallParentFunction)
  (CallFunction|SetWidgetRotation (Variables|Default|GetTimerWidget))
  (Default|UpdateCraftingTimer (Variables|Default|GetProgressRef) (Class|KismetSystemLibrary|GetTimerElapsedTimeHandle (Variables|Default|GetCraftingTimer)) (not (Variables|Default|GetCraftingHalted))))

(event EventDropOffResource
  (params (ResourceName :type Name :default "None") (ResourceAmount :type Integer))
  (|CallParentFunction ResourceName ResourceAmount)
  (if (Variables|Default|GetCraftingHalted)
    (CallFunction|SwitchRecipe (Variables|Default|GetActiveRecipe))))

(event EventUpgrade
  (params (Upgrades :type E_Upgrades%20Enum :default "NewEnumerator0"))
  (bind _asbp_fpcharacter (Utilities|Casting|CastToBP_FPCharacter (Game|GetPlayerCharacter 0)))
  (switch Utilities|FlowControl|Switch|SwitchonE_Upgrades Upgrades
    (:NewEnumerator0
      (CallFunction|UpgradeCraftingSpeed)
      (Default|DisplayAlert _asbp_fpcharacter "Upgraded crafting speed!"))
    (:NewEnumerator2
      (CallFunction|UpgradeExtraResource)
      (Default|DisplayAlert _asbp_fpcharacter "Extra resource from crafting!"))
    (:NewEnumerator3
      (CallFunction|UpgradeConverterDamage)
      (Default|DisplayAlert _asbp_fpcharacter "Upgraded converter damage!!"))))

(event EventPlaceMachine
  (params (Player :type BP%20FP%20Character%20Object%20Reference))
  (|CallParentFunction Player)
  (Rendering|SetVisibility (Variables|Default|GetTimerWidget) true false))

(event EventPickupMachine
  (params (Player :type BP%20FP%20Character%20Object%20Reference))
  (|CallParentFunction Player)
  (Rendering|SetVisibility (Variables|Default|GetTimerWidget) false false))

(fn ConstructionScript
  (|CallParentFunction))

(fn SwitchRecipe
  (params (Recipe :type S%20Recipes%20Structure))
  (bind _menu_widget (Variables|Default|GetMenu%20Widget))
  (Variables|Default|SetCraftingHalted true)
  (Variables|Default|SetActiveRecipe Recipe)
  (CallFunction|StopCraftingTimer)
  (bind _returnvalue (Utilities|Time|SetTimerbyEvent (EventDispatchers|CreateEvent :!event Custom|OnCraftingTimer) (.productionrate (Variables|Default|GetMachine%20Info%20Defaults)) true))
  (Variables|Default|SetCraftingTimer _returnvalue)
  (bind _namenowhitespace (CallFunction|StripWhitespaceName (.Name (Utilities|Struct|BreakS_Recipes (Variables|Default|GetActiveRecipe)))))
  (bind _returnvalue_2 (Utilities|GetDataTableRow "/Game/Blueprints/DT_Resources.DT_Resources" _namenowhitespace)
    (:then
      (Default|SetResource (Variables|Default|GetProgressRef) _returnvalue_2 (.productionrate (Variables|Default|GetMachine%20Info%20Defaults)))
      (Utilities|IsValid _menu_widget
        (:Is%20Valid
          (Default|SetRecipeResourceData _menu_widget))))))

(fn StopCraftingTimer
  (Utilities|Time|ClearandInvalidateTimerbyHandle (Variables|Default|GetCraftingTimer)))

(fn AttachtoComponet
  (|CallParentFunction)
  (CallFunction|StopCraftingTimer))

(fn Craft
  (bind _activerecipe (Variables|Default|GetActiveRecipe))
  (bind _bp_inventory (Variables|Default|GetBP_Inventory))
  (bind (_name _amounttocraft _requiredmachine _requiredresources) (Utilities|Struct|BreakS_Recipes _activerecipe))
  (bind _hasenoughresources (CallFunction|HasEnoughResourcesforRecipe))
  (if _hasenoughresources
    (Variables|Default|SetCraftingHalted false)
    (LocalVariables|SetL_ResourceNameToCraft _name)
    (bind (_keypin _valuepin) (Utilities|Map|ForEachLoop(Map) _requiredresources)
      (:then
        (Default|RemoveResourcefromInventory _bp_inventory _keypin _valuepin))
      (:CompletedPin
        (Default|AddResourcetoInventory _bp_inventory (LocalVariables|GetL_ResourceNameToCraft) _amounttocraft)
        (if (Variables|Default|GetDuplicateUpgrade)
          (bind _output_get (Variables|Default|SetDuplicateCraftedItem (Math|Random|RandomInteger 10)))
          (if (Math|Integer|InRange(Integer) _output_get 7 10)
            (Default|AddResourcetoInventory (Variables|Default|GetBP_Inventory) (LocalVariables|GetL_ResourceNameToCraft) 1)))))
    (else
      (Utilities|Time|ClearandInvalidateTimerbyHandle (Variables|Default|GetCraftingTimer))
      (Variables|Default|SetCraftingHalted true))))

(fn HasEnoughResourcesforRecipe
  (bind (_keypin _valuepin) (Utilities|Map|ForEachLoop(Map) (.RequiredResources (Utilities|Struct|BreakS_Recipes (Variables|Default|GetActiveRecipe))))
    (:then
      (bind _resource_amount (Default|GetResourceAmount (Variables|Default|GetBP_Inventory) _keypin))
      (if (< _resource_amount _valuepin)
        (return false)))
    (:CompletedPin
      (return true))))

(fn AddingRecipes
  (Utilities|Array|Clear (Variables|Default|GetRecipeInventory))
  (for _array_element (Variables|Default|GetRecipeNames)
    (bind _namenowhitespace (CallFunction|StripWhitespaceName _array_element))
    (bind _returnvalue (Utilities|GetDataTableRow "/Game/Blueprints/DT_Recipes.DT_Recipes" _namenowhitespace)
      (:then
        (Utilities|Array|Add (Variables|Default|GetRecipeInventory) _returnvalue)
        (bind _keypin (Utilities|Map|ForEachLoop(Map) (.RequiredResources (Utilities|Struct|BreakS_Recipes _returnvalue)))
          (:then
            (Default|AddResourcetoInventory (Variables|Default|GetBP_Inventory) _keypin)))))))

(fn UpdateCraftTimer
  (Variables|/Game/UI/WidgetBlueprints/WB_CraftingTimer.WB_CraftingTimer_C|SetMaxTime (Variables|Default|GetProgressRef) (.productionrate (Variables|Default|GetMachine%20Info)))
  (Variables|/Game/UI/WidgetBlueprints/WB_CraftingTimer.WB_CraftingTimer_C|SetCurrentTime (Variables|Default|GetProgressRef) (Variables|Default|GetCraftingTimePassed))
  (return))

(fn ActionInteract
  (params (Player :type BP%20FP%20Character%20Object%20Reference))
  (|CallParentFunction Player)
  (switch Utilities|FlowControl|Switch|SwitchonE_OperationalState (Variables|Default|GetOperational%20State)
    (:NewEnumerator2
      (Utilities|IsValid (Variables|Default|GetMenu%20Widget)
        (:Is%20Valid
          _)
        (:Is%20Not%20Valid
          (bind _returnvalue (UserInterface|CreateWidget "/Game/UI/WidgetBlueprints/MachineInventory/W_CraftingMachineOptions.W_CraftingMachineOptions_C" 0 self (Variables|Default|GetBP_Inventory)))
          (bind _output_get (Variables|Default|SetMenu%20Widget _returnvalue))
          (Default|InitializeRecipeSlots _output_get)
          (Default|InitializeUpgradeSlots (Variables|Default|GetMenu%20Widget))
          (Default|InitializeGridSlots (Variables|/Game/UI/WidgetBlueprints/MachineInventory/W_CraftingMachineOptions.W_CraftingMachineOptions_C|GetInventoryGrid (Variables|Default|GetMenu%20Widget)) 3 6)
          (Variables|/Game/UI/WidgetBlueprints/CraftingSystemMenus/W_InventoryGrid.W_InventoryGrid_C|SetInteractable (Variables|/Game/UI/WidgetBlueprints/MachineInventory/W_CraftingMachineOptions.W_CraftingMachineOptions_C|GetInventoryGrid (Variables|Default|GetMenu%20Widget)) self)
          (Default|PopulateGrid (Variables|/Game/UI/WidgetBlueprints/MachineInventory/W_CraftingMachineOptions.W_CraftingMachineOptions_C|GetInventoryGrid (Variables|Default|GetMenu%20Widget)) (Variables|Default|GetBP_Inventory) (Variables|/Game/UI/WidgetBlueprints/CraftingSystemMenus/W_Inventory.W_Inventory_C|GetW_Hotbar (Variables|/Game/Blueprints/Player/BP_FPCharacter.BP_FPCharacter_C|GetInventoryUI Player)))))
      (if (UserInterface|Viewport|IsinViewport (Variables|Default|GetMenu%20Widget))
        (Widget|RemovefromParent (Variables|Default|GetMenu%20Widget))
        (Variables|/Game/Blueprints/Player/BP_FPCharacter.BP_FPCharacter_C|SetMovementEnabled Player true)
        (Variables|/Game/Blueprints/Player/BP_FPCharacter.BP_FPCharacter_C|SetMenuOpen Player false)
        (Input|SetInputModeGameOnly (Game|GetPlayerController 0) true)
        (Variables|/Script/Engine.PlayerController|SetbShowMouseCursor (Game|GetPlayerController 0) false)
        (else
          (UserInterface|Viewport|AddtoViewport (Variables|Default|GetMenu%20Widget) 0)
          (Default|InstantiateMachineValues (Variables|Default|GetMenu%20Widget) (Variables|Default|GetBP_Inventory))
          (Variables|/Game/Blueprints/Player/BP_FPCharacter.BP_FPCharacter_C|SetMovementEnabled Player false)
          (Variables|/Game/Blueprints/Player/BP_FPCharacter.BP_FPCharacter_C|SetMenuOpen Player true)
          (Input|SetInputModeGameandUI (Game|GetPlayerController 0) 0 "DoNotLock" true false)
          (Variables|/Script/Engine.PlayerController|SetbShowMouseCursor (Game|GetPlayerController 0) true))))))

(fn UpgradeCraftingSpeed
  (bind _mesh (Variables|Character|GetMesh))
  (bind _returnvalue (Transformation|GetWorldTransform _mesh))
  (Transformation|SetWorldTransform _mesh (Math|Transform|MakeTransform (.location _returnvalue) (.rotation _returnvalue) "1.200000,1.200000,1.200000") false false)
  (Development|PrintString "Upgraded crafting speed"))

(fn UpgradeExtraResource
  (Variables|Default|SetDuplicateUpgrade true))

(fn UpgradeConverterDamage)

(fn UpgradeConverterDoubleCraftingSpeed
  (|CallParentFunction))

(fn UpdateStatus
  (|CallParentFunction)
  (switch Utilities|FlowControl|Switch|SwitchonE_OperationalState (Variables|Default|GetOperational%20State)
    (:NewEnumerator1
      (if (Utilities|Time|IsTimerActivebyHandle (Variables|Default|GetCraftingTimer))
        (Utilities|Time|ClearandInvalidateTimerbyHandle (Variables|Default|GetCraftingTimer))))
    (:NewEnumerator2
      (if (Utilities|Time|IsValidTimerHandle (Variables|Default|GetCraftingTimer))
        (if (not (Utilities|Time|IsTimerActivebyHandle (Variables|Default|GetCraftingTimer)))
          (CallFunction|SwitchRecipe (Variables|Default|GetActiveRecipe)))
        (else
          (CallFunction|SwitchRecipe (Variables|Default|GetActiveRecipe)))))))

(fn GetName
  (return (Variables|Default|GetName)))

(fn GetMachineMesh
  (return (Variables|Character|GetMesh)))

(fn Interact
  (params (Player :type BP%20FP%20Character%20Object%20Reference))
  (CallFunction|ActionInteract Player)
  (return (Variables|Default|GetMenu%20Widget)))