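; Placeable robot station that charges robots, opens a programming menu for the player and can be repaired by holding R.
; On BeginPlay it spawns a BP_RobotManager and feeds it to the W_RobotProgrammer widget that Interact toggles.
; Placement registers it with the nearest in-range BP_EngineCore, setting the power state shown on camera-facing text.
; Box overlaps set robot charge rate from that state or show player prompts, while a looping timer restores health.
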(event OnComponentBeginOverlap(Box)
  (params (OverlappedComponent :type Primitive%20Component%20Object%20Reference) (OtherActor :type Actor%20Object%20Reference) (OtherComp :type Primitive%20Component%20Object%20Reference) (OtherBodyIndex :type Integer) (bFromSweep :type Boolean) (SweepResult :type Hit%20Result%20Structure%20%28by%20ref%29))
  ;[0.15 0.15 0.15 0.5] Interactions with other actors
  (switch Utilities|FlowControl|Switch|SwitchonE_MachineState (Variables|Default|GetMachineStates)
    (:NewEnumerator0
      (if (Utilities|DoesObjectImplementInterface OtherActor "/Game/Blueprints/Robot/BPI_Robot.BPI_Robot_C") :!label _label
        (switch Utilities|FlowControl|Switch|SwitchonE_OperationalState (Variables|Default|GetOperational%20State)
          (:NewEnumerator0
            (Class|BPIRobot|SetChargePerSecond(Message) OtherActor 0.0))
          (:NewEnumerator2
            (Class|BPIRobot|SetChargePerSecond(Message) OtherActor (.productionrate (Variables|Default|GetMachine%20Info%20Defaults)))))
        (elif (< (Variables|Default|GetCurrent%20Health) (.maxhealth (Variables|Default|GetMachine%20Info)))
          (bind _asbp_fpcharacter (Utilities|Casting|CastToBP_FPCharacter OtherActor))
          (Default|DisplayInputPrompt _asbp_fpcharacter "Press E to Interact & R to Repair")
          (else
            (bind _asbp_fpcharacter_2 (Utilities|Casting|CastToBP_FPCharacter OtherActor))
            (Default|DisplayInputPrompt _asbp_fpcharacter_2 "Press E to open robot menu")))))
    (:NewEnumerator3
      (goto _label))
    (:NewEnumerator2
      (bind _asbp_fpcharacter_3 (Utilities|Casting|CastToBP_FPCharacter (Game|GetPlayerCharacter 0)))
      (Default|HideInputPrompt _asbp_fpcharacter_3))))

(event OnComponentEndOverlap(Box)
  (params (OverlappedComponent :type Primitive%20Component%20Object%20Reference) (OtherActor :type Actor%20Object%20Reference) (OtherComp :type Primitive%20Component%20Object%20Reference) (OtherBodyIndex :type Integer))
  ;[0.15 0.15 0.15 0.5] Interactions with other actors
  (if (Utilities|DoesObjectImplementInterface OtherActor "/Game/Blueprints/Robot/BPI_Robot.BPI_Robot_C")
    (Class|BPIRobot|SetChargePerSecond(Message) OtherActor 0.0)
    (else
      (bind _asbp_fpcharacter (Utilities|Casting|CastToBP_FPCharacter OtherActor))
      (Default|HideInputPrompt _asbp_fpcharacter))))

(event Custom|BuildMachine
  (params (Player :type BP%20FP%20Character%20Object%20Reference))
  ;[0.15 0.15 0.15 0.5] BPI Logic
  (Variables|/Game/Blueprints/Player/BP_FPCharacter.BP_FPCharacter_C|SetBuildMachine Player self)
  (Transformation|AttachComponentToComponent (Variables|/Game/Blueprints/Player/BP_FPCharacter.BP_FPCharacter_C|GetObjectPickup Player) "None" "SnapToTarget" "KeepRelative" "KeepRelative" true)
  (Variables|Default|SetMachineStates "NewEnumerator2"))

(event Custom|UpdateWidget
  (bind _poweredbytext (Variables|Default|GetPoweredByText))
  (Transformation|SetWorldRotation _poweredbytext (Math|Rotator|FindLookatRotation (Transformation|GetWorldLocation _poweredbytext) (Transformation|GetWorldLocation (Variables|/Script/Engine.PlayerCameraManager|GetTransformComponent (Game|GetPlayerCameraManager 0)))) false false))

(event Custom|RepairLoop
  (bind _machine_info (Variables|Default|GetMachine%20Info))
  ;[0.15 0.15 0.15 0.5] Start repair timer when holding R and stop when R is released - Set player state to repairing if health isn't full, otherise cancel this event - Also stop if repairing finishes
  (if (< (Variables|Default|GetCurrent%20Health) (.maxhealth _machine_info))
    (bind _output_get (Variables|Default|SetCurrent%20Health (Math|Float|Clamp(Float) (+ (Variables|Default|GetCurrent%20Health) 1.0) 0.0 (.maxhealth _machine_info))))
    (Default|DisplayRepairing (stale EventRepair Player) _output_get (.maxhealth _machine_info) true)
    (if (Utilities|Enum|Equal(Enum) (Variables|Default|GetOperational%20State) "NewEnumerator1")
      (CallFunction|EventChange))
    (else
      (Utilities|Time|ClearandInvalidateTimerbyHandle (Variables|Default|GetRepair%20Timer))
      (Default|DisplayRepairing (stale EventRepair Player) (Variables|Default|GetCurrent%20Health) (.maxhealth _machine_info) false))))

(event Custom|EventChange
  ;[0.15 0.15 0.15 0.5] Event Logic
  (CallFunction|SetCorePoweredby)
  (switch Utilities|FlowControl|Switch|SwitchonE_MachineState (Variables|Default|GetMachineStates)
    (:NewEnumerator0
      (Utilities|FlowControl|DoOnce false
        (:Completed
          (Variables|Default|SetMachineStates "NewEnumerator3")
          (CallFunction|EventChange))))
    (:NewEnumerator3
      (CallFunction|SetPoweredbyText)
      (switch Utilities|FlowControl|Switch|SwitchonE_OperationalState (Variables|Default|GetOperational%20State)
        (:NewEnumerator0
          (CallFunction|SetCorePoweredby))))))

(event Custom|Set%20Powered%20By%20Text
  (bind _poweredbytext (Variables|Default|GetPoweredByText))
  (bind _operational_state (Variables|Default|GetOperational%20State))
  ;[0.15 0.15 0.15 0.5] Set Text Render PoweredByText and Color (temp)
  (Rendering|Components|TextRender|SetText _poweredbytext (|GenerictoText _operational_state))
  (Rendering|Components|TextRender|SetTextRenderColor _poweredbytext (Utilities|Select :Index _operational_state :NewEnumerator0 (Class|KismetMathLibrary|LinearColortoRGBE "(R=0.679543,G=0.005182,B=0.040915,A=1.000000)") :NewEnumerator1 (Class|KismetMathLibrary|LinearColortoRGBE) :NewEnumerator2 (Class|KismetMathLibrary|LinearColortoRGBE "(R=0.000000,G=1.000000,B=0.327778,A=1.000000)"))))

(event EventPickupMachine
  (params (Player :type BP%20FP%20Character%20Object%20Reference))
  ;[0.15 0.15 0.15 0.5] BPI Logic
  (Transformation|AttachComponentToComponent (.ItemSocket (Utilities|Struct|BreakS_Linetrace (Variables|/Game/Blueprints/Player/BP_FPCharacter.BP_FPCharacter_C|GetLineTraceInfo (stale EventSelection Player)))) "None" "SnapToTarget" "KeepRelative" "KeepRelative" true)
  (Variables|Default|SetMachineStates "NewEnumerator2")
  (CallFunction|EventChange))

(event EventBeginPlay
  ;[0.15 0.15 0.15 0.5] Initialization
  (CallFunction|EventChange)
  (bind _returnvalue (Actor|GetActorOfClass "/Game/Blueprints/Player/BP_FPCharacter.BP_FPCharacter_C"))
  (bind _returnvalue_2 (Game|SpawnActorfromClass "/Game/Blueprints/Robot/BP_RobotManager.BP_RobotManager_C" (Transformation|GetActorTransform) "Undefined" "MultiplyWithRoot" 0 _returnvalue self 0))
  (bind _returnvalue_3 (UserInterface|CreateWidget "/Game/UI/WidgetBlueprints/RobotProgrammer/W_RobotProgrammer.W_RobotProgrammer_C" 0 _returnvalue_2))
  (Variables|Default|SetProgrammerScreen _returnvalue_3)
  (Utilities|Time|SetTimerbyEvent (delegate Custom|UpdateWidget) 0.01 true))

(event EventPlaceMachine
  ;[0.15 0.15 0.15 0.5] BPI Logic
  (bind _asbp_fpcharacter (Utilities|Casting|CastToBP_FPCharacter (Game|GetPlayerCharacter 0)))
  (Transformation|DetachFromActor "KeepRelative" "KeepRelative" "KeepRelative")
  (Transformation|SetActorTransform self (Math|Conversions|ToTransform(Vector) (Variables|/Game/Blueprints/Player/BP_FPCharacter.BP_FPCharacter_C|GetTestLocation _asbp_fpcharacter)))
  (Variables|Default|SetMachineStates "NewEnumerator3")
  (CallFunction|EventChange))

(event EventInteract
  (params (Player :type BP%20FP%20Character%20Object%20Reference))
  (bind _returnvalue (Game|GetPlayerCharacter 0))
  (bind _returnvalue_2 (Game|GetPlayerController 0))
  (bind _programmerscreen (Variables|Default|GetProgrammerScreen))
  (if (UserInterface|Viewport|IsinViewport _programmerscreen)
    (Variables|/Game/Blueprints/Player/BP_FPCharacter.BP_FPCharacter_C|SetInventoryToggleEnabled Player true)
    (Widget|RemovefromParent _programmerscreen)
    (Input|SetInputModeGameOnly _returnvalue_2 true)
    (Variables|/Script/Engine.PlayerController|SetbShowMouseCursor _returnvalue_2 false)
    (bind _asbp_fpcharacter (Utilities|Casting|CastToBP_FPCharacter _returnvalue))
    (Default|EnableMovement _asbp_fpcharacter)
    (else
      (Variables|/Game/Blueprints/Player/BP_FPCharacter.BP_FPCharacter_C|SetInventoryToggleEnabled Player false)
      (UserInterface|Viewport|AddtoViewport _programmerscreen 0)
      (Input|SetInputModeGameandUI _returnvalue_2 0 "DoNotLock" true true)
      (Variables|/Script/Engine.PlayerController|SetbShowMouseCursor _returnvalue_2 true)
      (bind _asbp_fpcharacter_2 (Utilities|Casting|CastToBP_FPCharacter _returnvalue))
      (Default|DisableMovement _asbp_fpcharacter_2)
      (Default|HideInputPrompt _asbp_fpcharacter_2))))

(event EventSelection
  (params (Player :type BP%20FP%20Character%20Object%20Reference))
  ;[0.15 0.15 0.15 0.5] BPI Logic
)

(event EventRecieveEnergy
  (params (Sending%20Core :type BP%20Engine%20Core%20Object%20Reference) (Operational? :type Boolean))
  ;[0.15 0.15 0.15 0.5] Recieving Energy From the Core
  (if Operational?
    (switch Utilities|FlowControl|Switch|SwitchonE_OperationalState (Variables|Default|GetOperational%20State)
      (:NewEnumerator0
        _)
      (:NewEnumerator2
        _))
    (Variables|Default|SetOperational%20State "NewEnumerator2")
    (CallFunction|SetPoweredbyText)
    (else
      (switch Utilities|FlowControl|Switch|SwitchonE_OperationalState (Variables|Default|GetOperational%20State)
        (:NewEnumerator0
          _)
        (:NewEnumerator2
          _))
      (Variables|Default|SetOperational%20State "NewEnumerator0")
      (CallFunction|SetPoweredbyText))))

(event EventRepair
  (params (Player :type BP%20FP%20Character%20Object%20Reference) (Repairing? :type Boolean))
  (bind _machine_info (Variables|Default|GetMachine%20Info))
  ;[0.15 0.15 0.15 0.5] Start repair timer when holding R and stop when R is released - Set player state to repairing if health isn't full, otherise cancel this event - Also stop if repairing finishes
  (if Repairing?
    (if (< (Variables|Default|GetCurrent%20Health) (.maxhealth _machine_info))
      (Variables|/Game/Blueprints/Player/BP_FPCharacter.BP_FPCharacter_C|SetPlayerStates Player "NewEnumerator6")
      (Utilities|Time|ClearandInvalidateTimerbyHandle (Variables|Default|GetRepair%20Timer))
      (bind _returnvalue (Utilities|Time|SetTimerbyEvent (delegate Custom|RepairLoop) 0.2 true))
      (Variables|Default|SetRepair%20Timer _returnvalue))
    (else
      (Utilities|Time|ClearandInvalidateTimerbyHandle (Variables|Default|GetRepair%20Timer))
      (Default|DisplayRepairing Player (Variables|Default|GetCurrent%20Health) (.maxhealth _machine_info) false))))

(fn ConstructionScript
  (bind _machine_info_defaults (Variables|Default|GetMachine%20Info%20Defaults))
  (bind _output_get (Variables|Default|SetMachine%20Info (Utilities|Struct|MakeStruct_MachineValues (.maxhealth _machine_info_defaults) (.distancefromcore _machine_info_defaults) (.energycost _machine_info_defaults) (.productionrate _machine_info_defaults))))
  (Variables|Default|SetCurrent%20Health (.maxhealth _output_get)))

(fn SetCorePoweredby
  (bind _self self)
  (bind _machine_info (Variables|Default|GetMachine%20Info))
  (LocalVariables|SetDistance 9999.0)
  (bind _outactors (Actor|GetAllActorsOfClass "/Game/Blueprints/EngineCores/BP_EngineCore.BP_EngineCore_C"))
  (for _array_element _outactors
    (if (and (< (Transformation|GetHorizontalDistanceTo _array_element self) (LocalVariables|GetDistance)) (<= (Transformation|GetHorizontalDistanceTo _array_element self) (.distancefromcore (Variables|Default|GetMachine%20Info))))
      (LocalVariables|SetTemp%20Core _array_element)
      (LocalVariables|SetDistance (Transformation|GetHorizontalDistanceTo _array_element self))))
  (bind _temp_core (LocalVariables|GetTemp%20Core)
    (:then
      (Variables|Default|SetCore%20Powered%20By _temp_core)
      (Variables|Default|SetOperational%20State "NewEnumerator2")
      (Development|PrintString "in range")
      (Default|VerifyDependentMachine (Variables|Default|GetCore%20Powered%20By) _self (.energycost _machine_info) true))
    (:else
      (Development|PrintString "Not in range of core!" true true "(R=1.000000,G=0.000000,B=0.077756,A=1.000000)")
      (Variables|Default|SetOperational%20State "NewEnumerator0")
      (bind _core_powered_by (Variables|Default|GetCore%20Powered%20By)
        (:then
          (Default|VerifyDependentMachine _core_powered_by _self (.energycost _machine_info) false))
        (:else)))))

(fn GameplayTag
  (return "(TagName=\"Robot\")"))

(fn GetMachineHealth
  (return 0.0 0.0))

(fn GetLocation1
  (return "0, 0, 0"))

(fn GetGameplayTags
  (return (Variables|Default|GetGameplayTags_0)))

(fn GetLocation
  (return (Transformation|GetActorLocation)))

(fn GetName
  (return "None"))

(fn HasResource1
  (params (Resource%20Robot%20Is%20Looking%20For :type Name :default "None"))
  (return "None" 0 0))

(fn HasResource
  (params (Resource%20Robot%20Is%20Looking%20For :type Name :default "None"))
  (return "None" 0 0))