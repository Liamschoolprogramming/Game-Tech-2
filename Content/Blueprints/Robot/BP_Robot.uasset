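; Robot pawn that cycles through machine locations via AI MoveTo, returning to a charging station when charge runs low.
; Temporary test code on BeginPlay gathers machine transforms, sets home from the stations found and starts the route.
; Each arrival spends charge and advances the looping index, while failed moves retry the same destination.
; The station supplies a charge rate, driving a self-rescheduling timer that refills charge while homebound and resumes the route when full.
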(event Custom|SetRobotHome
  (params (RobotStation :type BP%20Robot%20Station%20Object%20Reference))
  ;[0.15 0.15 0.15 0.5] Manage setting and navigating to next destination (machine or home charger)
  (Variables|Default|SetHome (Transformation|GetActorTransform RobotStation)))

(event Custom|GoHome
  ;[0.15 0.15 0.15 0.5] Manage setting and navigating to next destination (machine or home charger)
  (Variables|Default|SetGoingHome true)
  (AI|AIMoveTo self (.location (Variables|Default|GetHome)) 0 5.0 true))

(event Custom|GoToNextDestination
  ;[0.15 0.15 0.15 0.5] Manage setting and navigating to next destination (machine or home charger)
  (if (<= (Variables|Default|GetCharge) 1.0)
    (CallFunction|GoHome)
    (else
      (AI|AIMoveTo self (.location (Utilities|Array|Get(acopy) (Variables|Default|GetDestinations) (Variables|Default|GetDestinationIndex))) 0 5.0 true
        (:OnSuccess
          (CallFunction|IncrementDestinationIndex)
          (CallFunction|DecrementCharge 1.0)
          (Utilities|FlowControl|Delay 0.3))
        (:OnFail
          _))
      (CallFunction|GotoNextDestination))))

(event Custom|IncrementDestinationIndex
  ;[0.15 0.15 0.15 0.5] Manage setting and navigating to next destination (machine or home charger)
  (if (>= (+ (Variables|Default|GetDestinationIndex) 1) (Utilities|Array|Length (Variables|Default|GetDestinations)))
    (Variables|Default|SetDestinationIndex 0)
    (else
      (Variables|Default|SetDestinationIndex (+ (Variables|Default|GetDestinationIndex) 1)))))

(event Custom|DecrementCharge
  (params (ChargeAmount :type Float%20%28double-precision%29))
  ;[0.15 0.15 0.15 0.5] Handle charging (initiated and ended by BP_Robot_Station)
  (Variables|Default|SetCharge (- (Variables|Default|GetCharge) ChargeAmount)))

(event Custom|IncrementCharge
  (bind _maxcharge (Variables|Default|GetMaxCharge))
  ;[0.15 0.15 0.15 0.5] Handle charging (initiated and ended by BP_Robot_Station)
  (if (> (Variables|Default|GetChargePerSecond) 0.0)
    (if (>= (+ (Variables|Default|GetChargePerSecond) (Variables|Default|GetCharge)) _maxcharge)
      (Variables|Default|SetCharge _maxcharge)
      (CallFunction|GotoNextDestination)
      (else
        (Variables|Default|SetCharge (+ (Variables|Default|GetChargePerSecond) (Variables|Default|GetCharge)))
        (Utilities|Time|SetTimerbyEvent (delegate Custom|IncrementCharge) 1.0)))))

(event EventSetChargePerSecond
  (params (ChargePerSecond :type Float%20%28double-precision%29))
  ;[0.15 0.15 0.15 0.5] Handle charging (initiated and ended by BP_Robot_Station)
  (if (Variables|Default|GetGoingHome)
    (Variables|Default|SetChargePerSecond ChargePerSecond)
    (CallFunction|IncrementCharge)))

(event EventBeginPlay
  ;[0.15 0.15 0.15 0.5] TESTING ONLY (will be replaced by programmer widget)
  (bind _outactors (Actor|GetAllActorsOfClass "/Game/Blueprints/Machines/MachineBaseClass/BP_Machine_Base.BP_Machine_Base_C"))
  (for _array_element _outactors
    (Utilities|Array|Add (Variables|Default|GetDestinations) (Transformation|GetActorTransform _array_element)))
  (bind _outactors_2 (Actor|GetAllActorsOfClass "/Game/Blueprints/Robot/BP_RobotStation.BP_RobotStation_C"))
  (for _array_element_2 _outactors_2
    (CallFunction|SetRobotHome _array_element_2))
  (CallFunction|GotoNextDestination))

(fn ConstructionScript)