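; BP_Scrap is a scrap interactable that the first-person player can destroy.
; Its Box overlap shows a "Press Q to destroy" prompt through BP_FPCharacter after a player-state switch, and hides it when the overlap ends.
; The construction script assigns BP_ObjectBreak_Scrap as its Destructable, while getter functions report the Interactable gameplay tag and the Scrap indicator mesh.
; The file holds no input or destruction logic.
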(event OnComponentBeginOverlap(Box)
  (params (OverlappedComponent :type Primitive%20Component%20Object%20Reference) (OtherActor :type Actor%20Object%20Reference) (OtherComp :type Primitive%20Component%20Object%20Reference) (OtherBodyIndex :type Integer) (bFromSweep :type Boolean) (SweepResult :type Hit%20Result%20Structure%20%28by%20ref%29))
  (bind _asbp_fpcharacter (Utilities|Casting|CastToBP_FPCharacter OtherActor))
  (switch Utilities|FlowControl|Switch|SwitchonE_PlayerState (Variables|/Game/Blueprints/Player/BP_FPCharacter.BP_FPCharacter_C|GetPlayerStates _asbp_fpcharacter)
    (:NewEnumerator0
      (Default|DisplayInputPrompt _asbp_fpcharacter "Press Q to destroy"))))

(event OnComponentEndOverlap(Box)
  (params (OverlappedComponent :type Primitive%20Component%20Object%20Reference) (OtherActor :type Actor%20Object%20Reference) (OtherComp :type Primitive%20Component%20Object%20Reference) (OtherBodyIndex :type Integer))
  (bind _asbp_fpcharacter (Utilities|Casting|CastToBP_FPCharacter OtherActor))
  (Default|HideInputPrompt _asbp_fpcharacter))

(event EventBeginPlay
  (|CallParentFunction))

(fn ConstructionScript
  (Variables|Default|SetDestructable "/Game/Blueprints/Interactable/BP_ObjectBreak_Scrap.BP_ObjectBreak_Scrap_C"))

(fn GetGameplayTags
  (return "(GameplayTags=((TagName=\"Interactable\")))"))

(fn GetIndicatorMesh
  (return "/Game/Assets/Set_Dressing/Scrap/Scrap.Scrap"))