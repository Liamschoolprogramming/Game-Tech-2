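; Base Blueprint for interactable actors, stubbing pickup, placement and machine-related calls, with GameplayTag returning Interactable.
; The PlaceMachine event moves the actor to the hit location of the player's line trace, converting only that location into a transform.
; PickupInteractable and PlaceInteractable are empty, leaving the print-only Pickup and the duplicate Place function unwired in the event graph.
; Interact, resource and other getters return empty or default values.
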(event EventPlaceInteractable
  (params (Player :type BP%20FP%20Character%20Object%20Reference)))

(event EventPlaceMachine
  (params (Player :type BP%20FP%20Character%20Object%20Reference))
  (Transformation|SetActorTransform (Math|Conversions|ToTransform(Vector) (.hitlocation (Variables|/Game/Blueprints/Player/BP_FPCharacter.BP_FPCharacter_C|GetLineTraceInfo Player)))))

(event EventBeginPlay)

(event EventPickupInteractable
  (params (Player :type BP%20FP%20Character%20Object%20Reference)))

(fn ConstructionScript)

(fn Pickup
  (params (Player :type BP%20FP%20Character%20Object%20Reference))
  (Development|PrintString "Picked up"))

(fn Place
  (params (Player :type BP%20FP%20Character%20Object%20Reference))
  (Transformation|SetActorTransform (Math|Conversions|ToTransform(Vector) (.hitlocation (Variables|/Game/Blueprints/Player/BP_FPCharacter.BP_FPCharacter_C|GetLineTraceInfo Player)))))

(fn GameplayTag
  (return "(TagName=\"Interactable\")"))

(fn GetGameplayTags
  (return ""))

(fn GetIndicatorMesh
  (return 0))

(fn GetLocation
  (return "0, 0, 0"))

(fn GetMachine
  (return 0))

(fn GetMachineClass
  (return 0))

(fn GetMachineMesh
  (return 0))

(fn GetName
  (return "None"))

(fn GetRotation
  (return 0.0))

(fn HasResource
  (params (Resource%20Name :type Name :default "None"))
  (return 0 false))

(fn Interact
  (params (Player :type BP%20FP%20Character%20Object%20Reference))
  (return 0))