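; BP_ResourceDrop is a collectible resource actor that represents a dropped resource in the world.
; Its construction script looks up its resource name in a data table, storing the row as its resource data and applying that row's mesh.
; On pickup it prints a message, adds the resource to the instigator's BP_Inventory component and destroys itself.
; A getter exposes the resource, while the location and resource-query functions return only default values.
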(event Custom|SetMesh
  (params (Mesh :type Static%20Mesh%20Object%20Reference))
  (Components|StaticMesh|SetStaticMesh (Variables|Default|GetStaticMesh) Mesh))

(event EventPickupResource
  (params (Instagator :type Actor%20Object%20Reference))
  (Development|PrintString (Utilities|String|Append (Utilities|GetDisplayName Instagator) " picked up " (Utilities|String|ToString(Name) (Variables|Default|GetResouce%20Name))))
  (Default|AddtoInventory (Actor|GetComponentbyClass Instagator "/Game/Blueprints/Components/BP_Inventory.BP_Inventory_C") (Variables|Default|GetResource))
  (Actor|DestroyActor))

(fn ConstructionScript
  (bind _returnvalue (Utilities|GetDataTableRow (Variables|Default|GetResource%20Data%20Table) (Variables|Default|GetResouce%20Name))
    (:then
      (Variables|Default|SetResource _returnvalue)
      (Components|StaticMesh|SetStaticMesh (Variables|Default|GetStaticMesh) (.Mesh (Utilities|Struct|BreakS_Resources _returnvalue))))))

(fn GameplayTag
  (return "(TagName=\"Resource\")"))

(fn GetLocation1
  (return "0, 0, 0"))

(fn HasResource1
  (params (Resource%20Robot%20Is%20Looking%20For :type Name :default "None"))
  (return "None" 0 0))