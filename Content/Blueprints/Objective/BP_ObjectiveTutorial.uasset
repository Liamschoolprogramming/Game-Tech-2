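; BP_ObjectiveTutorial is the tutorial objective that guides the player through restoring power to the Main Core.
; It extends a parent objective's interaction with one-time staged dialogue: a first hint about Star Dust, then a Furnace hint once the inventory holds some.
; On completion it swaps the cylinder material, turns the light green, removes the objective widget and triggers the success dialogue.
; Each dialogue goes through the GameInstance, disabling movement and passing a cutscene stage.
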(event EventBeginPlay
  (|CallParentFunction))

(fn ConstructionScript
  (|CallParentFunction))

(fn PlayerInteract
  (params (Player :type BP%20FP%20Character%20Object%20Reference))
  (|CallParentFunction Player)
  (if (not (Widget|IsVisible (Variables|Default|GetObjectiveWidget)))
    (if (Variables|Default|GetInitialInteraction)
      (if (and (> (.Value (Utilities|Map|Find (Variables|/Game/Blueprints/Components/BP_Inventory.BP_Inventory_C|GetResource%20Inventory (Variables|Default|GetBP_Inventory)) "Star Dust")) 0) (not (Variables|Default|GetSecondInteraction)))
        (Variables|Default|SetSecondInteraction true)
        (Class|BPIGameInstance|CallDialogue(Message) (Game|GetGameInstance) (Utilities|Array|MakeArray "Star Dust alone won't fix the generator. " "To smelt Celestial Ore and Astral Ingots, you will need a Furnace.") false 6))
      (else
        (Variables|Default|SetInitialInteraction true)
        (Class|BPIGameInstance|CallDialogue(Message) (Game|GetGameInstance) (Utilities|Array|MakeArray "The first ingredient is Star Dust. ") false 4)))))

(fn CompletedObjective
  (Rendering|Material|SetMaterial (Variables|Default|GetCylinder) 0 "/Game/Blueprints/Objective/M_Objective.M_Objective")
  (Rendering|Components|Light|SetLightColor (Variables|Default|GetPointLight) "(R=0.216954,G=1.000000,B=0.000000,A=1.000000)" true)
  (Variables|Default|SetObjectiveState 0)
  (Widget|RemovefromParent (Variables|Default|GetObjectiveWidget))
  (Variables|/Script/Engine.PlayerController|SetbShowMouseCursor (Game|GetPlayerController 0) false)
  (Class|BPIGameInstance|CallDialogue(Message) (Game|GetGameInstance) (Utilities|Array|MakeArray "Excellent! You have successfully restored power to the Main Core. Unlocking the next wing of the Synthera.") false 11))