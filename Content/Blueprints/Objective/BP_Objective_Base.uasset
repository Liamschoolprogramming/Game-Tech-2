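; Base objective actor that takes resources from the interacting player into its own inventory.
; BeginPlay builds a name-to-index map, which Interact uses to look up both inventories and transfer the named resource.
; It then updates the HUD with the first slot's amount and the stored Celestial Ore amount.
; Crafting logic is unwired; location and resource query functions return defaults, while GameplayTag returns Objective.
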(event EventInteract
  (params (Player :type BP%20FP%20Character%20Object%20Reference))
  (bind _resourceinventory (Variables|Default|GetResourceInventory))
  (bind _resourceinventory_2 (Variables|/Game/Blueprints/Player/BP_FPCharacter.BP_FPCharacter_C|GetResourceInventory Player))
  (bind (_resourcename _resourceindex _resourceamount) (CallFunction|GetResourceValues _resourceinventory_2 (Variables|/Game/Blueprints/Player/BP_FPCharacter.BP_FPCharacter_C|GetResourceIndex Player) (Variables|Default|Getname)))
  (bind _resourceindex_2 (CallFunction|GetResourceValues (Variables|Default|GetResourceInventory) (Variables|Default|GetResourceIndex) (Variables|Default|Getname)))
  (bind _new_map_index (CallFunction|SetResourceBothDestinations _resourceindex _resourceamount _resourceinventory_2 _resourceinventory _resourceindex_2 (Variables|Default|GetResourceIndex) (Variables|Default|Getname)))
  (Utilities|FlowControl|Sequence
    (:then_0
      (Class|BPIUI|UpdateObjective(Message) (HUD|GetHUD (Game|GetPlayerController 0)) (Utilities|String|ToString(Integer) (.Amount (Utilities|Struct|BreakS_Resources (Utilities|Array|Get(acopy) _resourceinventory))))))
    (:then_1
      (bind _resourceamount_2 (CallFunction|GetResourceValues (Variables|Default|GetResourceInventory) (Variables|Default|GetResourceIndex) "Celestial Ore"))
      (Class|BPIUI|AmountNeeded(Message) (HUD|GetHUD (Game|GetPlayerController 0)) (Utilities|String|ToString(Integer) _resourceamount_2)))))

(event EventBeginPlay
  (CallFunction|InventoryMap (Variables|Default|GetResourceInventory) (Variables|Default|GetResourceIndex)))

(fn ConstructionScript)

(fn GameplayTag
  (return "(TagName=\"Objective\")"))

(fn GetLocation1
  (return "0, 0, 0"))

(fn HasResource1
  (params (Resource%20Robot%20Is%20Looking%20For :type Name :default "None"))
  (return "None" 0 0))