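; BP_SterileDoor is an objective door that opens by removing itself when its objective completes.
; On BeginPlay it finds the BP_LevelEventManager and subscribes itself as a BPI_Observer.
; ObjectiveActivate clears IsLocked, reports tutorial completion to the manager, then destroys the actor.
; The remaining functions, including machine, tag, location and resource queries, are stubs returning empty or default values.
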(event EventBeginPlay
  (bind _returnvalue (Actor|GetActorOfClass "/Game/Blueprints/LevelEventManager/BP_LevelEventManager.BP_LevelEventManager_C"))
  (Variables|Default|SetLevelEventManager _returnvalue)
  (bind _asbpi_observer (Utilities|Casting|CastToBPI_Observer self))
  (Default|SubscribeObserver (Variables|Default|GetLevelEventManager) _asbpi_observer))

(event EventObjectiveActivate
  ;[0.15 0.15 0.15 0.5] When objective complete, open door
  (Variables|Default|SetIsLocked false)
  (Default|TutorialCompleted (Variables|Default|GetLevelEventManager))
  (Actor|DestroyActor))

(fn ConstructionScript)

(fn GameplayTag
  (return ""))

(fn GetGameplayTags
  (return ""))

(fn GetLocation
  (return "0, 0, 0"))

(fn GetMachine
  (return 0))

(fn GetMachineClass
  (return 0))

(fn GetMachineMesh
  (return 0))

(fn GetName
  (return "None"))

(fn HasResource
  (params (Resource%20Name :type Name :default "None"))
  (return 0 false))