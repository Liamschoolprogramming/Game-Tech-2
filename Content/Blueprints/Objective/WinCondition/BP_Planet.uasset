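; BP_Planet is a planet actor that listens for the level's win condition as an observer.
; On BeginPlay it finds BP_LevelEventManager and subscribes itself through BPI_Observer.
; On a Win Condition notify it prints a message and caches the level's BP_LocationPoint.
; Timelines for scaling and for lerping its Y toward that point exist but are unwired, so the planet never moves.
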(event EventOnNotify
  (params (EventType :type E_LevelEventType%20Enum :default "NewEnumerator0"))
  (switch Utilities|FlowControl|Switch|SwitchonE_LevelEventType EventType
    (:NewEnumerator14
      (Development|PrintString "Win Condition")
      (bind _returnvalue (Actor|GetActorOfClass "/Game/Blueprints/Objective/WinCondition/BP_LocationPoint.BP_LocationPoint_C"))
      (Variables|Default|SetLocationPoint _returnvalue))))

(event EventBeginPlay
  (bind _returnvalue (Actor|GetActorOfClass "/Game/Blueprints/LevelEventManager/BP_LevelEventManager.BP_LevelEventManager_C"))
  (Variables|Default|SetLevelEventManager _returnvalue)
  (bind _asbpi_observer (Utilities|Casting|CastToBPI_Observer self))
  (Default|SubscribeObserver (Variables|Default|GetLevelEventManager) _asbpi_observer))

(fn ConstructionScript)