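; A tutorial door that removes itself from the level when the tutorial is completed.
; On BeginPlay it finds the BP_LevelEventManager and subscribes itself as a BPI_Observer.
; When notified of the Tutorial Completed event, it destroys its actor to open the way.
; ObjectiveActivate and the other getter functions, such as the machine and resource queries, are empty stubs returning defaults.
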(event EventBeginPlay
  (bind _returnvalue (Actor|GetActorOfClass "/Game/Blueprints/LevelEventManager/BP_LevelEventManager.BP_LevelEventManager_C"))
  (Variables|Default|SetLevelEventManager _returnvalue)
  (bind _asbpi_observer (Utilities|Casting|CastToBPI_Observer self))
  (Default|SubscribeObserver (Variables|Default|GetLevelEventManager) _asbpi_observer))

(event EventObjectiveActivate)

(event EventOnNotify
  (params (EventType :type E_LevelEventType%20Enum :default "NewEnumerator0"))
  ;[0.15 0.15 0.15 0.5] When objective complete, open door
  (switch Utilities|FlowControl|Switch|SwitchonE_LevelEventType EventType
    (:NewEnumerator12
      (Actor|DestroyActor))))

(fn ConstructionScript)

(fn GameplayTag
  (return ""))

(fn GetGameplayTags
  (return ""))

(fn GetLocation
  (return "0, 0, 0"))

(fn GetMachine
  (return 0))

(fn GetMachineClass
  (return 0))

(fn GetMachineMesh
  (return 0))

(fn GetName
  (return "None"))

(fn HasResource
  (params (Resource%20Name :type Name :default "None"))
  (return 0 false))