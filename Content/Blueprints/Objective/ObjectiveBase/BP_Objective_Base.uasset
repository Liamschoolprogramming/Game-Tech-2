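; Base actor for objective stations, which robots supply with resources to complete objectives that unlock player recipes.
; BeginPlay loads the recipe from DT_Recipes, seeds the inventory and registers with the level event manager; interacting toggles the terminal widget.
; Each drop-off updates the UI and checks requirements; completion notifies the game instance, then grants recipes or triggers the win condition.
; Unlocks are hard-coded by recipe name in both CompletedObjective and SetUnlocksFromRecipe.
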(event OnComponentBeginOverlap(InteractionBox)
  (params (OverlappedComponent :type Primitive%20Component%20Object%20Reference) (OtherActor :type Actor%20Object%20Reference) (OtherComp :type Primitive%20Component%20Object%20Reference) (OtherBodyIndex :type Integer) (bFromSweep :type Boolean) (SweepResult :type Hit%20Result%20Structure%20%28by%20ref%29))
  (bind _asbp_fpcharacter (Utilities|Casting|CastToBP_FPCharacter OtherActor))
  (Default|DisplayInputPrompt _asbp_fpcharacter "Press E to open objective terminal"))

(event OnComponentEndOverlap(InteractionBox)
  (params (OverlappedComponent :type Primitive%20Component%20Object%20Reference) (OtherActor :type Actor%20Object%20Reference) (OtherComp :type Primitive%20Component%20Object%20Reference) (OtherBodyIndex :type Integer))
  (bind _asbp_fpcharacter (Utilities|Casting|CastToBP_FPCharacter OtherActor))
  (Default|HideInputPrompt _asbp_fpcharacter))

(event Custom|Completed%20Objective
  (bind _recipe (Variables|Default|GetRecipe))
  (switch Utilities|FlowControl|Switch|SwitchonE_ObjectiveStatus (Variables|Default|GetObjectiveState)
    (:NewEnumerator0
      (Variables|Default|SetObjectiveState "NewEnumerator1")
      (Default|ObjectiveComplete (Variables|Default|GetBP%20Game%20Instance) (.name _recipe))
      (switch name (.name _recipe)
        (:Reinforce%20Transmitters
          (Class|BPIGameInstance|AddorRemovePlayerRecipe(Message) (Game|GetGameInstance) "Compressor" true)
          (Class|BPIGameInstance|AddorRemovePlayerRecipe(Message) (Game|GetGameInstance) "Furnace" true)
          (Class|BPIGameInstance|AddorRemovePlayerRecipe(Message) (Game|GetGameInstance) "Basic Turret" true)
          (CallFunction|NotifiyPlayer "Compressor")
          (Utilities|FlowControl|Delay 2.0)
          (CallFunction|NotifiyPlayer "Furnace")
          (Utilities|FlowControl|Delay 2.0)
          (CallFunction|NotifiyPlayer "Basic Turret"))
        (:Restore%20Thermoelectric%20Generators
          (Class|BPIGameInstance|AddorRemovePlayerRecipe(Message) (Game|GetGameInstance) "Robot Station" true)
          (Class|BPIGameInstance|AddorRemovePlayerRecipe(Message) (Game|GetGameInstance) "Fabricator" true)
          (CallFunction|NotifiyPlayer "Robot Station")
          (Utilities|FlowControl|Delay 2.0)
          (CallFunction|NotifiyPlayer "Fabricator"))
        (:Open%20Boiler%20Room%20Door
          (Class|BPIGameInstance|AddorRemovePlayerRecipe(Message) (Game|GetGameInstance) "Barricade" true)
          (Class|BPIGameInstance|AddorRemovePlayerRecipe(Message) (Game|GetGameInstance) "Combiner" true)
          (CallFunction|NotifiyPlayer "Barricade")
          (Utilities|FlowControl|Delay 2.0)
          (CallFunction|NotifiyPlayer "Combiner"))
        (:Fortify%20Boiler%20Pipeline
          (Class|BPIGameInstance|AddorRemovePlayerRecipe(Message) (Game|GetGameInstance) "Flame Thrower" true)
          (CallFunction|NotifiyPlayer "Flame Thrower"))
        (:Strengthen%20Heat%20Sink
          (Class|BPIGameInstance|AddorRemovePlayerRecipe(Message) (Game|GetGameInstance) "Teleporter" true)
          (Class|BPIGameInstance|AddorRemovePlayerRecipe(Message) (Game|GetGameInstance) "Synthesizer" true)
          (CallFunction|NotifiyPlayer "Teleporter")
          (Utilities|FlowControl|Delay 2.0)
          (CallFunction|NotifiyPlayer "Synthesizer"))
        (:Open%20Greenhouse%20Door
          (Class|BPIGameInstance|AddorRemovePlayerRecipe(Message) (Game|GetGameInstance) "Chain Shot" true)
          (CallFunction|NotifiyPlayer "Chain Shot")
          (Class|BPIGameInstance|AddorRemovePlayerRecipe(Message) (Game|GetGameInstance) "Empty Container" true)
          (CallFunction|NotifiyPlayer "Empty Container"))
        (:Decontaminate%20Bio%20Filter
          (Class|BPIGameInstance|AddorRemovePlayerRecipe(Message) (Game|GetGameInstance) "Bubble Shot" true)
          (CallFunction|NotifiyPlayer "Bubble Shot"))
        (:Pressurize%20Ventilation%20System
          (Class|BPIGameInstance|AddorRemovePlayerRecipe(Message) (Game|GetGameInstance) "Blackhole Trap" true)
          (Class|BPIGameInstance|AddorRemovePlayerRecipe(Message) (Game|GetGameInstance) "Refinery" true)
          (CallFunction|NotifiyPlayer "Blackhole Trap")
          (Utilities|FlowControl|Delay 2.0)
          (CallFunction|NotifiyPlayer "Refinery"))
        (:Activate%20Ship%20Engines
          (bind _returnvalue (Actor|GetActorOfClass "/Game/Blueprints/Objective/WinCondition/BP_WinCondition.BP_WinCondition_C"))
          (Default|WinConditionAction _returnvalue))))))

(event Custom|HasEnoughResources
  (CallFunction|CompletedObjective))

(event EventDropOffResource
  (params (ResourceName :type Name :default "None") (ResourceAmount :type Integer))
  ;[0.15 0.15 0.15 0.5] When robots drop off resources
  (Default|AddResourcetoInventory (Variables|Default|GetBP_Inventory) ResourceName ResourceAmount)
  (CallFunction|CheckResourceAmounts)
  (Default|UpdateResourcesInfo (Variables|Default|GetObjectiveWidget) (Variables|/Game/Blueprints/Components/BP_Inventory.BP_Inventory_C|GetResource%20Inventory (Variables|Default|GetBP_Inventory)))
  (Class|BPIUI|UpdateResourcesHUD(Message) (HUD|GetHUD (Game|GetPlayerController 0)) self))

(event EventBeginPlay
  ;[0.15 0.15 0.15 0.5] Begin play
  (CallFunction|SetGameInstance)
  (Components|Animation|PlayAnimation (Variables|Default|GetSkeletalMesh) "/Game/Assets/Objective_station/Animation/Objective_station_Floating_crystals.Objective_station_Floating_crystals" true)
  (bind _namenowhitespace (CallFunction|StripWhitespaceName (Variables|Default|GetName)))
  (bind _returnvalue (Utilities|GetDataTableRow "/Game/Blueprints/DT_Recipes.DT_Recipes" _namenowhitespace)
    (:then
      (Variables|Default|SetRecipe _returnvalue))
    (:RowNotFound
      (bind _namenowhitespace_2 (CallFunction|StripWhitespaceName (.name (Variables|Default|GetRecipe))))
      (bind _returnvalue_2 (Utilities|GetDataTableRow "/Game/Blueprints/DT_Recipes.DT_Recipes" _namenowhitespace_2)
        (:then
          (Variables|Default|SetRecipe _returnvalue_2)
          (Variables|Default|SetName (.name (Variables|Default|GetRecipe)))))))
  (CallFunction|GetResourcesfromRecipe)
  (for _array_element (Variables|/Game/Blueprints/Managers/BP_GameInstance.BP_GameInstance_C|GetObjectives (Variables|Default|GetBP%20Game%20Instance))
    (if (== (.DisplayName (Utilities|Struct|BreakS_Objective _array_element)) (Variables|Default|GetName))
      (Variables|Default|SetObjectiveIndex (.IDInternalName (Utilities|Struct|BreakS_Objective _array_element)))))
  (CallFunction|SubscribetoLevelEventManager)
  (CallFunction|SetObjectiveManager)
  (CallFunction|SetUnlocksfromRecipe))

(fn ConstructionScript)

(fn SubscribetoLevelEventManager
  (bind _returnvalue (Actor|GetActorOfClass "/Game/Blueprints/LevelEventManager/BP_LevelEventManager.BP_LevelEventManager_C"))
  (Variables|Default|SetLevelEventManager _returnvalue)
  (bind _asbpi_observer (Utilities|Casting|CastToBPI_Observer self))
  (Default|SubscribeObserver (Variables|Default|GetLevelEventManager) _asbpi_observer))

(fn PlayerInteract
  (params (Player :type BP%20FP%20Character%20Object%20Reference))
  (Utilities|IsValid (Variables|Default|GetObjectiveWidget)
    (:Is%20Valid
      _)
    (:Is%20Not%20Valid
      (bind _returnvalue (UserInterface|CreateWidget "/Game/UI/WidgetBlueprints/CraftingSystemMenus/W_ObjectiveTerminalMenu.W_ObjectiveTerminalMenu_C" 0 self))
      (Variables|Default|SetObjectiveWidget _returnvalue)
      (LocalVariables|SetL_ObjectiveGrid (Variables|/Game/UI/WidgetBlueprints/CraftingSystemMenus/W_ObjectiveTerminalMenu.W_ObjectiveTerminalMenu_C|GetW_InventoryGrid (Variables|Default|GetObjectiveWidget)))
      (Default|InitializeGridSlots (LocalVariables|GetL_ObjectiveGrid) 1 (Utilities|Map|Length (.requiredresources (Variables|Default|GetRecipe))))
      (Default|PopulateGrid (LocalVariables|GetL_ObjectiveGrid) (Variables|Default|GetBP_Inventory) (Variables|/Game/UI/WidgetBlueprints/CraftingSystemMenus/W_Inventory.W_Inventory_C|GetW_Hotbar (Variables|/Game/Blueprints/Player/BP_FPCharacter.BP_FPCharacter_C|GetInventoryUI Player)))
      (Variables|/Game/UI/WidgetBlueprints/CraftingSystemMenus/W_InventoryGrid.W_InventoryGrid_C|SetInteractable (LocalVariables|GetL_ObjectiveGrid) self)
      (Default|InitRecipesData (Variables|Default|GetObjectiveWidget) (Variables|Default|GetRecipe) (Variables|Default|GetRecipesToUnlock))
      (Default|SetSlotsMaxCapacity (LocalVariables|GetL_ObjectiveGrid) (.requiredresources (Variables|Default|GetRecipe)))))
  (if (Widget|IsVisible (Variables|Default|GetObjectiveWidget))
    (Widget|RemovefromParent (Variables|Default|GetObjectiveWidget))
    (Input|SetInputModeGameOnly (Game|GetPlayerController 0) false)
    (Variables|/Script/Engine.PlayerController|SetbShowMouseCursor (Game|GetPlayerController 0) false)
    (Variables|/Game/Blueprints/Player/BP_FPCharacter.BP_FPCharacter_C|SetMovementEnabled Player true)
    (Variables|/Game/Blueprints/Player/BP_FPCharacter.BP_FPCharacter_C|SetMenuOpen Player false)
    (Default|ToggleReticle Player true)
    (else
      (UserInterface|Viewport|AddtoViewport (Variables|Default|GetObjectiveWidget) 0)
      (Input|SetInputModeGameandUI (Game|GetPlayerController 0) (Variables|Default|GetObjectiveWidget) "DoNotLock" true false)
      (Variables|/Script/Engine.PlayerController|SetbShowMouseCursor (Game|GetPlayerController 0) true)
      (Variables|/Game/Blueprints/Player/BP_FPCharacter.BP_FPCharacter_C|SetMovementEnabled Player false)
      (Variables|/Game/Blueprints/Player/BP_FPCharacter.BP_FPCharacter_C|SetMenuOpen Player true)
      (Default|ToggleReticle Player false))))

(fn SetObjectiveManager
  (bind _returnvalue (Actor|GetActorOfClass "/Game/Blueprints/Managers/BP_ObjectiveManager.BP_ObjectiveManager_C"))
  (Variables|Default|SetObjectiveManager _returnvalue))

(fn SetGameInstance
  (bind _asbp_game_instance (Utilities|Casting|CastToBP_GameInstance (Game|GetGameInstance)))
  (Variables|Default|SetBP%20Game%20Instance _asbp_game_instance))

(fn GetResourcesfromRecipe
  (bind _keypin (Utilities|Map|ForEachLoop(Map) (.requiredresources (Variables|Default|GetRecipe)))
    (:then
      (Default|AddResourcetoInventory (Variables|Default|GetBP_Inventory) _keypin))))

(fn CheckResourceAmounts
  (bind (_keypin _valuepin) (Utilities|Map|ForEachLoop(Map) (.requiredresources (Variables|Default|GetRecipe)))
    (:then
      (bind _resource_amount (Default|GetResourceAmount (Variables|Default|GetBP_Inventory) _keypin))
      (if (< _resource_amount _valuepin)
        (LocalVariables|SetL_NotEnoughResources true)))
    (:CompletedPin
      (if (not (LocalVariables|GetL_NotEnoughResources))
        (CallFunction|HasEnoughResources)))))

(fn NotifiyPlayer
  (params (Recipe%20Name :type Name))
  (bind _namenowhitespace (CallFunction|StripWhitespaceName Recipe%20Name))
  (bind _returnvalue (Utilities|GetDataTableRow "/Game/Blueprints/DT_Machines.DT_Machines" _namenowhitespace)
    (:then
      (bind _returnvalue_2 (UserInterface|CreateWidget "/Game/UI/WidgetBlueprints/WB_RecipeUnlockNotify.WB_RecipeUnlockNotify_C" 0 (.Icon (Utilities|Struct|BreakS_Machine_InventoryData _returnvalue)) Recipe%20Name))
      (bind _w_hud (Class|BPIUI|GetHUDWigdet(Message) (HUD|GetHUD (Game|GetPlayerController 0))))
      (Class|VerticalBox|AddChildtoVerticalBox (Variables|/Game/UI/WidgetBlueprints/HUD/W_HUD.W_HUD_C|GetResourcePickupBox _w_hud) _returnvalue_2))
    (:RowNotFound
      (bind _namenowhitespace_2 (CallFunction|StripWhitespaceName Recipe%20Name))
      (bind _returnvalue_3 (Utilities|GetDataTableRow "/Game/Blueprints/DT_Artillery.DT_Artillery" _namenowhitespace_2)
        (:then
          (bind _returnvalue_4 (UserInterface|CreateWidget "/Game/UI/WidgetBlueprints/WB_RecipeUnlockNotify.WB_RecipeUnlockNotify_C" 0 (.Icon (Utilities|Struct|BreakS_Machine_InventoryData _returnvalue_3)) Recipe%20Name))
          (bind _w_hud_2 (Class|BPIUI|GetHUDWigdet(Message) (HUD|GetHUD (Game|GetPlayerController 0))))
          (Class|VerticalBox|AddChildtoVerticalBox (Variables|/Game/UI/WidgetBlueprints/HUD/W_HUD.W_HUD_C|GetResourcePickupBox _w_hud_2) _returnvalue_4))))))

(fn SetUnlocksfromRecipe
  (Utilities|Array|Clear (Variables|Default|GetRecipesToUnlock))
  (switch name (.name (Variables|Default|GetRecipe))
    (:Reinforce%20Transmitters
      (Utilities|Array|Add (Variables|Default|GetRecipesToUnlock) "Compressor")
      (Utilities|Array|Add (Variables|Default|GetRecipesToUnlock) "Furnace")
      (Utilities|Array|Add (Variables|Default|GetRecipesToUnlock) "Basic Turret"))
    (:Restore%20Thermoelectric%20Generators
      (Utilities|Array|Add (Variables|Default|GetRecipesToUnlock) "Robot Station")
      (Utilities|Array|Add (Variables|Default|GetRecipesToUnlock) "Fabricator"))
    (:Open%20Boiler%20Room%20Door
      (Utilities|Array|Add (Variables|Default|GetRecipesToUnlock) "Barricade")
      (Utilities|Array|Add (Variables|Default|GetRecipesToUnlock) "Combiner"))
    (:Fortify%20Boiler%20Pipeline
      (Utilities|Array|Add (Variables|Default|GetRecipesToUnlock) "Flame Thrower"))
    (:Strengthen%20Heat%20Sink
      (Utilities|Array|Add (Variables|Default|GetRecipesToUnlock) "Teleporter")
      (Utilities|Array|Add (Variables|Default|GetRecipesToUnlock) "Synthesizer"))
    (:Open%20Greenhouse%20Door
      (Utilities|Array|Add (Variables|Default|GetRecipesToUnlock) "Chain Shot")
      (Utilities|Array|Add (Variables|Default|GetRecipesToUnlock) "Empty Container"))
    (:Decontaminate%20Bio%20Filter
      (Utilities|Array|Add (Variables|Default|GetRecipesToUnlock) "Bubble Shot"))
    (:Pressurize%20Ventilation%20System
      (Utilities|Array|Add (Variables|Default|GetRecipesToUnlock) "Blackhole Trap")
      (Utilities|Array|Add (Variables|Default|GetRecipesToUnlock) "Refinery"))))

(fn GameplayTag
  (return "(TagName=\"Objective\")"))

(fn GetGameplayTags
  (return "(GameplayTags=((TagName=\"Objective\")))"))

(fn GetIndicatorMesh
  (return 0))

(fn GetLocation
  (return (Transformation|GetActorLocation)))

(fn GetMachine
  (return 0))

(fn GetMachineClass
  (return (Utilities|GetClass self)))

(fn GetMachineMesh
  (return 0))

(fn GetName
  (return (Variables|Default|GetName)))

(fn GetRotation
  (return 0.0))

(fn HasResource
  (params (Resource%20Name :type Name :default "None"))
  (bind _resource_amount (Default|GetResourceAmount (Variables|Default|GetBP_Inventory) Resource%20Name))
  (return _resource_amount (> _resource_amount 0)))

(fn Interact
  (params (Player :type BP%20FP%20Character%20Object%20Reference))
  (CallFunction|PlayerInteract Player)
  (return (Variables|Default|GetObjectiveWidget)))