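; BP_ObjectiveMinor is a minor objective Blueprint that acts as a one-time recipe unlock once its resource requirement is met.
; The HasEnoughResources event calls UnlockRecipe the first time and sets a RecipeUnlocked flag, so later triggers only print an already-unlocked message.
; UnlockRecipe is currently a stub that prints debug strings for unlocking the Robot Station and Robots.
; BeginPlay and Player Interact simply defer to the parent class.
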(event EventBeginPlay
  (|CallParentFunction))

(event EventHasEnoughResources
  (if (not (Variables|Default|GetRecipeUnlocked))
    (CallFunction|UnlockRecipe)
    (Variables|Default|SetRecipeUnlocked true)
    (else
      (Development|PrintString "Already unlocked the recipe"))))

(fn ConstructionScript)

(fn UnlockRecipe
  (Development|PrintString "Unlock Robot Station")
  (Development|PrintString "Unlock Robots"))

(fn PlayerInteract
  (params (Player :type BP%20FP%20Character%20Object%20Reference))
  (|CallParentFunction Player))