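; BP_EngineCore is a damageable, repairable engine core (Bridge, Boiler or Overgrown) that generates its own resource and powers machines on a grid.
; Bridge starts online, while the others initialize on unlock events from BP_LevelEventManager, which also triggers save restoration.
; While active, a delayed self-calling event fills the inventory that players open through a widget.
; Machines reserve energy from a fixed budget and are notified when zero health disables the core.
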(event OnComponentBeginOverlap(InputInteractionBox)
  (params (OverlappedComponent :type Primitive%20Component%20Object%20Reference) (OtherActor :type Actor%20Object%20Reference) (OtherComp :type Primitive%20Component%20Object%20Reference) (OtherBodyIndex :type Integer) (bFromSweep :type Boolean) (SweepResult :type Hit%20Result%20Structure%20%28by%20ref%29))
  ;[0.15 0.15 0.15 0.5] Show Interact Prompt When Close To Player and Hide When Player Leaves
  (if (not (Utilities|DoesObjectImplementInterface OtherActor "/Game/Blueprints/Robot/BPI_Robot.BPI_Robot_C"))
    (if (< (Variables|Default|GetHealth) (Variables|Default|GetMaxHealth))
      (bind _asbp_fpcharacter (Utilities|Casting|CastToBP_FPCharacter OtherActor))
      (Default|DisplayInputPrompt _asbp_fpcharacter "Press E to Interact & R to Repair")
      (else
        (bind _asbp_fpcharacter_2 (Utilities|Casting|CastToBP_FPCharacter OtherActor))
        (Default|DisplayInputPrompt _asbp_fpcharacter_2 "Press E to Interact")))))

(event OnComponentEndOverlap(InputInteractionBox)
  (params (OverlappedComponent :type Primitive%20Component%20Object%20Reference) (OtherActor :type Actor%20Object%20Reference) (OtherComp :type Primitive%20Component%20Object%20Reference) (OtherBodyIndex :type Integer))
  ;[0.15 0.15 0.15 0.5] Show Interact Prompt When Close To Player and Hide When Player Leaves
  (if (not (Utilities|DoesObjectImplementInterface OtherActor "/Game/Blueprints/Robot/BPI_Robot.BPI_Robot_C"))
    (bind _asbp_fpcharacter (Utilities|Casting|CastToBP_FPCharacter OtherActor))
    (Default|HideInputPrompt _asbp_fpcharacter)))

(event Custom|InitializeCoreOnline
  ;[0.15 0.15 0.15 0.5] Begin Functions When Core Unlocked (Bridge unlocked by default)
  (Rendering|SetVisibility (Variables|Default|GetHP%20Widget) true false)
  (Variables|Default|SetIsActive true)
  (CallFunction|GenerateResources))

(event Custom|CoreDisable
  ;[0.15 0.15 0.15 0.5] Handle activating/deactivating
  (CallFunction|SetActive false)
  (Default|CoreStatusCheck (Variables|Default|GetCoreManager))
  (bind _keypin (Utilities|Map|ForEachLoop(Map) (Variables|Default|GetMachines%20on%20Grid%20+%20Cost))
    (:then
      (Class|BPIMachine|ReceiveEnergy(Message) _keypin self (Variables|Default|GetIsActive)))))

(event Custom|GenerateResources
  ;[0.15 0.15 0.15 0.5] Generate star dust
  (if (Variables|Default|GetIsActive)
    (switch name (Variables|Default|GetName)
      (:Default
        (Default|AddResourcetoInventory (Variables|Default|GetBP_Inventory) (Utilities|Name|MakeLiteralName "Star Dust") (Variables|Default|GetResourceGenRate) :!label _label)
        (bind _resource_amount (Default|GetResourceAmount (Variables|Default|GetBP_Inventory) "Star Dust"))
        (Default|SetResourceQuantity (Variables|Default|GetCore%20Inventory%20Widget) _resource_amount)
        (Utilities|FlowControl|Delay (Variables|Default|GetResourceGenDelay))
        (CallFunction|GenerateResources))
      (:bridge
        (goto _label))
      (:boiler
        (Default|AddResourcetoInventory (Variables|Default|GetBP_Inventory) (Utilities|Name|MakeLiteralName "Plasma") (Variables|Default|GetResourceGenRate))
        (bind _resource_amount_2 (Default|GetResourceAmount (Variables|Default|GetBP_Inventory) "Plasma"))
        (Default|SetResourceQuantity (Variables|Default|GetCore%20Inventory%20Widget) _resource_amount_2)
        (Utilities|FlowControl|Delay (Variables|Default|GetResourceGenDelay))
        (CallFunction|GenerateResources))
      (:overgrown
        (Default|AddResourcetoInventory (Variables|Default|GetBP_Inventory) (Utilities|Name|MakeLiteralName "Cell") (Variables|Default|GetResourceGenRate))
        (bind _resource_amount_3 (Default|GetResourceAmount (Variables|Default|GetBP_Inventory) "Star Dust"))
        (Default|SetResourceQuantity (Variables|Default|GetCore%20Inventory%20Widget) _resource_amount_3)
        (Utilities|FlowControl|Delay (Variables|Default|GetResourceGenDelay))
        (CallFunction|GenerateResources)))))

(event Custom|RepairLoop
  (bind _maxhealth (Variables|Default|GetMaxHealth))
  ;[0.15 0.15 0.15 0.5] Start repair timer when holding R and stop when R is released - Set player state to repairing if health isn't full, otherise cancel this event - Also stop if repairing finishes
  (if (< (Variables|Default|GetHealth) (Variables|Default|GetMaxHealth))
    (bind _output_get (Variables|Default|SetHealth (Math|Float|Clamp(Float) (+ (Variables|Default|GetHealth) 1.0) 0.0 _maxhealth)))
    (CallFunction|UpdateHealthBar)
    (Default|DisplayRepairing (stale EventRepair Player) _output_get _maxhealth true)
    (if (not (Variables|Default|GetIsActive))
      (CallFunction|SetActive true))
    (else
      (Utilities|Time|ClearandInvalidateTimerbyHandle (Variables|Timers|GetRepairTimer))
      (Default|DisplayRepairing (stale EventRepair Player) (Variables|Default|GetHealth) (Variables|Default|GetMaxHealth) false))))

(event Custom|SetActive
  (params (ActiveStatus :type Boolean))
  (bind _ns_powerradius (Variables|Default|GetNS_PowerRadius))
  (bind _ns_powerradius_2 (Variables|Default|GetNS_PowerRadius))
  ;[0.15 0.15 0.15 0.5] Handle activating/deactivating
  (bind _output_get (Variables|Default|SetIsActive ActiveStatus))
  (if _output_get
    (Effects|Components|ParticleSystem|SetBoolParameter _ns_powerradius "Bool_Color" true)
    (if (not (Components|Activation|IsActive _ns_powerradius_2))
      (Components|Activation|Activate _ns_powerradius_2 false))
    (else
      (Effects|Components|ParticleSystem|SetBoolParameter _ns_powerradius "Bool_Color" false))))

(event Custom|Set%20Powered%20By%20Text
  (bind _poweredbytext (Variables|Default|GetPoweredByText))
  ;[0.15 0.15 0.15 0.5] Set Text Render PoweredByText and Color (temp)
  (Rendering|Components|TextRender|SetText _poweredbytext (Utilities|String|SelectText "Active" "Inactive" (Variables|Default|GetIsActive)))
  (Rendering|Components|TextRender|SetTextRenderColor _poweredbytext (select (Variables|Default|GetIsActive) (Class|KismetMathLibrary|LinearColortoRGBE "(R=0.000000,G=1.000000,B=0.327778,A=1.000000)") (Class|KismetMathLibrary|LinearColortoRGBE "(R=0.679543,G=0.005182,B=0.040915,A=1.000000)"))))

(event Game|Damage|EventAnyDamage
  (params (Damage :type Float%20%28single-precision%29) (DamageType :type Damage%20Type%20Object%20Reference) (InstigatedBy :type Controller%20Object%20Reference) (DamageCauser :type Actor%20Object%20Reference))
  ;[0.15 0.15 0.15 0.5] Damage
  (if (> (Variables|Default|GetHealth) 0)
    (bind _output_get (Variables|Default|SetHealth (- (Variables|Default|GetHealth) Damage)))
    (CallFunction|UpdateHealthBar)
    (if (<= _output_get 0)
      (CallFunction|CoreDisable))))

(event EventBeginPlay
  ;[0.15 0.15 0.15 0.5] Begin Play
  (CallFunction|UpdateHealthBar)
  (bind _returnvalue (Game|SpawnActorfromClass "/Game/Blueprints/Managers/BP_CoreManager.BP_CoreManager_C" (Transformation|GetActorTransform) "Undefined" "MultiplyWithRoot" 0 0))
  (Variables|Default|SetCoreManager _returnvalue)
  (CallFunction|SetPoweredbyText)
  (for _array_element (Components|GetChildrenComponents (Variables|Default|GetArrow) false)
    (Utilities|Array|Add (Variables|Default|GetTargetLocations) (Transformation|GetWorldLocation _array_element)))
  (bind _returnvalue_2 (UserInterface|CreateWidget "/Game/UI/WidgetBlueprints/CoreUI/W_CoreInventory.W_CoreInventory_C" 0 self))
  (Variables|Default|SetCore%20Inventory%20Widget _returnvalue_2)
  (bind _returnvalue_3 (Actor|GetActorOfClass "/Game/Blueprints/LevelEventManager/BP_LevelEventManager.BP_LevelEventManager_C"))
  (Variables|Default|SetLevelEventManager _returnvalue_3)
  (Default|SubscribeObserver (Variables|Default|GetLevelEventManager) self)
  (Rendering|SetVisibility (Variables|Default|GetHP%20Widget) false false)
  (switch name (Variables|Default|GetName)
    (:bridge
      (CallFunction|InitializeCoreOnline))))

(event EventInteract
  (params (Player :type BP%20FP%20Character%20Object%20Reference))
  ;[0.15 0.15 0.15 0.5] Player Interacts with Core
  (CallFunction|PlayerInteract Player))

(event EventPickupResource
  (params (Instigator :type Actor%20Object%20Reference) (ResourceName :type Name :default "None") (Amount :type Integer))
  (bind _asbp_fpcharacter (Utilities|Casting|CastToBP_FPCharacter (Game|GetPlayerCharacter 0)))
  (bind _resource_amount (Default|GetResourceAmount (Variables|Default|GetBP_Inventory) ResourceName))
  (if (> _resource_amount 0)
    (CallFunction|SetResourceBothDestinations Amount ResourceName (Variables|Default|GetBP_Inventory) (Variables|/Game/Blueprints/Player/BP_FPCharacter.BP_FPCharacter_C|GetBP_Inventory _asbp_fpcharacter))
    (bind _resource_amount_2 (Default|GetResourceAmount (Variables|Default|GetBP_Inventory) ResourceName))
    (Default|SetResourceQuantity (Variables|Default|GetCore%20Inventory%20Widget) _resource_amount_2)))

(event EventRepair
  (params (Player :type BP%20FP%20Character%20Object%20Reference) (Repairing? :type Boolean))
  ;[0.15 0.15 0.15 0.5] Start repair timer when holding R and stop when R is released - Set player state to repairing if health isn't full, otherise cancel this event - Also stop if repairing finishes
  (if Repairing?
    (if (< (Variables|Default|GetHealth) (Variables|Default|GetMaxHealth))
      (Variables|/Game/Blueprints/Player/BP_FPCharacter.BP_FPCharacter_C|SetPlayerStates Player "NewEnumerator6")
      (Utilities|Time|ClearandInvalidateTimerbyHandle (Variables|Timers|GetRepairTimer))
      (bind _returnvalue (Utilities|Time|SetTimerbyEvent (delegate Custom|RepairLoop) 0.2 true))
      (Variables|Timers|SetRepairTimer _returnvalue))
    (else
      (Utilities|Time|ClearandInvalidateTimerbyHandle (Variables|Timers|GetRepairTimer))
      (Default|DisplayRepairing Player (Variables|Default|GetHealth) (Variables|Default|GetMaxHealth) false))))

(event EventOnNotify
  (params (EventType :type E_LevelEventType%20Enum :default "NewEnumerator0"))
  (switch Utilities|FlowControl|Switch|SwitchonE_LevelEventType EventType
    (:NewEnumerator7
      (CallFunction|ResetCoreHealthInventoryonLoad))
    (:NewEnumerator8
      (switch name (Variables|Default|GetName)
        (:boiler
          (CallFunction|InitializeCoreOnline))))
    (:NewEnumerator9
      (switch name (Variables|Default|GetName)
        (:overgrown
          (CallFunction|InitializeCoreOnline))))))

(event EventRemoveResource
  (params (Resource%20Name :type Name :default "None") (Amount%20To%20Remove :type Integer) (Resource%20Index :type Integer))
  (Default|RemoveResourcefromInventory (Variables|Default|GetBP_Inventory) Resource%20Name Amount%20To%20Remove))

(event EventDropOffResource
  (params (ResourceName :type Name :default "None") (ResourceAmount :type Integer))
  (Default|AddResourcetoInventory (Variables|Default|GetBP_Inventory) ResourceName ResourceAmount))

(fn ConstructionScript
  (Variables|Default|SetHealth (Variables|Default|GetMaxHealth))
  (Variables|Default|SetEnergy (Variables|Default|GetMaxEnergy))
  (Effects|Components|ParticleSystem|SetFloatParameter (Variables|Default|GetNS_PowerRadius) "Uniform Sprite Size" (* 4.5e+03 1.73)))

(fn UpdateHealthBar
  (bind _aswb_healthbar (Utilities|Casting|CastToWB_Healthbar (UserInterface|GetUserWidgetObject (Variables|Default|GetHP%20Widget))))
  (Variables|/Game/UI/WidgetBlueprints/CoreUI/WB_Healthbar.WB_Healthbar_C|SetHealth _aswb_healthbar (Variables|Default|GetHealth))
  (Variables|/Game/UI/WidgetBlueprints/CoreUI/WB_Healthbar.WB_Healthbar_C|SetMax%20Health _aswb_healthbar (Variables|Default|GetMaxHealth))
  (return))

(fn FindRandomLocationinRadius
  (params (FromTransform :type Transform) (Radius :type Float%20%28double-precision%29))
  (bind _returnvalue (Math|Random|RandomFloatinRange 2e+02 Radius))
  (bind _returnvalue_2 (Math|Random|RandomUnitVector))
  (bind _returnvalue_3 (* _returnvalue_2 _returnvalue))
  (bind _returnvalue_4 (+ _returnvalue_3 (.location FromTransform)))
  (return (Math|Transform|MakeTransform (Math|Vector|MakeVector (.x _returnvalue_4) (.y _returnvalue_4) (- (.Z (Math|Vector|BreakVector (.location FromTransform))) 5e+01)) "0, 0, 0" "5.000000,5.000000,5.000000")))

(fn VerifyDependentMachine
  (params (Machine :type Actor%20Object%20Reference) (Energy%20Cost :type Integer) (Added%20to%20Grid? :type Boolean))
  ;[0.15 0.15 0.15 0.5] Observe a request by a machine to be added or removed from the power grid - then allocate or stop allocating energy to that machine
  (if (.ReturnValue (Utilities|Map|Find (Variables|Default|GetMachines%20on%20Grid%20+%20Cost) Machine))
    (if (not Added%20to%20Grid?)
      (Utilities|Map|Remove (Variables|Default|GetMachines%20on%20Grid%20+%20Cost) Machine)
      (Variables|Default|SetEnergy (Math|Integer|Clamp(Integer) (+ (Variables|Default|GetEnergy) Energy%20Cost) 0 (Variables|Default|GetMaxEnergy)))
      (Class|BPIMachine|ReceiveEnergy(Message) Machine self (Variables|Default|GetIsActive) :!label _label))
    (elif Added%20to%20Grid?
      (if (>= (Variables|Default|GetEnergy) Energy%20Cost)
        (Utilities|Map|Add (Variables|Default|GetMachines%20on%20Grid%20+%20Cost) Machine Energy%20Cost)
        (Variables|Default|SetEnergy (Math|Integer|Clamp(Integer) (- (Variables|Default|GetEnergy) Energy%20Cost) 0 (Variables|Default|GetMaxEnergy)))
        (goto _label)
        (else
          (Class|BPIMachine|ReceiveEnergy(Message) Machine self false))))))

(fn PlayerInteract
  (params (Player :type BP%20FP%20Character%20Object%20Reference))
  ;[0.15 0.15 0.15 0.5] Open Menu on Interact Key Pressed, and close on same key press
  (if (Widget|IsVisible (Variables|Default|GetCore%20Inventory%20Widget))
    (Widget|RemovefromParent (Variables|Default|GetCore%20Inventory%20Widget))
    (Input|SetInputModeGameOnly (Game|GetPlayerController 0) false)
    (Variables|/Script/Engine.PlayerController|SetbShowMouseCursor (Game|GetPlayerController 0) false)
    (Variables|/Game/Blueprints/Player/BP_FPCharacter.BP_FPCharacter_C|SetMovementEnabled Player true)
    (Variables|/Game/Blueprints/Player/BP_FPCharacter.BP_FPCharacter_C|SetMenuOpen Player false)
    (else
      (UserInterface|Viewport|AddtoViewport (Variables|Default|GetCore%20Inventory%20Widget) 0)
      (Input|SetInputModeGameandUI (Game|GetPlayerController 0) (Variables|Default|GetCore%20Inventory%20Widget) "DoNotLock" true false)
      (Variables|/Script/Engine.PlayerController|SetbShowMouseCursor (Game|GetPlayerController 0) true)
      (Variables|/Game/Blueprints/Player/BP_FPCharacter.BP_FPCharacter_C|SetMovementEnabled Player false)
      (Variables|/Game/Blueprints/Player/BP_FPCharacter.BP_FPCharacter_C|SetMenuOpen Player true)
      (Variables|/Game/UI/WidgetBlueprints/CoreUI/W_CoreInventory.W_CoreInventory_C|SetPlayer (Variables|Default|GetCore%20Inventory%20Widget) Player))))

(fn ResetCoreHealthInventoryonLoad
  (bind _asbp_game_instance (Utilities|Casting|CastToBP_GameInstance (Game|GetGameInstance)))
  (LocalVariables|SetSaveFile (Variables|/Game/Blueprints/Managers/BP_GameInstance.BP_GameInstance_C|GetCurrentSaveFIle _asbp_game_instance))
  (bind _resource (CallFunction|GetCoreResourceName))
  (Default|ResetResourceInventorytoAmount (Variables|Default|GetBP_Inventory) _resource (.Value (Utilities|Map|Find (Variables|/Game/Blueprints/Managers/SaveGameData/BP_SaveGame.BP_SaveGame_C|GetCoreInventories (LocalVariables|GetSaveFile)) (Variables|Default|GetName))))
  (bind _output_get (Variables|Default|SetHealth (.Value (Utilities|Map|Find (Variables|/Game/Blueprints/Managers/SaveGameData/BP_SaveGame.BP_SaveGame_C|GetCoreHealths (LocalVariables|GetSaveFile)) (Variables|Default|GetName)))))
  (CallFunction|UpdateHealthBar)
  (if (> _output_get 0.0)
    (CallFunction|SetActive true)
    (bind _returnvalue (Actor|GetActorOfClass "/Game/Blueprints/LevelEventManager/BP_LevelEventManager.BP_LevelEventManager_C"))
    (Default|NotifyCoreOnline _returnvalue)))

(fn GetCoreResourceName
  (switch name (Variables|Default|GetName)
    (:Default
      _)
    (:Boiler
      (return "Plasma"))
    (:Overgrown
      (return "Cell"))
    (:Bridge
      _))
  (return "Star Dust"))

(fn GameplayTag
  (return "(TagName=\"Interactable\")"))

(fn GetMachineHealth
  (return 0.0 0.0))

(fn GetGameplayTags
  (return (Variables|Default|GetGameplay%20Tags)))

(fn GetLocation
  (return (Transformation|GetWorldLocation (Variables|Default|GetArrow))))

(fn GetMachine
  (return 0))

(fn GetMachineClass
  (return 0))

(fn GetMachineMesh
  (return 0))

(fn GetName
  (return (Variables|Default|GetName)))

(fn HasResource
  (params (Resource%20Name :type Name :default "None"))
  (bind _resource_amount (Default|GetResourceAmount (Variables|Default|GetBP_Inventory) Resource%20Name))
  (return _resource_amount (> _resource_amount 0)))