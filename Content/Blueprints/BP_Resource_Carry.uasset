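; BP_Resource_Carry is an actor that displays a resource, apparently while it is carried.
; The construction script looks up the resource's row in a data table by name and sets the static mesh.
; BeginPlay subscribes to the level event manager and applies a skeletal mesh for Star Dust, static otherwise.
; It destroys itself on a Load Game notification; most interface-style getters and Interact are empty stubs.
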(event Custom|SetMesh
  (params (Mesh :type Static%20Mesh%20Object%20Reference))
  (Components|StaticMesh|SetStaticMesh (Variables|Default|GetStatic%20Mesh) Mesh))

(event Custom|SetSkeletalMesh
  (params (SkeletalMesh :type Skeletal%20Mesh%20Object%20Reference))
  (Components|SkeletalMesh|SetSkeletalMeshAsset (Variables|Default|GetSkeletalMesh) SkeletalMesh))

(event EventOnNotify
  (params (EventType :type E_LevelEventType%20Enum :default "NewEnumerator0"))
  (switch Utilities|FlowControl|Switch|SwitchonE_LevelEventType EventType
    (:NewEnumerator7
      (Actor|DestroyActor))))

(event EventBeginPlay
  (bind _resource (Variables|Default|GetResource))
  (bind _returnvalue (Actor|GetActorOfClass "/Game/Blueprints/LevelEventManager/BP_LevelEventManager.BP_LevelEventManager_C"))
  (CallFunction|SubscribeLevelEventManager self _returnvalue)
  (switch name (.name _resource)
    (:Default
      (CallFunction|SetMesh (.mesh _resource)))
    (:Star%20Dust
      (CallFunction|SetSkeletalMesh (.skeletalmesh _resource)))))

(fn ConstructionScript
  (bind _namenowhitespace (CallFunction|StripWhitespaceName (Variables|Default|GetResouce%20Name)))
  (bind _returnvalue (Utilities|GetDataTableRow (Variables|Default|GetResource%20Data%20Table) _namenowhitespace)
    (:then
      (Variables|Default|SetResource _returnvalue)
      (Components|StaticMesh|SetStaticMesh (Variables|Default|GetStatic%20Mesh) (.Mesh (Utilities|Struct|BreakS_Resources _returnvalue))))))

(fn GameplayTag
  (return "(TagName=\"Resource\")"))

(fn GetGameplayTags
  (return (Variables|Default|GetGameplay%20Tags)))

(fn GetIndicatorMesh
  (return 0))

(fn GetLocation
  (return "0, 0, 0"))

(fn GetMachine
  (return 0))

(fn GetMachineClass
  (return 0))

(fn GetMachineMesh
  (return 0))

(fn GetName
  (return "None"))

(fn GetRotation
  (return 0.0))

(fn HasResource
  (params (Resource%20Name :type Name :default "None"))
  (return 0 false))

(fn Interact
  (params (Player :type BP%20FP%20Character%20Object%20Reference))
  (return 0))