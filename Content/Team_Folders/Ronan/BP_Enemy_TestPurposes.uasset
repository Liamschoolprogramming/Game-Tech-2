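; BP_Enemy_TestPurposes is a test enemy that, on BeginPlay, targets the first turret found and walks to it via AIMoveTo.
; Health starts at MaxHealth in the construction script; damage sets it to Damage minus Health, apparently reversed operands, destroying the actor at zero or below.
; Attack only prints a message and is never called here.
; Health, location and resource query functions are stubs returning default values.
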(event EventAttack
  (Development|PrintString "Attack!"))

(event EventNavigatetoAttackTarget
  (bind _movementresult (AI|AIMoveTo self (.location (Transformation|GetActorTransform (Variables|Default|GetAttackTarget))) 0 1.0 false)
    (:then
      (Development|PrintString (Utilities|String|EnumtoString _movementresult)))))

(event Game|Damage|EventAnyDamage
  (params (Damage :type Float%20%28single-precision%29) (DamageType :type Damage%20Type%20Object%20Reference) (InstigatedBy :type Controller%20Object%20Reference) (DamageCauser :type Actor%20Object%20Reference))
  (Variables|Default|SetHealth (- Damage (Variables|Default|GetHealth)))
  (if (<= (Variables|Default|GetHealth) 0.0)
    (Actor|DestroyActor)))

(event EventSetAttackTarget
  (params (AttackTarget :type Actor%20Object%20Reference))
  (Variables|Default|SetAttackTarget AttackTarget)
  (CallFunction|NavigatetoAttackTarget))

(event EventBeginPlay
  (bind _outactors (Actor|GetAllActorsOfClass "/Game/Blueprints/Machines/Turret/BP_Turret_Base.BP_Turret_Base_C"))
  (CallFunction|SetAttackTarget (Utilities|Array|Get(acopy) _outactors)))

(fn ConstructionScript
  (Variables|Default|SetHealth (Variables|Default|GetMax%20Health)))

(fn GetMachineHealth
  (return 0.0 0.0))

(fn GetEnemyCurrentHP
  (return 0.0))

(fn GetLocation
  (return "0, 0, 0"))

(fn HasResource
  (params (Resource%20Robot%20Is%20Looking%20For :type Name :default "None"))
  (return "None" 0 0))