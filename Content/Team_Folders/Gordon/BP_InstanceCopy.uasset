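; BP_InstanceCopy provides save events that write a BP_SaveGame to a named slot or trigger the level's save manager.
; NowSaving loads the existing save in the given slot, or creates a new one, stores it in SaveVar and writes it straight back without changing any fields.
; NowSaving2 is a separate path that finds the BP_SaveManager actor and calls its SaveTheGame.
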(event Custom|NowSaving
  (params (File%20Name :type String))
  (bind _returnvalue (SaveGame|DoesSaveGameExist File%20Name))
  (if _returnvalue
    (bind _returnvalue_2 (SaveGame|LoadGamefromSlot File%20Name))
    (bind _asbp_save_game (Utilities|Casting|CastToBP_SaveGame _returnvalue_2))
    (Variables|Default|SetSaveVar _asbp_save_game)
    (else
      (bind _returnvalue_3 (SaveGame|CreateSaveGameObject "/Game/Team_Folders/Gordon/BP_SaveGame.BP_SaveGame_C"))
      (Variables|Default|SetSaveVar _returnvalue_3)))
  (SaveGame|SaveGametoSlot (Variables|Default|GetSaveVar) File%20Name))

(event Custom|NowSaving2
  (bind _returnvalue (Actor|GetActorOfClass "/Game/Blueprints/Managers/BP_SaveManager.BP_SaveManager_C"))
  (Default|SavetheGame _returnvalue))