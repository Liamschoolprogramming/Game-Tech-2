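; Save manager that writes the health of the engine cores to a save slot and reads it back.
; SaveTheGame creates the save object if needed, maps each BP_EngineCore's name to its Health, and saves it to the slot.
; LoadTheGame copies the stored map from an existing slot into SaveReference, without creating that object or applying values back to the cores.
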(event Custom|SaveTheGame
  ;[0.15 0.15 0.15 0.5] Save
  (Utilities|FlowControl|Sequence
    (:then_0
      (Utilities|IsValid (Variables|Default|GetSaveReference)
        (:Is%20Not%20Valid
          (bind _returnvalue (SaveGame|CreateSaveGameObject "/Game/Team_Folders/Gordon/SaveGame.SaveGame_C"))
          (Variables|Default|SetSaveReference _returnvalue))))
    (:then_1
      (bind _outactors (Actor|GetAllActorsOfClass "/Game/Blueprints/EngineCores/BP_EngineCore.BP_EngineCore_C"))
      ;;[0.15 0.15 0.15 0.5] Loop through all 3 Cores
      (for _array_element _outactors
        (Utilities|Map|Add (Variables|Default|GetCoreHealths) (Variables|/Game/Blueprints/EngineCores/BP_EngineCore.BP_EngineCore_C|GetName _array_element) (Variables|/Game/Blueprints/EngineCores/BP_EngineCore.BP_EngineCore_C|GetHealth _array_element)))
      (Variables|/Game/Team_Folders/Gordon/SaveGame.SaveGame_C|SetCoreHealths (Variables|Default|GetSaveReference) (Variables|Default|GetCoreHealths)))
    (:then_2
      (SaveGame|SaveGametoSlot (Variables|Default|GetSaveReference) (Variables|Default|GetSaveSlot)))))

(event Custom|LoadTheGame
  ;[0.15 0.15 0.15 0.5] Load
  (bind _returnvalue (SaveGame|DoesSaveGameExist (Variables|Default|GetSaveSlot)))
  (if _returnvalue
    (bind _returnvalue_2 (SaveGame|LoadGamefromSlot (Variables|Default|GetSaveSlot)))
    (bind _assave_game (Utilities|Casting|CastToSaveGame _returnvalue_2))
    (Variables|/Game/Team_Folders/Gordon/SaveGame.SaveGame_C|SetCoreHealths (Variables|Default|GetSaveReference) (Variables|/Game/Team_Folders/Gordon/SaveGame.SaveGame_C|GetCoreHealths _assave_game))))

(fn ConstructionScript)