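; Base crafting machine Actor that players can pick up and place, with interface functions for robots to query and remove its resources.
; BeginPlay loads recipes from a data table and enters the Placed state, starting a looping timer that pauses while carried.
; Each tick of that timer deducts one named ingredient of the active recipe, located through a name-to-index map over the inventory array.
; Work in progress: crafting yields no output item, and several graph chains are disconnected.
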(event Custom|Start%20Timer
  ;[0.15 0.15 0.15 0.5] Crafting An Item
  (bind _returnvalue (Utilities|Time|SetTimerbyEvent (delegate Custom|Timer) (Variables|Default|GetSpeed) true)))

(event Custom|Timer
  ;[0.15 0.15 0.15 0.5] Crafting An Item
  (bind (_resource_name _resource_index) (CallFunction|GetResourceAmount (Variables|Containers|GetResourceIndex) (Variables|Default|Getname)))
  (CallFunction|CraftItem (Variables|Default|GetActiveRecipe) (Variables|Containers|GetResourceInventory) _resource_name _resource_index))

(event Custom|Stop%20Timer
  ;[0.15 0.15 0.15 0.5] Crafting An Item
  (Utilities|Time|ClearandInvalidateTimerbyHandle (stale Custom|Start%20Timer _returnvalue)))

(event Custom|EventChange
  ;[0.15 0.15 0.15 0.5] Event Logic
  (switch Utilities|FlowControl|Switch|SwitchonE_MachineState (Variables|Enum|GetMachineStates)
    (:NewEnumerator0
      (Utilities|FlowControl|DoOnce false
        (:Completed
          (Development|PrintString "In the default state")
          (Variables|Enum|SetMachineStates "NewEnumerator3")
          (Development|PrintString "Switching to crafting")
          (CallFunction|EventChange))))
    (:NewEnumerator3
      (switch Utilities|FlowControl|Switch|SwitchonE_MachineSubState (Variables|Enum|GetMachineSubStates)
        (:NewEnumerator0
          (CallFunction|StartTimer)
          (Development|PrintString " Started crafting"))))))

(event EventRemoveResource1
  (params (Resource%20Name :type Name :default "None") (Amount%20To%20Remove :type Integer) (Resource%20Index :type Integer))
  ;[0.15 0.15 0.15 0.5] BPI Logic
  (CallFunction|SetResourceAmount Resource%20Index Amount%20To%20Remove (Variables|Containers|GetResourceInventory)))

(event EventRenameMachine
  (Rendering|Components|TextRender|SetText (Variables|Default|GetTextRender) (Utilities|Text|ToText(String) (Utilities|String|Append (Utilities|String|ToString(Name) (Variables|Default|GetMachineName)) (Utilities|String|ToString(Integer) (Math|Random|RandomInteger 100)))))
  (Variables|Enum|SetMachineRecipeSlot (Utilities|Enum|ByteToEnumE_MachineRecipeSlot (Math|Conversions|ToByte(Integer) (Math|Random|RandomInteger 3)))))

(event EventSelection
  (params (Player :type BP%20FP%20Character%20Object%20Reference))
  ;[0.15 0.15 0.15 0.5] BPI Logic
)

(event EventBeginPlay
  (CallFunction|AddingRecipes (Variables|DataTables|GetRecipes) (Variables|Containers|GetRecipeInventory))
  (CallFunction|EventChange))

(event EventPickupMachine
  (params (Player :type BP%20FP%20Character%20Object%20Reference))
  ;[0.15 0.15 0.15 0.5] BPI Logic
  (Transformation|AttachComponentToComponent (.ItemSocket (Utilities|Struct|BreakS_Linetrace (Variables|/Game/Blueprints/Player/BP_FPCharacter.BP_FPCharacter_C|GetLineTraceInfo (stale EventSelection Player)))) "None" "SnapToTarget" "KeepRelative" "KeepRelative" true)
  (Variables|Enum|SetMachineStates "NewEnumerator2")
  (CallFunction|StopTimer)
  (Development|PrintString "Is picked up")
  (CallFunction|EventChange))

(event EventPlaceMachine
  ;[0.15 0.15 0.15 0.5] BPI Logic
  (Transformation|DetachFromActor "KeepRelative" "KeepRelative" "KeepRelative")
  (Transformation|SetActorTransform self (Math|Conversions|ToTransform(Vector) (.HitLocation (Utilities|Struct|BreakS_Linetrace (Variables|/Game/Blueprints/Player/BP_FPCharacter.BP_FPCharacter_C|GetLineTraceInfo (stale EventSelection Player))))))
  (Variables|Enum|SetMachineStates "NewEnumerator3")
  (CallFunction|StartTimer)
  (Development|PrintString "Is placed")
  (CallFunction|EventChange))

(fn ConstructionScript
  (Variables|Default|SetMachineName (Utilities|String|StringToName (Utilities|GetDisplayName self)))
  (CallFunction|InventoryMap (Variables|Containers|GetResourceInventory) (Variables|Containers|GetResourceIndex)))

(fn ResourceUpdate
  (params (TargetMap :type Map%20of%20Strings%20to%20Structs) (Resource%20Name :type String))
  (bind _value (Utilities|Map|Find TargetMap Resource%20Name))
  (return 0 _value ""))

(fn AddtoInventory
  (params (ResourceInventory :type Array%20of%20S%20Resources%20Structures) (Item :type S%20Resources%20Structure%20%28by%20ref%29))
  (bind (_name _mesh _amount) (Utilities|Struct|BreakS_Resources Item))
  (if (Utilities|Array|IsEmpty ResourceInventory)
    (Utilities|Array|Add ResourceInventory Item)
    (return)
    (else
      (for (_array_element _array_index) ResourceInventory
        (if (== (.Name (Utilities|Struct|BreakS_Resources _array_element)) _name)
          (bind _structout (Utilities|Struct|SetmembersinS_Resources (Utilities|Array|Get(acopy) ResourceInventory _array_index) (+ _amount (.Amount (Utilities|Struct|BreakS_Resources _array_element)))))
          (Development|PrintString (Utilities|String|ToString(Name) (.Name (Utilities|Struct|BreakS_Resources _structout))))
          (else
            (Utilities|Array|Add ResourceInventory Item)))))))

(fn InventoryMap
  (params (Resource%20Inventory :type Array%20of%20S%20Resources%20Structures) (ResourceIndex :type Map%20of%20Names%20to%20Integers))
  (for (_array_element _array_index) Resource%20Inventory
    (Utilities|Map|Add ResourceIndex (.Name (Utilities|Struct|BreakS_Resources _array_element)) _array_index)))

(fn GetResourceAmount
  (params (TargetMap :type Map%20of%20Names%20to%20Integers) (name :type Name))
  (bind _value (Utilities|Map|Find TargetMap name))
  (bind _resourceinventory (Variables|Containers|GetResourceInventory))
  (bind _output (Utilities|Array|Get(acopy) _resourceinventory _value))
  (bind (_name _mesh _amount) (Utilities|Struct|BreakS_Resources _output))
  (return _name _value _amount))

(fn CraftItem
  (params (Recipe :type S%20Recipes%20Structure%20%28by%20ref%29) (Resource%20Inventory :type Array%20of%20S%20Resources%20Structures) (Item%20Name :type Name) (Item%20Index :type Integer))
  (bind _requiredresources (Utilities|Struct|BreakS_Recipes Recipe))
  (bind _output (Utilities|Array|Get(acopy) Resource%20Inventory Item%20Index))
  (bind _amount (Utilities|Struct|BreakS_Resources _output))
  (bind _value (Utilities|Map|Find _requiredresources Item%20Name))
  (if (>= _amount _value)
    (Utilities|Struct|SetmembersinS_Resources _output (- _amount _value))
    (Development|PrintString "Item crafted")
    (return)
    (else
      (return))))

(fn RemoveResource
  (params (Resource%20Inventory :type Array%20of%20S%20Resources%20Structures) (Resource%20Index :type Map%20of%20Names%20to%20Integers) (Name :type Name) (Item%20Index :type Integer)))

(fn SetResourceAmount
  (params (Index :type Integer) (Amount%20To%20Remove :type Integer) (Array :type Array%20of%20S%20Resources%20Structures))
  (bind _output (Utilities|Array|Get(acopy) Array Index))
  (Utilities|Struct|SetmembersinS_Resources _output (- (.Amount (Utilities|Struct|BreakS_Resources _output)) Amount%20To%20Remove)))

(fn AddingRecipes
  (params (Recipes :type Data%20Table%20Object%20Reference%20%28by%20ref%29) (Recipe%20Inventory :type Array%20of%20S%20Recipes%20Structures))
  (for _array_element (Variables|Containers|GetRecipeNames)
    (bind _returnvalue (Utilities|GetDataTableRow Recipes _array_element)
      (:then
        (Utilities|Array|Add Recipe%20Inventory _returnvalue)))))

(fn GameplayTag
  (return "(TagName=\"Interactable\")"))

(fn GetMachineHealth
  (return (Variables|Default|GetCurrentHealth) (Variables|Default|GetMaxHealth)))

(fn GetLocation1
  (return (Transformation|GetActorLocation)))

(fn GetLocation
  (return (Transformation|GetActorLocation)))

(fn HasResource1
  (params (Resource%20Robot%20Is%20Looking%20For :type Name :default "None"))
  (bind (_resource_name _resource_index _resourceamount) (CallFunction|GetResourceAmount (Variables|Containers|GetResourceIndex) Resource%20Robot%20Is%20Looking%20For))
  (return _resource_name _resource_index _resourceamount))

(fn HasResource
  (params (Resource%20Robot%20Is%20Looking%20For :type Name :default "None"))
  (return "None" 0 0))