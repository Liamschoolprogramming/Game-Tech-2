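; BP_RobotStation is a station that charges robots while they stand inside its Box trigger.
; On begin overlap it sends ChargeAmount as a charge-per-second message to actors implementing BPI_Robot, and resets the rate to zero on end overlap.
; GetLocation returns the Arrow component's world location.
; GetMachineHealth and HasResource return only empty default values, so the station reports no health or resources.
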(event OnComponentBeginOverlap(Box)
  (params (OverlappedComponent :type Primitive%20Component%20Object%20Reference) (OtherActor :type Actor%20Object%20Reference) (OtherComp :type Primitive%20Component%20Object%20Reference) (OtherBodyIndex :type Integer) (bFromSweep :type Boolean) (SweepResult :type Hit%20Result%20Structure%20%28by%20ref%29))
  (if (Utilities|DoesObjectImplementInterface OtherActor "/Game/Blueprints/Robot/BPI_Robot.BPI_Robot_C")
    (Class|BPIRobot|SetChargePerSecond(Message) OtherActor (Variables|Default|GetChargeAmount))))

(event OnComponentEndOverlap(Box)
  (params (OverlappedComponent :type Primitive%20Component%20Object%20Reference) (OtherActor :type Actor%20Object%20Reference) (OtherComp :type Primitive%20Component%20Object%20Reference) (OtherBodyIndex :type Integer))
  (if (Utilities|DoesObjectImplementInterface OtherActor "/Game/Blueprints/Robot/BPI_Robot.BPI_Robot_C")
    (Class|BPIRobot|SetChargePerSecond(Message) OtherActor 0.0)))

(fn ConstructionScript)

(fn GetMachineHealth
  (return 0.0 0.0))

(fn GetLocation
  (return (Transformation|GetWorldLocation (Variables|Default|GetArrow))))

(fn HasResource
  (params (Resource%20Robot%20Is%20Looking%20For :type Name :default "None"))
  (return "None" 0 0))