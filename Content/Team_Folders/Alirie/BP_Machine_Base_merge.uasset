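; Base Blueprint for placeable, powered machines the player can build, pick up, place, repair and use.
; UpdateStatus finds the nearest in-range BP_EngineCore, registers energy cost and sets operational state, shown on camera-facing, color-coded text.
; Interface events drive attach/detach placement, overlap prompts, a looping repair timer and resource drop-off to its inventory.
; ActionInteract is empty, and most type-specific upgrade functions raise script errors, expecting child-class overrides.
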(event OnComponentBeginOverlap(InputInteractionBox)
  (params (OverlappedComponent :type Primitive%20Component%20Object%20Reference) (OtherActor :type Actor%20Object%20Reference) (OtherComp :type Primitive%20Component%20Object%20Reference) (OtherBodyIndex :type Integer) (bFromSweep :type Boolean) (SweepResult :type Hit%20Result%20Structure%20%28by%20ref%29))
  ;[0.15 0.15 0.15 0.5] Interactions with other actors
  (CallFunction|DisplayInteract OtherActor))

(event OnComponentEndOverlap(InputInteractionBox)
  (params (OverlappedComponent :type Primitive%20Component%20Object%20Reference) (OtherActor :type Actor%20Object%20Reference) (OtherComp :type Primitive%20Component%20Object%20Reference) (OtherBodyIndex :type Integer))
  ;[0.15 0.15 0.15 0.5] Interactions with other actors
  (CallFunction|HideInteract OtherActor))

(event Custom|Upgrade
  (params (Upgrades :type E_Upgrades%20Enum :default "NewEnumerator0"))
  (CallFunction|UpgradeMachine))

(event Custom|UpdateWidgets
  ;[0.15 0.15 0.15 0.5] Initialize Text Widgets
  (CallFunction|SetWidgetRotation (Variables|Default|GetTextRender))
  (CallFunction|SetWidgetRotation (Variables|Default|GetPoweredByText))
  (CallFunction|UpdateStatus))

(event EventBuildMachine
  (params (Player :type BP%20FP%20Character%20Object%20Reference))
  ;[0.15 0.15 0.15 0.5] BPI Logic
  (CallFunction|BuildtheMachine Player))

(event EventEnergy
  (params (Sending%20Core :type BP%20Engine%20Core%20Object%20Reference) (Operational? :type Boolean))
  ;[0.15 0.15 0.15 0.5] Recieving Energy From the Core
  (if Operational?
    (switch Utilities|FlowControl|Switch|SwitchonE_OperationalState (Variables|Enum|GetOperational%20State)
      (:NewEnumerator0
        _)
      (:NewEnumerator2
        _))
    (Variables|Enum|SetOperational%20State "NewEnumerator2")
    (CallFunction|UpdateStatus)
    (CallFunction|SetPoweredbyText)
    (else
      (switch Utilities|FlowControl|Switch|SwitchonE_OperationalState (Variables|Enum|GetOperational%20State)
        (:NewEnumerator0
          _)
        (:NewEnumerator2
          _))
      (Variables|Enum|SetOperational%20State "NewEnumerator0")
      (CallFunction|SetPoweredbyText))))

(event EventDropOffResource
  (params (ResourceName :type Name :default "None") (ResourceAmount :type Integer))
  (CallFunction|DropOffResourceAction ResourceName ResourceAmount))

(event EventPickupMachine
  (params (Player :type BP%20FP%20Character%20Object%20Reference))
  ;[0.15 0.15 0.15 0.5] BPI Logic
  (CallFunction|AttachtoComponet)
  (CallFunction|UpdateStatus))

(event EventPlaceMachine
  (params (Player :type BP%20FP%20Character%20Object%20Reference))
  ;[0.15 0.15 0.15 0.5] BPI Logic
  (CallFunction|PlaceMachineDown Player)
  (CallFunction|UpdateStatus))

(event EventRepair
  (params (Player :type BP%20FP%20Character%20Object%20Reference) (Repairing? :type Boolean))
  ;[0.15 0.15 0.15 0.5] Start repair timer when holding R and stop when R is released - Set player state to repairing if health isn't full, otherise cancel this event - Also stop if repairing finishes
  (CallFunction|RepairMachine Player Repairing?))

(event EventInteract
  (params (Player :type BP%20FP%20Character%20Object%20Reference))
  (CallFunction|ActionInteract Player))

(fn ConstructionScript
  (bind _machine_info_defaults (Variables|Default|GetMachine%20Info%20Defaults))
  (CallFunction|SetUniqueName)
  (bind _output_get (Variables|Default|SetMachine%20Info (Utilities|Struct|MakeStruct_MachineValues (.maxhealth _machine_info_defaults) (.distancefromcore _machine_info_defaults) (.energycost _machine_info_defaults) (.productionrate _machine_info_defaults))))
  (Variables|Default|SetCurrentHealth (.maxhealth _output_get)))

(fn ResourceUpdate
  (params (TargetMap :type Map%20of%20Strings%20to%20Structs) (Resource%20Name :type String))
  (bind _value (Utilities|Map|Find TargetMap Resource%20Name))
  (return 0 _value ""))

(fn AddtoInventory
  (params (ResourceInventory :type Array%20of%20S%20Resources%20Structures) (Item :type S%20Resources%20Structure%20%28by%20ref%29))
  (bind (_name _mesh _amount) (Utilities|Struct|BreakS_Resources Item))
  (if (Utilities|Array|IsEmpty ResourceInventory)
    (Utilities|Array|Add ResourceInventory Item)
    (return)
    (else
      (for (_array_element _array_index) ResourceInventory
        (if (== (.Name (Utilities|Struct|BreakS_Resources _array_element)) _name)
          (Utilities|Struct|SetmembersinS_Resources (Utilities|Array|Get(acopy) ResourceInventory _array_index) (+ _amount (.Amount (Utilities|Struct|BreakS_Resources _array_element))))
          (else
            (Utilities|Array|Add ResourceInventory Item)))))))

(fn SetResourceAmount
  (params (Index :type Integer) (Amount%20To%20Remove :type Integer) (Array :type Array%20of%20S%20Resources%20Structures))
  (bind _output (Utilities|Array|Get(acopy) Array Index))
  (Utilities|Struct|SetmembersinS_Resources _output (- (.Amount (Utilities|Struct|BreakS_Resources _output)) Amount%20To%20Remove)))

(fn SetCorePoweredby
  (LocalVariables|SetL_Distance 9999.0)
  (bind _outactors (Actor|GetAllActorsOfClass "/Game/Blueprints/EngineCores/BP_EngineCore.BP_EngineCore_C"))
  (for _array_element _outactors
    (LocalVariables|SetL_CoreArrayItem _array_element)
    (if (and (< (Transformation|GetHorizontalDistanceTo (LocalVariables|GetL_CoreArrayItem) self) (LocalVariables|GetL_Distance)) (<= (Transformation|GetHorizontalDistanceTo (LocalVariables|GetL_CoreArrayItem) self) (.distancefromcore (Variables|Default|GetMachine%20Info))))
      (LocalVariables|SetL_TempCore (LocalVariables|GetL_CoreArrayItem))
      (LocalVariables|SetL_Distance (Transformation|GetHorizontalDistanceTo (LocalVariables|GetL_CoreArrayItem) self))))
  (bind _l_tempcore (LocalVariables|GetL_TempCore)
    (:then
      (Variables|Default|SetCore%20Powered%20By _l_tempcore)
      (Variables|Enum|SetOperational%20State "NewEnumerator2")
      (Default|VerifyDependentMachine (Variables|Default|GetCore%20Powered%20By) self (.energycost (Variables|Default|GetMachine%20Info)) true))
    (:else
      (bind _asbp_fpcharacter (Utilities|Casting|CastToBP_FPCharacter (Game|GetPlayerCharacter 0)))
      (Default|DisplayAlert _asbp_fpcharacter "Machine not in range of core!")
      (Variables|Enum|SetOperational%20State "NewEnumerator0")
      (bind _core_powered_by (Variables|Default|GetCore%20Powered%20By)
        (:then
          (Default|VerifyDependentMachine _core_powered_by self (.energycost (Variables|Default|GetMachine%20Info)) false))
        (:else)))))

(fn SetPoweredbyText
  (bind _poweredbytext (Variables|Default|GetPoweredByText))
  (bind _operational_state (Variables|Enum|GetOperational%20State))
  (Rendering|Components|TextRender|SetText _poweredbytext (|GenerictoText _operational_state))
  (Rendering|Components|TextRender|SetTextRenderColor _poweredbytext (Utilities|Select :Index _operational_state :NewEnumerator0 (Class|KismetMathLibrary|LinearColortoRGBE "(R=0.679543,G=0.005182,B=0.040915,A=1.000000)") :NewEnumerator1 (Class|KismetMathLibrary|LinearColortoRGBE) :NewEnumerator2 (Class|KismetMathLibrary|LinearColortoRGBE "(R=0.000000,G=1.000000,B=0.327778,A=1.000000)"))))

(fn ChangeCoreState
  (CallFunction|SetCorePoweredby)
  (switch Utilities|FlowControl|Switch|SwitchonE_MachineState (Variables|Enum|GetMachineStates)
    (:NewEnumerator0
      (Variables|Enum|SetMachineStates "NewEnumerator3"))
    (:NewEnumerator3
      (CallFunction|SetPoweredbyText)
      (switch Utilities|FlowControl|Switch|SwitchonE_OperationalState (Variables|Enum|GetOperational%20State)
        (:NewEnumerator0
          (CallFunction|SetCorePoweredby))
        (:NewEnumerator2
          (switch Utilities|FlowControl|Switch|SwitchonE_MachineSubState (Variables|Enum|GetMachineSubStates)))))))

(fn AttachtoComponet
  (Transformation|AttachComponentToComponent 0 "None" "SnapToTarget" "KeepRelative" "KeepRelative" true)
  (Variables|Enum|SetMachineStates "NewEnumerator2"))

(fn PlaceMachineDown
  (params (Player :type BP%20FP%20Character%20Object%20Reference))
  (Transformation|DetachFromActor "KeepRelative" "KeepRelative" "KeepRelative")
  (Transformation|SetActorTransform self (Math|Conversions|ToTransform(Vector) (.hitlocation (Variables|/Game/Blueprints/Player/BP_FPCharacter.BP_FPCharacter_C|GetLineTraceInfo Player))))
  (Variables|Enum|SetMachineStates "NewEnumerator3"))

(fn BuildtheMachine
  (params (Player :type BP%20FP%20Character%20Object%20Reference))
  (Variables|/Game/Blueprints/Player/BP_FPCharacter.BP_FPCharacter_C|SetBuildMachine Player self)
  (Transformation|AttachComponentToComponent (Variables|/Game/Blueprints/Player/BP_FPCharacter.BP_FPCharacter_C|GetObjectPickup Player) "None" "SnapToTarget" "KeepRelative" "KeepRelative" true)
  (Variables|Enum|SetMachineStates "NewEnumerator2"))

(fn CalculateWidgetRotation
  (params (Widget :type Scene%20Component%20Object%20Reference))
  (return (Math|Rotator|FindLookatRotation (Transformation|GetWorldLocation Widget) (Transformation|GetWorldLocation (Variables|/Script/Engine.PlayerCameraManager|GetTransformComponent (Game|GetPlayerCameraManager 0))))))

(fn SetWidgetRotation
  (params (Widget :type Scene%20Component%20Object%20Reference))
  (Transformation|SetWorldRotation Widget (CallFunction|CalculateWidgetRotation Widget) false false))

(fn ReceiveBeginPlay
  (bind _returnvalue (Actor|GetActorOfClass "/Game/Blueprints/LevelEventManager/BP_LevelEventManager.BP_LevelEventManager_C"))
  (Variables|Default|SetLevelEventManager _returnvalue)
  (bind _returnvalue_2 (Actor|GetActorOfClass "/Game/Blueprints/Managers/BP_CoreManager.BP_CoreManager_C"))
  (Variables|Default|SetCoreManager _returnvalue_2))

(fn UpgradeMachine
  (bind _output_get (Variables|Default|SetMachine%20Info%20Defaults (Utilities|Struct|MakeStruct_MachineValues 0.0 0.0 0 (- (.productionrate (Variables|Default|GetMachine%20Info%20Defaults)) 0.2))))
  (Development|PrintString (Utilities|String|ToString(Float) (.ProductionRate (Utilities|Struct|BreakStruct_MachineValues _output_get)))))

(fn DisplayInteract
  (params (Actor :type Actor%20Object%20Reference))
  (if (not (Utilities|DoesObjectImplementInterface Actor "/Game/Blueprints/Robot/BPI_Robot.BPI_Robot_C"))
    (if (< (Variables|Default|GetCurrentHealth) (.maxhealth (Variables|Default|GetMachine%20Info)))
      (bind _asbp_fpcharacter (Utilities|Casting|CastToBP_FPCharacter Actor))
      (Default|DisplayInputPrompt _asbp_fpcharacter "Press E to Interact & R to Repair")
      (else
        (bind _asbp_fpcharacter_2 (Utilities|Casting|CastToBP_FPCharacter Actor))
        (Default|DisplayInputPrompt _asbp_fpcharacter_2 "Press E to Interact")))))

(fn HideInteract
  (params (Object :type Object%20Object%20Reference))
  (if (not (Utilities|DoesObjectImplementInterface Object "/Game/Blueprints/Robot/BPI_Robot.BPI_Robot_C"))
    (bind _asbp_fpcharacter (Utilities|Casting|CastToBP_FPCharacter Object))
    (Default|HideInputPrompt _asbp_fpcharacter)))

(fn RepairMachine
  (params (Player :type BP%20FP%20Character%20Object%20Reference) (Condition :type Boolean))
  (if Condition
    (if (< (Variables|Default|GetCurrentHealth) (.maxhealth (Variables|Default|GetMachine%20Info)))
      (Variables|/Game/Blueprints/Player/BP_FPCharacter.BP_FPCharacter_C|SetPlayerStates Player "NewEnumerator6")
      (Utilities|Time|ClearandInvalidateTimerbyHandle (Variables|Default|GetRepair%20Timer))
      (bind _returnvalue (Utilities|Time|SetTimerbyEvent (EventDispatchers|CreateEvent :!event RepairAction) 0.2 true))
      (Variables|Default|SetRepair%20Timer _returnvalue))
    (else
      (Utilities|Time|ClearandInvalidateTimerbyHandle (Variables|Default|GetRepair%20Timer))
      (Default|DisplayRepairing Player (Variables|Default|GetCurrentHealth) (.maxhealth (Variables|Default|GetMachine%20Info)) false))))

(fn RepairAction
  (if (< (Variables|Default|GetCurrentHealth) (.maxhealth (Variables|Default|GetMachine%20Info)))
    (Default|DisplayRepairing (LocalVariables|GetL_Player) (Math|Float|Clamp(Float) (+ (Variables|Default|GetCurrentHealth) 1.0) 0.0 (.maxhealth (Variables|Default|GetMachine%20Info))) (.maxhealth (Variables|Default|GetMachine%20Info)) true)
    (if (Utilities|Enum|Equal(Enum) (Variables|Enum|GetOperational%20State) "NewEnumerator1")
      (CallFunction|UpdateStatus))
    (else
      (Utilities|Time|ClearandInvalidateTimerbyHandle (Variables|Default|GetRepair%20Timer))
      (Default|DisplayRepairing (LocalVariables|GetL_Player) (Variables|Default|GetCurrentHealth) (.maxhealth (Variables|Default|GetMachine%20Info)) false))))

(fn ActionInteract
  (params (Player :type BP%20FP%20Character%20Object%20Reference)))

(fn DropOffResourceAction
  (params (ResourceName :type Name) (Amount :type Integer))
  (Default|AddResourcetoInventory (Variables|Default|GetBP_Inventory) ResourceName Amount))

(fn UpdateStatus
  (CallFunction|SetCorePoweredby)
  (switch Utilities|FlowControl|Switch|SwitchonE_MachineState (Variables|Enum|GetMachineStates)
    (:NewEnumerator0
      (Variables|Enum|SetMachineStates "NewEnumerator3"))
    (:NewEnumerator3
      (CallFunction|SetPoweredbyText)
      (switch Utilities|FlowControl|Switch|SwitchonE_OperationalState (Variables|Enum|GetOperational%20State)
        (:NewEnumerator0
          (CallFunction|SetCorePoweredby))
        (:NewEnumerator2
          (switch Utilities|FlowControl|Switch|SwitchonE_MachineSubState (Variables|Enum|GetMachineSubStates)))))))

(fn MachineReceiveEnergy
  (params (Operational? :type Boolean))
  (if Operational?
    (switch Utilities|FlowControl|Switch|SwitchonE_OperationalState (Variables|Enum|GetOperational%20State)
      (:NewEnumerator0
        _)
      (:NewEnumerator2
        _))
    (Variables|Enum|SetOperational%20State "NewEnumerator2")
    (CallFunction|SetPoweredbyText)
    (else
      (switch Utilities|FlowControl|Switch|SwitchonE_OperationalState (Variables|Enum|GetOperational%20State)
        (:NewEnumerator0
          _)
        (:NewEnumerator2
          _))
      (Variables|Enum|SetOperational%20State "NewEnumerator0")
      (CallFunction|SetPoweredbyText))))

(fn UpgradeCraftingSpeed
  (CallFunction|UpgradeError))

(fn UpgradeRobotStationInventorySize
  (CallFunction|UpgradeError))

(fn UpgradeConvertorExtraResource
  (CallFunction|UpgradeError))

(fn UpgradeError
  (Utilities|Debugging|RaiseScriptError "Upgrade is being called from the baseclass. Please over ride the functionality of this upgrade in the child class of the machine that will use it"))

(fn UpgradeConvertorDamage
  (CallFunction|UpgradeError))

(fn UpgradeConverterDoubleCraftingSpeed
  (CallFunction|UpgradeError))

(fn UpgradeRobotStationTurboCharge
  (CallFunction|UpgradeRobotStationTurboCharge))

(fn SetUniqueName
  (LocalVariables|SetL_NewName (Utilities|String|Append (Utilities|String|ToString(Name) (Variables|Default|GetMachineType)) (Utilities|String|ToString(Integer) (Math|Random|RandomInteger 100))))
  (bind _outactors (Actor|GetAllActorsOfClass "/Game/Blueprints/Machines/MachineBaseClass/BP_Machine_Base.BP_Machine_Base_C"))
  (bind _array_element (Utilities|Array|ForEachLoopwithBreak _outactors :!label _label)
    (:LoopBody
      (if (== (Variables|BP_Machine_Base_merge_C|GetName _array_element) (LocalVariables|GetL_NewName))
        (CallFunction|SetUniqueName)
        (LocalVariables|SetL_NotUnique true)
        (goto _label Break)))
    (:Completed
      (if (not (LocalVariables|GetL_NotUnique))
        (Variables|Default|SetName (Utilities|String|StringToName (LocalVariables|GetL_NewName)))))))

(fn GameplayTag
  (return "(TagName=\"Interactable\")"))

(fn GetMachineHealth
  (return 0.0 0.0))

(fn GetGameplayTags
  (return (Variables|Default|GetGameplayTags)))

(fn GetLocation
  (return (Transformation|GetActorLocation)))

(fn GetMachine
  (return self))

(fn GetMachineClass
  (return 0))

(fn GetMachineMesh
  (return 0))

(fn GetName
  (return (Variables|Default|GetName)))

(fn HasResource
  (params (Resource%20Name :type Name :default "None"))
  (bind _resource_amount (Default|GetResourceAmount (Variables|Default|GetBP_Inventory) Resource%20Name))
  (return _resource_amount (> _resource_amount 0)))