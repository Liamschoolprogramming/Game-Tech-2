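; Crafting machine that turns resources in its inventory into the selected recipe's output on a looping timer.
; SwitchRecipe starts the timer for recipe slots 1 and 2; Craft halts on missing inputs, and resource drop-offs restart it.
; A timer widget shows progress, and interacting toggles an options menu that locks player movement.
; Upgrades add chance-based bonus output or defer to the parent; crafting speed only rescales the mesh, and converter damage is empty.
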(event Custom|OnCraftingTimer
  (bind _menu_widget (Variables|Default|GetMenu%20Widget))
  (CallFunction|Craft)
  (Utilities|IsValid _menu_widget
    (:Is%20Valid
      (if (UserInterface|Viewport|IsinViewport _menu_widget)
        (Default|RefreshInventory (Variables|Default|GetMenu%20Widget))))))

(event EventBeginPlay
  (|CallParentFunction)
  (bind _returnvalue (UserInterface|CreateWidget "/Game/UI/WidgetBlueprints/WB_CraftingTimer.WB_CraftingTimer_C" 0 self))
  (bind _output_get (Variables|Default|SetProgressRef _returnvalue))
  (UserInterface|SetWidget (Variables|Default|GetTimerWidget) _output_get)
  (Utilities|Time|SetTimerbyEvent (EventDispatchers|CreateEvent :!event UpdateWidgets) 0.01 true)
  (CallFunction|SwitchRecipe))

(event EventInteract
  (params (Player :type BP%20FP%20Character%20Object%20Reference))
  (CallFunction|ActionInteract Player))

(event EventUpgrade
  (params (Upgrades :type E_Upgrades%20Enum :default "NewEnumerator0"))
  (switch Utilities|FlowControl|Switch|SwitchonE_Upgrades Upgrades
    (:NewEnumerator0
      (CallFunction|UpgradeCraftingSpeed))
    (:NewEnumerator2
      (CallFunction|UpgradeExtraResource))
    (:NewEnumerator3
      (CallFunction|UpgradeConverterDamage))
    (:NewEnumerator4
      (CallFunction|UpgradeConverterDoubleCraftingSpeed))))

(event EventUpdateWidgets
  (|CallParentFunction)
  (CallFunction|SetWidgetRotation (Variables|Default|GetTimerWidget))
  (Default|UpdateCraftingTimer (Variables|Default|GetProgressRef) (Class|KismetSystemLibrary|GetTimerElapsedTimeHandle (Variables|Default|GetCraftingTimer)) (not (Variables|Default|GetCraftingHalted))))

(event EventDropOffResource
  (params (ResourceName :type Name :default "None") (ResourceAmount :type Integer))
  (|CallParentFunction ResourceName ResourceAmount)
  (if (Variables|Default|GetCraftingHalted)
    (CallFunction|SwitchRecipe)))

(fn ConstructionScript
  (|CallParentFunction))

(fn SwitchRecipe
  (bind _returnvalue (CallFunction|SelectRecipe))
  (Variables|Default|SetCraftingHalted false)
  (switch Utilities|FlowControl|Switch|SwitchonE_MachineRecipeSlot (Variables|Default|GetMachineRecipeSlot)
    (:NewEnumerator0
      (Variables|Default|SetActiveRecipe _returnvalue))
    (:NewEnumerator1
      (Variables|Default|SetActiveRecipe _returnvalue)))
  (CallFunction|StopCraftingTimer)
  (bind _returnvalue_2 (Utilities|Time|SetTimerbyEvent (EventDispatchers|CreateEvent :!event Custom|OnCraftingTimer) (.productionrate (Variables|Default|GetMachine%20Info%20Defaults)) true))
  (Variables|Default|SetCraftingTimer _returnvalue_2)
  (bind _namenowhitespace (CallFunction|StripWhitespaceName (.Name (Utilities|Struct|BreakS_Recipes (Variables|Default|GetActiveRecipe)))))
  (bind _returnvalue_3 (Utilities|GetDataTableRow "/Game/Blueprints/DT_Resources.DT_Resources" _namenowhitespace)
    (:then
      (Default|SetResource (Variables|Default|GetProgressRef) _returnvalue_3 (.productionrate (Variables|Default|GetMachine%20Info%20Defaults))))))

(fn StopCraftingTimer
  (Utilities|Time|ClearandInvalidateTimerbyHandle (Variables|Default|GetCraftingTimer)))

(fn AttachtoComponet
  (|CallParentFunction)
  (CallFunction|StopCraftingTimer))

(fn Craft
  (bind _activerecipe (Variables|Default|GetActiveRecipe))
  (bind _bp_inventory (Variables|Default|GetBP_Inventory))
  (bind (_name _amounttocraft _requiredmachine _requiredresources) (Utilities|Struct|BreakS_Recipes _activerecipe))
  (bind _hasenoughresources (CallFunction|HasEnoughResourcesforRecipe))
  (if _hasenoughresources
    (Variables|Default|SetCraftingHalted false)
    (LocalVariables|SetL_ResourceNameToCraft _name)
    (bind (_keypin _valuepin) (Utilities|Map|ForEachLoop(Map) _requiredresources)
      (:then
        (Default|RemoveResourcefromInventory _bp_inventory _keypin _valuepin))
      (:CompletedPin
        (Default|AddResourcetoInventory _bp_inventory (LocalVariables|GetL_ResourceNameToCraft) _amounttocraft)
        (if (Variables|Default|GetDuplicateUpgrade)
          (bind _output_get (Variables|Default|SetDuplicateCraftedItem (Math|Random|RandomInteger 10)))
          (if (Math|Integer|InRange(Integer) _output_get 7 10)
            (Default|AddResourcetoInventory (Variables|Default|GetBP_Inventory) (LocalVariables|GetL_ResourceNameToCraft) 1)))))
    (else
      (Variables|Default|SetCraftingHalted true))))

(fn HasEnoughResourcesforRecipe
  (bind (_keypin _valuepin) (Utilities|Map|ForEachLoop(Map) (.RequiredResources (Utilities|Struct|BreakS_Recipes (Variables|Default|GetActiveRecipe))))
    (:then
      (bind _resource_amount (Default|GetResourceAmount (Variables|Default|GetBP_Inventory) _keypin))
      (if (< _resource_amount _valuepin)
        (return false)))
    (:CompletedPin
      (return true))))

(fn AddingRecipes
  (params (Recipes :type Data%20Table%20Object%20Reference%20%28by%20ref%29) (Recipe%20Inventory :type Array%20of%20S%20Recipes%20Structures))
  (for _array_element (Variables|Default|GetRecipeNames)
    (bind _returnvalue (Utilities|GetDataTableRow Recipes _array_element)
      (:then
        (Utilities|Array|Add Recipe%20Inventory _returnvalue)))))

(fn UpdateCraftTimer
  (Variables|/Game/UI/WidgetBlueprints/WB_CraftingTimer.WB_CraftingTimer_C|SetMaxTime (Variables|Default|GetProgressRef) (.productionrate (Variables|Default|GetMachine%20Info)))
  (Variables|/Game/UI/WidgetBlueprints/WB_CraftingTimer.WB_CraftingTimer_C|SetCurrentTime (Variables|Default|GetProgressRef) (Variables|Default|GetCraftingTimePassed))
  (return))

(fn SelectRecipe
  (bind _recipeinventory (Variables|Default|GetRecipeInventory))
  (bind _machinerecipeslot (Variables|Default|GetMachineRecipeSlot))
  (bind _returnvalue (Math|Conversions|ToInteger(Byte) _machinerecipeslot))
  (bind _output (Utilities|Array|Get(acopy) _recipeinventory _returnvalue))
  (return (Utilities|Select :Index _machinerecipeslot :NewEnumerator0 _output :NewEnumerator1 _output :NewEnumerator2 _output :NewEnumerator3 _output)))

(fn ActionInteract
  (params (Player :type BP%20FP%20Character%20Object%20Reference))
  (bind _bp_inventory (Variables|/Game/Blueprints/Player/BP_FPCharacter.BP_FPCharacter_C|GetBP_Inventory Player))
  (|CallParentFunction Player)
  (Utilities|IsValid (Variables|Default|GetMenu%20Widget)
    (:Is%20Valid
      _)
    (:Is%20Not%20Valid
      (bind _returnvalue (UserInterface|CreateWidget "/Game/UI/WidgetBlueprints/MachineInventory/W_CraftingMachineOptions.W_CraftingMachineOptions_C" (Game|GetPlayerController 0) _bp_inventory self (Variables|Default|GetBP_Inventory)))
      (Variables|Default|SetMenu%20Widget _returnvalue)
      (Default|InstantiateMachineValues _returnvalue _bp_inventory (Variables|Default|GetBP_Inventory))))
  (if (UserInterface|Viewport|IsinViewport (Variables|Default|GetMenu%20Widget))
    (Widget|RemovefromParent (Variables|Default|GetMenu%20Widget))
    (Variables|/Game/Blueprints/Player/BP_FPCharacter.BP_FPCharacter_C|SetMovementEnabled Player true)
    (Variables|/Game/Blueprints/Player/BP_FPCharacter.BP_FPCharacter_C|SetMenuOpen Player false)
    (Input|SetInputModeGameOnly (Game|GetPlayerController 0) true)
    (Variables|/Script/Engine.PlayerController|SetbShowMouseCursor (Game|GetPlayerController 0) false)
    (else
      (UserInterface|Viewport|AddtoViewport (Variables|Default|GetMenu%20Widget) 0)
      (Variables|/Game/Blueprints/Player/BP_FPCharacter.BP_FPCharacter_C|SetMovementEnabled Player false)
      (Variables|/Game/Blueprints/Player/BP_FPCharacter.BP_FPCharacter_C|SetMenuOpen Player true)
      (Input|SetInputModeGameandUI (Game|GetPlayerController 0) 0 "DoNotLock" true true)
      (Variables|/Script/Engine.PlayerController|SetbShowMouseCursor (Game|GetPlayerController 0) true)
      (Widget|SetVisibility (Variables|Default|GetMenu%20Widget) "Visible"))))

(fn UpgradeCraftingSpeed
  (bind _mesh (Variables|Character|GetMesh))
  (bind _returnvalue (Transformation|GetWorldTransform _mesh))
  (Transformation|SetWorldTransform _mesh (Math|Transform|MakeTransform (.location _returnvalue) (.rotation _returnvalue) "1.200000,1.200000,1.200000") false false))

(fn UpgradeExtraResource
  (Variables|Default|SetDuplicateUpgrade true))

(fn UpgradeConverterDamage)

(fn UpgradeConverterDoubleCraftingSpeed
  (|CallParentFunction))

(fn HasResource
  (params (Resource%20Name :type Name :default "None"))
  (bind (_resource_amount _has_resource) (|CallParentFunction Resource%20Name))
  (return _resource_amount _has_resource))