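; BP_TestInteractCube is a test actor for checking the interaction system.
; It adds an "Interactable" tag to its actor tags in the Construction Script, marking it as interactable.
; On BeginPlay it prints its display name as present in the level, and its Interact event prints a message naming itself.
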(event EventInteract
  (Development|PrintString (Utilities|String|Append "Interacted with " (Utilities|GetDisplayName self))))

(event EventBeginPlay
  (Development|PrintString (Utilities|String|Append (Utilities|GetDisplayName self) " in level")))

(fn ConstructionScript
  (bind _objecttags (Variables|Default|GetObjectTags))
  ;[0.15 0.15 0.15 0.5] Initialize object tags
  (Utilities|Array|Add _objecttags "Interactable")
  (Variables|Default|SetTags _objecttags))